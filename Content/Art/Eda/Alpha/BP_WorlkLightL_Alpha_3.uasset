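; Work light Blueprint that builds a cable with an end plug along a spline in the construction script; its event graph is unused.
; Cable spline meshes repeat at intervals scaled by actor X scale, with tangents clamped to segment length.
; The plug sits at the spline point indexed by the loop's final Index + 1, oriented by tangent and selected forward axis, then adjusted by scale, offset and rotation variables.
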(event EventBeginPlay)

(event Collision|EventActorBeginOverlap
  (params (OtherActor :type Actor%20Object%20Reference)))

(event EventTick
  (params (DeltaSeconds :type Float%20%28single-precision%29)))

(fn ConstructionScript
  (bind _spline (Variables|Default|GetSpline))
  (bind _end_mesh_roll (Variables|Default|GetEnd%20Mesh%20Roll))
  (bind _spline_2 (Variables|Default|GetSpline))
  (bind (_x _y _z) (Math|Vector|BreakVector _end_mesh_roll))
  (Utilities|FlowControl|Sequence
    (:then_0
      (Variables|Default|SetSectionalEngth (* (.x (Transformation|GetActorScale3D)) 7.0))
      (for _index (range 0 (Math|Float|Truncate (/ (Spline|GetSplineLength (Variables|Default|GetSpline)) (Variables|Default|GetSectionalEngth))))
        (bind _returnvalue (AddComponent|AddSplineMeshComponent false))
        (SplineMesh|SetForwardAxis _returnvalue "X" true)
        (Components|StaticMesh|SetStaticMesh _returnvalue "/Game/Art/Eda/MDL/WorkLight/Cable.Cable")
        (SplineMesh|SetStartandEnd _returnvalue (Spline|GetLocationatDistanceAlongSpline _spline_2 (* _index (Variables|Default|GetSectionalEngth)) "Local") (Math|Vector|ClampVectorSize (Spline|GetTangentatDistanceAlongSpline _spline_2 (* _index (Variables|Default|GetSectionalEngth)) "Local") 0.0 (Variables|Default|GetSectionalEngth)) (Spline|GetLocationatDistanceAlongSpline _spline (* (+ _index 1) (Variables|Default|GetSectionalEngth)) "Local") (Math|Vector|ClampVectorSize (Spline|GetTangentatDistanceAlongSpline _spline (* (+ _index 1) (Variables|Default|GetSectionalEngth)) "Local") 0.0 (Variables|Default|GetSectionalEngth)) true :!class /Script/Engine.SplineMeshComponent)))
    (:then_1
      (bind _returnvalue_2 (AddComponent|AddStaticMeshComponent false))
      (Components|StaticMesh|SetStaticMesh _returnvalue_2 "/Game/Art/Eda/MDL/WorkLight/Plug.Plug")
      (Transformation|SetRelativeLocationAndRotation _returnvalue_2 (.Location (Spline|GetLocationandTangentatSplinePoint (Variables|Default|GetSpline) (+ _index 1) "Local")) (Utilities|Select :Index (Variables|Default|GetTerminations%20Forward%20Axis) :X (Math|Conversions|RotationFromXVector (.Tangent (Spline|GetLocationandTangentatSplinePoint (Variables|Default|GetSpline) (+ _index 1) "Local"))) :Y (Math|Rotator|MakeRotator (+ (.Roll (Math|Rotator|BreakRotator (Math|Conversions|RotationFromXVector (.Tangent (Spline|GetLocationandTangentatSplinePoint (Variables|Default|GetSpline) (+ _index 1) "Local"))))) 9e+01) (.Pitch (Math|Rotator|BreakRotator (Math|Conversions|RotationFromXVector (.Tangent (Spline|GetLocationandTangentatSplinePoint (Variables|Default|GetSpline) (+ _index 1) "Local"))))) (.Yaw (Math|Rotator|BreakRotator (Math|Conversions|RotationFromXVector (.Tangent (Spline|GetLocationandTangentatSplinePoint (Variables|Default|GetSpline) (+ _index 1) "Local")))))) :Z (Math|Rotator|MakeRotator (.Roll (Math|Rotator|BreakRotator (Math|Conversions|RotationFromXVector (.Tangent (Spline|GetLocationandTangentatSplinePoint (Variables|Default|GetSpline) (+ _index 1) "Local"))))) (+ (.Pitch (Math|Rotator|BreakRotator (Math|Conversions|RotationFromXVector (.Tangent (Spline|GetLocationandTangentatSplinePoint (Variables|Default|GetSpline) (+ _index 1) "Local"))))) 9e+01) (.Yaw (Math|Rotator|BreakRotator (Math|Conversions|RotationFromXVector (.Tangent (Spline|GetLocationandTangentatSplinePoint (Variables|Default|GetSpline) (+ _index 1) "Local"))))))) false false)
      (Transformation|SetRelativeScale3D _returnvalue_2 (Variables|Default|GetEnd%20Mesh%20Scale))
      (Transformation|AddLocalOffset _returnvalue_2 (Variables|Default|GetEnd%20Mesh%20Offset) false false)
      (Transformation|AddLocalRotation _returnvalue_2 (Math|Rotator|MakeRotator _x _y _z) false false))))