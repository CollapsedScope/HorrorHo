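; Spline-based construction Blueprint that lays a cable static mesh along an editable spline.
; The construction script splits the spline into fixed-length sections, scaled by the actor's X scale, and adds a spline mesh component for each.
; Each section takes its start and end from spline distances, with tangents clamped to the section length.
; The event graph has no active logic.
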(event EventBeginPlay)

(event Collision|EventActorBeginOverlap
  (params (OtherActor :type Actor%20Object%20Reference)))

(event EventTick
  (params (DeltaSeconds :type Float%20%28single-precision%29)))

(fn ConstructionScript
  (bind _spline (Variables|Default|GetSpline))
  (bind _spline_2 (Variables|Default|GetSpline))
  (Variables|Default|SetSectionalEngth (* (.x (Transformation|GetActorScale3D)) 10.5))
  (for _index (range 0 (Math|Float|Truncate (/ (Spline|GetSplineLength (Variables|Default|GetSpline)) (Variables|Default|GetSectionalEngth))))
    (bind _returnvalue (AddComponent|AddSplineMeshComponent false))
    (SplineMesh|SetForwardAxis _returnvalue "X" true)
    (Components|StaticMesh|SetStaticMesh _returnvalue "/Game/Art/Eda/MDL/WorkLight/Cable.Cable")
    (SplineMesh|SetStartandEnd _returnvalue (Spline|GetLocationatDistanceAlongSpline _spline_2 (* _index (Variables|Default|GetSectionalEngth)) "Local") (Math|Vector|ClampVectorSize (Spline|GetTangentatDistanceAlongSpline _spline_2 (* _index (Variables|Default|GetSectionalEngth)) "Local") 0.0 (Variables|Default|GetSectionalEngth)) (Spline|GetLocationatDistanceAlongSpline _spline (* (+ _index 1) (Variables|Default|GetSectionalEngth)) "Local") (Math|Vector|ClampVectorSize (Spline|GetTangentatDistanceAlongSpline _spline (* (+ _index 1) (Variables|Default|GetSectionalEngth)) "Local") 0.0 (Variables|Default|GetSectionalEngth)) true :!class /Script/Engine.SplineMeshComponent)))