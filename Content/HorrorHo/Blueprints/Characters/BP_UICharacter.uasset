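; BP_UICharacter is the character for menu levels, showing the title, rule, customize or main menu screen.
; On BeginPlay it creates the widget matching LevelType, adds it to the viewport, shows the cursor and sets Game and UI input focused on it.
; Menu input actions are forwarded to that widget as directional, A and B messages.
; On destruction it restores Game Only input, leaving the cursor visible.
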(event EventBeginPlay
  (bind _returnvalue (Game|GetPlayerController 0))
  (switch Utilities|FlowControl|Switch|SwitchonELevelType (Variables|Default|GetLevelType)
    (:NewEnumerator0
      ;[1 1 1] タイトル
      (bind _returnvalue_2 (UserInterface|CreateWidget "/Game/HorrorHo/Blueprints/Widgets/UI_Title.UI_Title_C"))
      (Variables|Default|SetLevel-SpecificWidget _returnvalue_2))
    (:NewEnumerator1
      ;[1 1 1] ルール画面の表示
      (bind _returnvalue_3 (UserInterface|CreateWidget "/Game/HorrorHo/Blueprints/Widgets/Alpha/UI_Rule.UI_Rule_C"))
      (Variables|Default|SetLevel-SpecificWidget _returnvalue_3))
    (:NewEnumerator2
      ;[1 1 1] カスタマイズ画面の表示
      (bind _returnvalue_4 (UserInterface|CreateWidget "/Game/HorrorHo/Blueprints/Widgets/Menus/UI_Powerup.UI_Powerup_C"))
      (Variables|Default|SetLevel-SpecificWidget _returnvalue_4))
    (:NewEnumerator6
      (bind _returnvalue_5 (UserInterface|CreateWidget "/Game/HorrorHo/Blueprints/Widgets/Menus/UI_MainMenu.UI_MainMenu_C"))
      (Variables|Default|SetLevel-SpecificWidget _returnvalue_5)))
  (UserInterface|Viewport|AddtoViewport (Variables|Default|GetLevel-SpecificWidget) 0)
  (Variables|/Script/Engine.PlayerController|SetbShowMouseCursor _returnvalue true)
  (Input|SetInputModeGameandUI _returnvalue (Variables|Default|GetLevel-SpecificWidget) "DoNotLock" false))

(event EventDestroyed
  (bind _returnvalue (Game|GetPlayerController 0))
  (Variables|/Script/Engine.PlayerController|SetbShowMouseCursor _returnvalue true)
  (Input|SetInputModeGameOnly _returnvalue))

(event Input|ActionEvents|InputActionMenuDown
  (params (Key :type Key%20Structure :default "None"))
  (:Pressed
    (Class|BPIKeyNotify|BPIDown(Message) (Variables|Default|GetLevel-SpecificWidget))))

(event Input|ActionEvents|InputActionMenuChoose
  (params (Key :type Key%20Structure :default "None"))
  (:Pressed
    (Class|BPIKeyNotify|BPIPressA(Message) (Variables|Default|GetLevel-SpecificWidget))))

(event Input|ActionEvents|InputActionMenuLeft
  (params (Key :type Key%20Structure :default "None"))
  (:Pressed
    (Class|BPIKeyNotify|BPILeft(Message) (Variables|Default|GetLevel-SpecificWidget))))

(event Input|ActionEvents|InputActionMenuRight
  (params (Key :type Key%20Structure :default "None"))
  (:Pressed
    (Class|BPIKeyNotify|BPIRight(Message) (Variables|Default|GetLevel-SpecificWidget))))

(event Input|ActionEvents|InputActionMenuUp/Heal
  (params (Key :type Key%20Structure :default "None"))
  (:Pressed
    (Class|BPIKeyNotify|BPIUp(Message) (Variables|Default|GetLevel-SpecificWidget))))

(event Input|ActionEvents|InputActionMenuCancel/Barricade
  (params (Key :type Key%20Structure :default "None"))
  (:Pressed
    (Class|BPIKeyNotify|BPIPressB(Message) (Variables|Default|GetLevel-SpecificWidget))))

(fn ConstructionScript)