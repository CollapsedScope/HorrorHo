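; BP_ZombieBase is a zombie character base that handles damage, death and behavior-tree state.
; AnyDamage feeds the health component and bar widget, then plays a random hit sound or, on death, a splatter, calls the empty InitDeathState and destroys the actor after a delay.
; Interface functions expose movement, player-area entry, transition and death flags plus the spawner, though the IsDead and IsTransitioning getters always return false.
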(event Custom|OnPlayerMovedAway)

(event Game|Damage|EventAnyDamage
  (params (Damage :type Float%20%28single-precision%29) (DamageType :type Damage%20Type%20Object%20Reference) (InstigatedBy :type Controller%20Object%20Reference) (DamageCauser :type Actor%20Object%20Reference))
  ;[1 1 1] Take damage, initiate death behavior if no hp left
  (bind _zero (Default|CalculateHealth (Variables|Default|GetBPC_Health) Damage (UserInterface|GetUserWidgetObject (Variables|Default|GetHealthBar))))
  (if _zero
    (Audio|SpawnSoundatLocation "/Game/HorrorHo/Audio/extra/death_splatter.death_splatter" (Transformation|GetActorLocation) "0, 0, 0" 1.0 1.0 0.0 0 0)
    (if (not (Variables|AIState|GetIsDead))
      (Variables|AIState|SetIsDead true)
      (CallFunction|InitDeathState)
      (Utilities|FlowControl|Delay 5.0)
      (Actor|DestroyActor))
    (else
      (CallFunction|PlayHitSound))))

(event Collision|EventActorBeginOverlap
  (params (OtherActor :type Actor%20Object%20Reference)))

(event EventTick
  (params (DeltaSeconds :type Float%20%28single-precision%29)))

(event EventDestroyed)

(event EventZCharSetCanEnterPlayerArea
  (params (CanEnter :type Boolean))
  ;[1 1 1] Interface Implementation for behavior tree
  (Variables|AIState|SetCanEnterPlayerArea CanEnter))

(event EventZCharSetIsTransitioning
  (params (Is%20Transitioning :type Boolean))
  ;[1 1 1] Interface Implementation for behavior tree
  (Variables|AIState|SetIsTransitioningToPlayerArea Is%20Transitioning))

(event EventZCharSetIsDead
  (params (IsDead :type Boolean))
  ;[1 1 1] Interface Implementation for behavior tree
  (Variables|AIState|SetIsDead IsDead))

(event EventZCharSetIsMoving
  (params (IsMoving :type Boolean))
  ;[1 1 1] Interface Implementation for behavior tree
  (Variables|Animation|SetIsMoving IsMoving))

(fn ConstructionScript
  (|CallParentFunction))

(fn InitDeathState)

(fn PlayHitSound
  (bind _returnvalue (Transformation|GetActorLocation))
  (switch int (Math|Random|RandomInteger 4)
    (:0
      (Audio|PlaySoundatLocation "/Game/HorrorHo/Audio/Body_Flesh_1.Body_Flesh_1" _returnvalue "0, 0, 0" 0.5 1.0 0.0 0 0 0))
    (:1
      (Audio|PlaySoundatLocation "/Game/HorrorHo/Audio/Body_Flesh_2.Body_Flesh_2" _returnvalue "0, 0, 0" 0.5 1.0 0.0 0 0 0))
    (:2
      (Audio|PlaySoundatLocation "/Game/HorrorHo/Audio/Body_Flesh_3.Body_Flesh_3" _returnvalue "0, 0, 0" 0.6 0.8 0.0 0 0 0))
    (:3
      (Audio|PlaySoundatLocation "/Game/HorrorHo/Audio/Body_Flesh_4.Body_Flesh_4" _returnvalue "0, 0, 0" 0.8 0.5 0.0 0 0 0))
    (:4
      (Audio|PlaySoundatLocation "/Game/HorrorHo/Audio/Body_Flesh_5.Body_Flesh_5" _returnvalue "0, 0, 0" 0.6 1.0 0.0 0 0 0))))

(fn ZCharGetCanEnterPlayerArea
  (return (Variables|AIState|GetCanEnterPlayerArea)))

(fn ZCharGetIsDead
  (return false))

(fn ZCharGetIsMoving
  (return (Variables|Animation|GetIsMoving)))

(fn ZCharGetIsTransitioning
  (return false))

(fn ZCharGetSpawner
  (return (Variables|Spawn|GetOriginalSpawner)))

(fn ZCharGetZombieCharacter
  (return self))