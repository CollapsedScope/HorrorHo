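; Base zombie character for a wave-based game, handling health, damage, death, voices and BPI_ZombieBase state accessors.
; Entry through a spawner's window or doorway plays a montage, with a timer moving the zombie along animation curves before registering it as active with the game mode.
; Death stops AI, swaps in dissolve materials, picks a directional animation, updates kill stats and wave count, and may drop ammo, likelier when player ammo is low.
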(event Custom|OnPlayerMovedAway)

(event Custom|Event%20KillSwitch
  (bind _bpc_health (Variables|Default|GetBPC_Health))
  ;[1 1 1] Event to instantly kill the zombie
  (Default|CalculateHealth _bpc_health (Variables|/Game/HorrorHo/Blueprints/Utilities/BPC_Health.BPC_Health_C|GetHealthMax _bpc_health) (UserInterface|GetUserWidgetObject (Variables|Default|GetHealthBar)))
  (Audio|SpawnSoundatLocation "/Game/HorrorHo/Audio/extra/death_splatter.death_splatter" (Transformation|GetActorLocation) "0, 0, 0" 0.5 1.0 0.0 "/Game/HorrorHo/Audio/SA_Barricade.SA_Barricade" 0)
  (CallFunction|InitDeathState 0 false)
  (Utilities|FlowControl|Delay 4.0)
  (Actor|DestroyActor))

(event Game|Damage|EventAnyDamage
  (params (Damage :type Float%20%28single-precision%29) (DamageType :type Damage%20Type%20Object%20Reference) (InstigatedBy :type Controller%20Object%20Reference) (DamageCauser :type Actor%20Object%20Reference))
  ;[1 1 1] Take damage, initiate death behavior if no hp left
  (bind _zero (Default|CalculateHealth (Variables|Default|GetBPC_Health) Damage (UserInterface|GetUserWidgetObject (Variables|Default|GetHealthBar))))
  (if _zero
    (Audio|SpawnSoundatLocation "/Game/HorrorHo/Audio/extra/death_splatter.death_splatter" (Transformation|GetActorLocation) "0, 0, 0" 1.0 1.0 0.0 0 0)
    (if (not (Variables|AIState|GetIsDead))
      (Variables|AIState|SetIsDead true)
      (CallFunction|InitDeathState DamageCauser true DamageType)
      (Utilities|FlowControl|Delay 4.0)
      (Actor|DestroyActor))
    (else
      (CallFunction|PlayHitSound))))

(event Collision|EventActorBeginOverlap
  (params (OtherActor :type Actor%20Object%20Reference)))

(event EventBeginPlay
  (CallFunction|GetDTSettings)
  (bind _returnvalue (Utilities|Time|SetTimerbyEvent (EventDispatchers|CreateEvent :!event QueryVoice) 5.0 true))
  (Variables|Default|SetAudioHandle _returnvalue))

(event EventZCharUpdateNavDist
  (params (RecentDist :type Float%20%28single-precision%29))
  (Variables|Default|SetMostRecentNavDist RecentDist))

(event Collision|EventHit
  (params (MyComp :type Primitive%20Component%20Object%20Reference) (Other :type Actor%20Object%20Reference) (OtherComp :type Primitive%20Component%20Object%20Reference) (bSelfMoved :type Boolean) (HitLocation :type Vector :default "0, 0, 0") (HitNormal :type Vector :default "0, 0, 0") (NormalImpulse :type Vector :default "0, 0, 0") (Hit :type Hit%20Result%20Structure%20%28by%20ref%29))
  ;[1 1 1] ゾンビがお互いをどかす
  (if (and (Utilities|DoesObjectImplementInterface Other "/Game/HorrorHo/Blueprints/Interfaces/BPI_ZombieBase.BPI_ZombieBase_C") (not bSelfMoved))
    (Physics|AddImpulse (Variables|Character|GetCharacterMovement) (* HitNormal 2.5e+04) false)))

(event EventTick
  (params (DeltaSeconds :type Float%20%28single-precision%29)))

(event EventZCharTransitionEvent
  (params (Is%20Transitioning :type Boolean))
  ;[1 1 1] Transition animation and logic
  (Variables|AIState|SetIsTransitioningToPlayerArea Is%20Transitioning)
  (Variables|AIState|SetIsAttacking false)
  (Variables|Animation|SetIsMoving true)
  (bind _newparam (Class|BPISpawner|BPISpawnerGetEntranceType(Message) (Variables|Spawn|GetOriginalSpawner)))
  (CallFunction|SetTransitionSettings)
  (Animation|Montage|PlayMontage (Variables|Character|GetMesh) (Utilities|Select :Index _newparam :NewEnumerator0 (Variables|Default|GetTransition_Window) :NewEnumerator1 (Variables|Default|GetTransition_Door))
    (:then
      (bind _returnvalue (Utilities|Time|SetTimerbyEvent (EventDispatchers|CreateEvent :!event TransitionUpdate) 0.016667 true))
      (Variables|Transition|SetTransitionTimerHandle _returnvalue))))

(event EventZCharKillSwitch
  ;[1 1 1] Event to instantly kill the zombie
  (Utilities|FlowControl|Delay 0.1)
  (CallFunction|EventKillSwitch))

(fn ConstructionScript
  (|CallParentFunction))

(fn InitDeathState
  (params (Instigator :type Actor%20Object%20Reference) (UseDirection :type Boolean) (DamageType :type Damage%20Type%20Object%20Reference))
  (bind _returnvalue (Pawn|GetController))
  (bind _mesh (Variables|Character|GetMesh))
  (bind _returnvalue_2 (AI|GetAIController _returnvalue))
  (Variables|AIState|SetIsDead true)
  (Utilities|FlowControl|Sequence
    (:then_0
      (if (Utilities|Array|IsValidIndex (Variables|Default|GetDissolveMats))
        (CallFunction|SetDissolveMaterials)
        (else
          (Development|PrintString (Utilities|String|Append "Dissolve materials not set properly for " (Utilities|GetDisplayName self)) true true "(R=0.000000,G=0.660000,B=1.000000,A=1.000000)" 5.0))))
    (:then_1
      (if UseDirection
        (CallFunction|CalculateDeathDirection Instigator)))
    (:then_2
      (Collision|SetCollisionEnabled (Variables|Collision|GetCapsuleComponent) "NoCollision")
      (Collision|SetCollisionEnabled _mesh "PhysicsOnly")
      (Collision|SetCollisionResponsetoChannel _mesh "ECC_Pawn" "ECR_Ignore")
      (Pawn|Components|CharacterMovement|DisableMovement (Variables|Character|GetCharacterMovement))
      (if (Variables|AIState|GetIsTransitioningToPlayerArea)
        (Class|BPISpawner|BPISpawnerSetIsBeingUsed(Message) (Variables|Spawn|GetOriginalSpawner) false)))
    (:then_3
      (Utilities|IsValid _returnvalue_2
        (:Is%20Valid
          (AI|Logic|StopLogic (Variables|/Script/AIModule.AIController|GetBrainComponent _returnvalue_2) "")
          (Actor|DestroyActor _returnvalue)
          (Class|Pawn|DetachfromControllerPendingDestroy))))
    (:then_4
      (CallFunction|SpawnAmmo)
      (Audio|Components|Audio|SetSound (Variables|Default|GetVoice) (.OutItem (Utilities|Array|Random (Variables|Default|GetHurtVoices))))
      (Audio|Components|Audio|Play (Variables|Default|GetVoice) 0.0))
    (:then_5
      (bind _damagetype (Class|BPIDamageCategory|BPIDamageCategoryGetType(Message) DamageType))
      (if (Math|Boolean|ORBoolean (Utilities|Enum|Equal(Enum) _damagetype "NewEnumerator0") (Utilities|Enum|Equal(Enum) _damagetype "NewEnumerator1") (Utilities|Enum|Equal(Enum) _damagetype "NewEnumerator2") (Utilities|Enum|Equal(Enum) _damagetype "NewEnumerator3"))
        (bind _type (Class|BPIZombieBase|ZCharGetZombieType(Message) self))
        (Class|BPIGameInstance|BPIGIIncrementStats(Message) (Game|GetGameInstance) true _type (Utilities|Enum|Equal(Enum) _damagetype "NewEnumerator2") false false false false false)))
    (:then_6
      (Class|BPIWavesMode|GMDecrementWaveZombieCount(Message) (Game|GetGameMode)))))

(fn PlayHitSound
  (bind _voice (Variables|Default|GetVoice))
  (Audio|Components|Audio|Stop _voice)
  (Audio|Components|Audio|SetSound _voice (.OutItem (Utilities|Array|Random (Variables|Default|GetHurtVoices))))
  (Audio|Components|Audio|Play _voice 0.0))

(fn SetTransitionSettings
  (bind _returnvalue (Transformation|GetActorLocation))
  (Pawn|Components|CharacterMovement|SetMovementMode (Variables|Character|GetCharacterMovement) "MOVE_None" 0)
  (CallFunction|ToggleCollisionsforTransition "ECR_Ignore")
  (bind (_entervolumetransform _exitvolumetramsform) (Class|BPISpawner|BPISpawnerGetVolumeTransform(Message) (Variables|Spawn|GetOriginalSpawner)))
  (Variables|Transition|SetOriginalPos (Transformation|GetActorLocation))
  (Variables|Transition|SetStartPos (Math|Vector|MakeVector (.x (.location _entervolumetransform)) (.y (.location _entervolumetransform)) (.z _returnvalue)))
  (Variables|Transition|SetEndPos (Math|Vector|MakeVector (.x (.location _exitvolumetramsform)) (.y (.location _exitvolumetramsform)) (.z _returnvalue)))
  (return))

(fn TransitionUpdate
  (bind _mesh (Variables|Character|GetMesh))
  (bind _returnvalue (Components|SkeletalMesh|GetAnimInstance _mesh))
  (bind _returnvalue_2 (Animation|Curves|GetCurveValue _returnvalue "Transition"))
  (bind _returnvalue_3 (Animation|Curves|GetCurveValue _returnvalue "ToStartPosition"))
  (if (Variables|AIState|GetIsDead)
    (Utilities|FlowControl|Sequence
      (:then_0
        (Utilities|Time|ClearandInvalidateTimerbyHandle (Variables|Transition|GetTransitionTimerHandle))
        (Animation|StopAnimMontage 0))
      (:then_1
        (Variables|AIState|SetIsTransitioningToPlayerArea false)
        (Variables|Default|SetIsTransitioned true)
        (Pawn|Components|CharacterMovement|SetMovementMode (Variables|Character|GetCharacterMovement) "MOVE_Walking" 0)
        (CallFunction|ToggleCollisionsforTransition "ECR_Block")))
    (else
      (Utilities|IsValid _returnvalue
        (:Is%20Valid
          (if (< _returnvalue_3 1.0)
            ;[1 1 1] Lerp to entry volume position at start of animation montage
            (Transformation|SetActorLocation (Math|Vector|Lerp(Vector) (Variables|Transition|GetOriginalPos) (Variables|Transition|GetStartPos) _returnvalue_3) false false)
            (bind _entervolumetransform (Class|BPISpawner|BPISpawnerGetVolumeTransform(Message) (Variables|Spawn|GetOriginalSpawner)))
            (Transformation|SetActorRotation (.rotation _entervolumetransform))
            (else
              ;[1 1 1] Lerp inside the player map
              (Transformation|SetActorLocation (+ (Math|Vector|Lerp(Vector) (Variables|Transition|GetStartPos) (Variables|Transition|GetEndPos) _returnvalue_2) (Math|Vector|MakeVector 0.0 0.0 (* (Animation|Curves|GetCurveValue _returnvalue "ZMod") (Variables|Transition|GetClimbHeight)))) true true)
              ;[1 1 1] Finish the transition
              (if (>= _returnvalue_2 0.99)
                (Utilities|FlowControl|Sequence
                  (:then_0
                    (if (Class|KismetMathLibrary|NotEqualExactlyVectorVector (Transformation|GetActorLocation) (Variables|Transition|GetEndPos))
                      (Transformation|SetActorLocation (Variables|Transition|GetEndPos) false true)))
                  (:then_1
                    (Variables|AIState|SetIsTransitioningToPlayerArea false)
                    (Variables|Default|SetIsTransitioned true)
                    (Pawn|Components|CharacterMovement|SetMovementMode (Variables|Character|GetCharacterMovement) "MOVE_Walking" 0)
                    (CallFunction|ToggleCollisionsforTransition "ECR_Block"))
                  (:then_2
                    (Utilities|Time|ClearandInvalidateTimerbyHandle (Variables|Transition|GetTransitionTimerHandle))
                    (Animation|StopAnimMontage 0)
                    (Class|BPIWavesMode|GMAddActiveZombie(Message) (Game|GetGameMode) self)))))))))))

(fn ToggleCollisionsforTransition
  (params (Collision%20Response :type ECollisionResponse%20Enum :default "ECR_Ignore"))
  (Collision|SetCollisionResponsetoChannel (Variables|Collision|GetCapsuleComponent) "ECC_WorldStatic" Collision%20Response)
  (Collision|SetCollisionResponsetoChannel (Variables|Character|GetMesh) "ECC_WorldStatic" Collision%20Response))

(fn GetDTSettings
  (bind _bpc_health (Variables|Default|GetBPC_Health))
  (bind _returnvalue (Utilities|GetDataTableRow "/Game/HorrorHo/Data/DataTable/ZombieParams/DT_WalkerParams.DT_WalkerParams" "Stats")
    (:then
      (bind _output_get (Variables|/Game/HorrorHo/Blueprints/Utilities/BPC_Health.BPC_Health_C|SetHealthMax _bpc_health (.Health (Utilities|Struct|BreakStruct_WalkerParams _returnvalue))))
      (Variables|/Game/HorrorHo/Blueprints/Utilities/BPC_Health.BPC_Health_C|SetHealth _bpc_health _output_get))))

(fn SetDissolveMaterials
  (if (== (Utilities|Array|Length (Rendering|Material|GetMaterials (Variables|Character|GetMesh))) (Utilities|Array|Length (Variables|Default|GetDissolveMats)))
    (for (_array_element _array_index) (Variables|Default|GetDissolveMats)
      (bind _returnvalue (Rendering|Material|CreateDynamicMaterialInstance _array_element "None" "None" :!class /Script/Engine.KismetMaterialLibrary))
      (Rendering|Material|SetMaterial (Variables|Character|GetMesh) _array_index _returnvalue)
      (Rendering|Material|SetScalarParameterValue _returnvalue "HitTime" (Utilities|Time|GetGameTimeinSeconds) :!class /Script/Engine.MaterialInstanceDynamic))
    (else
      (Development|PrintString (Utilities|String|Append (Utilities|GetDisplayName self) " does not have the correct number of dissolve materials")))))

(fn SpawnAmmo
  ;[1 1 1] プレイヤーが行ける距離以内の場合のみアイテムを出現する
  (if (Variables|Default|GetIsTransitioned)
    (bind (_ammocountinmagazine _ammoowned) (Class|BPIPlayer|BPIPlayerGetPlayersAmmoState(Message) (Game|Player|GetPlayerPawn 0)))
    (if (<= (Math|Random|RandomFloatinRange 0.0 1.0) (Math|Float|Lerp (Variables|AmmoDrop|GetAmmoDropChanceDefault) 1.0 (Math|Float|Clamp(Float) (/ (Math|Conversions|ToFloat(Integer) (Variables|AmmoDrop|GetDropChanceIncreaseThreshold)) (Math|Conversions|ToFloat(Integer) (+ _ammocountinmagazine _ammoowned))))))
      (Game|SpawnActorfromClass "/Game/HorrorHo/Blueprints/Actors/Props/BP_AmmoBox.BP_AmmoBox_C" (Transformation|GetWorldTransform (Variables|Character|GetMesh)) "Undefined" 0 0))))

(fn CalculateDeathDirection
  (params (Instigator :type Actor%20Object%20Reference))
  (bind _returnvalue (Transformation|GetActorLocation Instigator))
  (bind _returnvalue_2 (Transformation|GetActorLocation))
  (bind _mesh (Variables|Character|GetMesh))
  (bind _returnvalue_3 (Components|SkeletalMesh|GetAnimInstance _mesh))
  (Utilities|IsValid Instigator
    (:Is%20Valid
      (if (< (Math|Vector|DotProduct (Transformation|GetActorForwardVector) (- (Math|Vector|MakeVector (.x _returnvalue) (.y _returnvalue) 0.0) (Math|Vector|MakeVector (.x _returnvalue_2) (.y _returnvalue_2) 0.0))) 0.0)
        (Class|BPIZombieAnim|SetDeathAnimation(Message) _returnvalue_3 "NewEnumerator0")
        (else
          (Class|BPIZombieAnim|SetDeathAnimation(Message) _returnvalue_3 "NewEnumerator1"))))))

(fn QueryVoice
  (if (not (Variables|AIState|GetIsDead))
    (switch Utilities|FlowControl|Switch|SwitchonEAudioComponentPlayState (Audio|Components|Audio|GetPlayState (Variables|Default|GetVoice))
      (:Stopped
        _)
      (:FadingOut
        _))
    (Audio|Components|Audio|SetSound (Variables|Default|GetVoice) (.OutItem (Utilities|Array|Random (Variables|Default|GetAmbientVoices))))
    (Audio|Components|Audio|Play (Variables|Default|GetVoice) 0.0)))

(fn BPIGetSocketLocation
  (params (Socket%20Name :type Name :default "None"))
  (return (Transformation|GetSocketLocation (Variables|Character|GetMesh) Socket%20Name)))

(fn ZCharAttackCommand
  (return (Variables|AIState|GetAttackCommand)))

(fn ZCharCanEnterPlayerArea
  (return (Variables|AIState|GetCanEnterPlayerArea)))

(fn ZCharGetMostRecentNavDist
  (return (Variables|Default|GetMostRecentNavDist)))

(fn ZCharGetSpawner
  (return (Variables|Spawn|GetOriginalSpawner)))

(fn ZCharGetZombieCharacter
  (return self))

(fn ZCharGetZombieType
  (return "NewEnumerator0"))

(fn ZCharIsAttacking
  (return (Variables|AIState|GetIsAttacking)))

(fn ZCharIsDead
  (return (Variables|AIState|GetIsDead)))

(fn ZCharIsMoving
  (return (Variables|Animation|GetIsMoving)))

(fn ZCharIsTransitioning
  (return (Variables|AIState|GetIsTransitioningToPlayerArea)))

(fn ZCharSetAttackCommand
  (params (NewAttackCommand :type Boolean))
  (bind _output_get (Variables|AIState|SetAttackCommand NewAttackCommand))
  (return _output_get))

(fn ZCharSetCanEnterPlayerArea
  (params (CanEnter :type Boolean))
  (bind _output_get (Variables|AIState|SetCanEnterPlayerArea CanEnter))
  (return _output_get))

(fn ZCharSetIsAttacking
  (params (IsAttacking :type Boolean))
  (bind _output_get (Variables|AIState|SetIsAttacking IsAttacking))
  (return _output_get))

(fn ZCharSetIsDead
  (params (IsDead :type Boolean))
  (bind _output_get (Variables|AIState|SetIsDead IsDead))
  (return _output_get))

(fn ZCharSetIsMoving
  (params (IsMoving :type Boolean))
  (bind _output_get (Variables|Animation|SetIsMoving IsMoving))
  (return _output_get))

(fn ZCharSetSpawnerReference
  (params (Original%20Spawner :type Actor%20Object%20Reference))
  (bind _output_get (Variables|Spawn|SetOriginalSpawner Original%20Spawner))
  (return _output_get))

(fn ZCharSetZombieAppearance
  (params (SkeletalMesh :type Skeletal%20Mesh%20Object%20Reference) (DissolveMaterials :type Array%20of%20Material%20Interface%20Object%20References))
  (Class|SkinnedMeshComponent|SetSkeletalMesh (Variables|Character|GetMesh) SkeletalMesh false)
  (Utilities|Array|Clear (Variables|Default|GetDissolveMats))
  (Variables|Default|SetDissolveMats DissolveMaterials)
  (return true))