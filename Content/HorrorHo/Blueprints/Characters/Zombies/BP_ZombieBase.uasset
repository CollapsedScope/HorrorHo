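; Base zombie character that takes damage, climbs through window or doorway entrances into the player area, and dies.
; Exposes state to the behavior tree through an interface and loads health from DT_WalkerParams.
; Entrance montage curves drive timer-updated movement between spawner volumes, then register the zombie with the game mode.
; Death picks a directional animation, stops AI, and, after entry, may drop ammo, likelier when the player runs low.
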(event Custom|OnPlayerMovedAway)

(event Custom|Event%20KillSwitch
  (bind _bpc_health (Variables|Default|GetBPC_Health))
  ;[1 1 1] Event to instantly kill the zombie
  (Default|CalculateHealth _bpc_health (Variables|/Game/HorrorHo/Blueprints/Components/BPC_Health.BPC_Health_C|GetHealthMax _bpc_health) (UserInterface|GetUserWidgetObject (Variables|Default|GetHealthBar)))
  (Audio|SpawnSoundatLocation "/Game/HorrorHo/Audio/extra/death_splatter.death_splatter" (Transformation|GetActorLocation) "0, 0, 0" 0.5 1.0 0.0 "/Game/HorrorHo/Audio/SA_Barricade.SA_Barricade" 0)
  (Variables|AIState|SetIsDead true)
  (CallFunction|InitDeathState)
  (Utilities|FlowControl|Delay 4.0)
  (Actor|DestroyActor))

(event Game|Damage|EventAnyDamage
  (params (Damage :type Float%20%28single-precision%29) (DamageType :type Damage%20Type%20Object%20Reference) (InstigatedBy :type Controller%20Object%20Reference) (DamageCauser :type Actor%20Object%20Reference))
  ;[1 1 1] Take damage, initiate death behavior if no hp left
  (bind _zero (Default|CalculateHealth (Variables|Default|GetBPC_Health) Damage (UserInterface|GetUserWidgetObject (Variables|Default|GetHealthBar))))
  (if _zero
    (Audio|SpawnSoundatLocation "/Game/HorrorHo/Audio/extra/death_splatter.death_splatter" (Transformation|GetActorLocation) "0, 0, 0" 1.0 1.0 0.0 0 0)
    (if (not (Variables|AIState|GetIsDead))
      (Variables|AIState|SetIsDead true)
      (CallFunction|InitDeathState DamageCauser)
      (Utilities|FlowControl|Delay 4.0)
      (Actor|DestroyActor))
    (else
      (CallFunction|PlayHitSound))))

(event Collision|EventActorBeginOverlap
  (params (OtherActor :type Actor%20Object%20Reference)))

(event EventBeginPlay
  (CallFunction|GetDTSettings))

(event Collision|EventHit
  (params (MyComp :type Primitive%20Component%20Object%20Reference) (Other :type Actor%20Object%20Reference) (OtherComp :type Primitive%20Component%20Object%20Reference) (bSelfMoved :type Boolean) (HitLocation :type Vector :default "0, 0, 0") (HitNormal :type Vector :default "0, 0, 0") (NormalImpulse :type Vector :default "0, 0, 0") (Hit :type Hit%20Result%20Structure%20%28by%20ref%29))
  ;[1 1 1] ゾンビがお互いをどかす
  (if (and (Utilities|DoesObjectImplementInterface Other "/Game/HorrorHo/Blueprints/Interfaces/BPI_ZombieBase.BPI_ZombieBase_C") (not bSelfMoved))
    (Physics|AddImpulse (Variables|Character|GetCharacterMovement) (* HitNormal 2.5e+04) false)))

(event EventTick
  (params (DeltaSeconds :type Float%20%28single-precision%29)))

(event EventDestroyed)

(event EventZCharSetCanEnterPlayerArea
  (params (CanEnter :type Boolean))
  ;[1 1 1] Interface Implementation for behavior tree
  (Variables|AIState|SetCanEnterPlayerArea CanEnter))

(event EventZCharTransitionEvent
  (params (Is%20Transitioning :type Boolean))
  ;[1 1 1] Transition animation and logic
  (Variables|AIState|SetIsTransitioningToPlayerArea Is%20Transitioning)
  (Variables|AIState|SetIsAttacking false)
  (Variables|Animation|SetIsMoving true)
  (CallFunction|SetTransitionSettings)
  (Animation|Montage|PlayMontage (Variables|Character|GetMesh) (Utilities|Select :Index (Variables|/Game/HorrorHo/Blueprints/Actors/Installation/BP_Spawner.BP_Spawner_C|GetEntranceType (Variables|Spawn|GetOriginalSpawner)) :NewEnumerator0 (Variables|Default|GetTransition_Window) :NewEnumerator1 (Variables|Default|GetTransition_Door))
    (:then
      (bind _returnvalue (Utilities|Time|SetTimerbyEvent (EventDispatchers|CreateEvent :!event TransitionUpdate) 0.016667 true))
      (Variables|Transition|SetTransitionTimerHandle _returnvalue))))

(event EventZCharSetIsDead
  (params (IsDead :type Boolean))
  ;[1 1 1] Interface Implementation for behavior tree
  (Variables|AIState|SetIsDead IsDead))

(event EventZCharSetIsMoving
  (params (IsMoving :type Boolean))
  ;[1 1 1] Interface Implementation for behavior tree
  (Variables|Animation|SetIsMoving IsMoving))

(event EventZCharSetIsAttacking
  (params (IsAttacking :type Boolean))
  ;[1 1 1] Interface Implementation for behavior tree
  (Variables|AIState|SetIsAttacking IsAttacking))

(event EventZCharKillSwitch
  ;[1 1 1] Event to instantly kill the zombie
  (CallFunction|EventKillSwitch))

(fn ConstructionScript
  (|CallParentFunction))

(fn InitDeathState
  (params (Instigator :type Actor%20Object%20Reference))
  (bind _returnvalue (Transformation|GetActorLocation Instigator))
  (bind _returnvalue_2 (Pawn|GetController))
  (bind _returnvalue_3 (Transformation|GetActorLocation))
  (bind _mesh (Variables|Character|GetMesh))
  (bind _returnvalue_4 (Components|SkeletalMesh|GetAnimInstance _mesh))
  (Utilities|FlowControl|Sequence
    (:then_0
      ;[1 1 1] Calculate death animation from direction
      (Utilities|IsValid Instigator
        (:Is%20Valid
          (if (< (Math|Vector|DotProduct (Transformation|GetActorForwardVector) (- (Math|Vector|MakeVector (.x _returnvalue) (.y _returnvalue) 0.0) (Math|Vector|MakeVector (.x _returnvalue_3) (.y _returnvalue_3) 0.0))) 0.0)
            (Class|BPIZombieAnim|SetDeathAnimation(Message) _returnvalue_4 "NewEnumerator0")
            (else
              (Class|BPIZombieAnim|SetDeathAnimation(Message) _returnvalue_4 "NewEnumerator1"))))))
    (:then_1
      (Collision|SetCollisionEnabled (Variables|Collision|GetCapsuleComponent) "NoCollision")
      (Collision|SetCollisionEnabled (Variables|Character|GetMesh) "NoCollision")
      (if (Variables|AIState|GetIsTransitioningToPlayerArea)
        (Variables|/Game/HorrorHo/Blueprints/Actors/Installation/BP_Spawner.BP_Spawner_C|SetIsBeingUsed (Variables|Spawn|GetOriginalSpawner) false)))
    (:then_2
      (bind _zombiecontroller (Class|BPIZombieController|ZConGetZombieController(Message) _returnvalue_2))
      (AI|Logic|StopLogic (Variables|/Script/AIModule.AIController|GetBrainComponent _zombiecontroller) "")
      (Actor|DestroyActor _returnvalue_2)
      (Class|Pawn|DetachfromControllerPendingDestroy)
      (Pawn|Components|CharacterMovement|SetMovementMode (Variables|Character|GetCharacterMovement) "MOVE_None" 0))
    (:then_3
      ;[1 1 1] プレイヤーが行ける距離以内の場合のみアイテムを出現する
      (if (Variables|Default|GetIsTransitioned)
        (bind (_ammocountinmagazine _ammoowned) (Class|BPIPlayer|BPIGetPlayersAmmoState(Message) (Game|Player|GetPlayerPawn 0)))
        (if (<= (Math|Random|RandomFloatinRange 0.0 1.0) (Math|Float|Lerp (Variables|AmmoDrop|GetAmmoDropChanceDefault) 1.0 (Math|Float|Clamp(Float) (/ (Math|Conversions|ToFloat(Integer) (Variables|AmmoDrop|GetDropChanceIncreaseThreshold)) (Math|Conversions|ToFloat(Integer) (+ _ammocountinmagazine _ammoowned))))))
          (Game|SpawnActorfromClass "/Game/HorrorHo/Blueprints/Actors/Props/BP_AmmoBox.BP_AmmoBox_C" (Transformation|GetWorldTransform (Variables|Character|GetMesh)) "Undefined" 0 0))))))

(fn PlayHitSound
  (bind _returnvalue (Transformation|GetActorLocation))
  (switch int (Math|Random|RandomInteger 4)
    (:0
      (Audio|PlaySoundatLocation 0 _returnvalue "0, 0, 0" 0.5 1.0 0.0 0 0 0))
    (:1
      (Audio|PlaySoundatLocation 0 _returnvalue "0, 0, 0" 0.5 1.0 0.0 0 0 0))
    (:2
      (Audio|PlaySoundatLocation 0 _returnvalue "0, 0, 0" 0.6 0.8 0.0 0 0 0))
    (:3
      (Audio|PlaySoundatLocation 0 _returnvalue "0, 0, 0" 0.8 0.5 0.0 0 0 0))
    (:4
      (Audio|PlaySoundatLocation 0 _returnvalue "0, 0, 0" 0.6 1.0 0.0 0 0 0))))

(fn SetTransitionSettings
  (bind _returnvalue (Transformation|GetActorLocation))
  (bind _originalspawner (Variables|Spawn|GetOriginalSpawner))
  (bind _entervolume (Variables|/Game/HorrorHo/Blueprints/Actors/Installation/BP_Spawner.BP_Spawner_C|GetEnterVolume _originalspawner))
  (bind _exitvolume (Variables|/Game/HorrorHo/Blueprints/Actors/Installation/BP_Spawner.BP_Spawner_C|GetExitVolume _originalspawner))
  (bind _returnvalue_2 (Transformation|GetWorldLocation _entervolume))
  (bind _returnvalue_3 (Transformation|GetWorldLocation _exitvolume))
  (Pawn|Components|CharacterMovement|SetMovementMode (Variables|Character|GetCharacterMovement) "MOVE_None" 0)
  (CallFunction|ToggleCollisionsforTransition "ECR_Ignore")
  (Variables|Transition|SetOriginalPos (Transformation|GetActorLocation))
  (Variables|Transition|SetStartPos (Math|Vector|MakeVector (.x _returnvalue_2) (.y _returnvalue_2) (.z _returnvalue)))
  (Variables|Transition|SetEndPos (Math|Vector|MakeVector (.x _returnvalue_3) (.y _returnvalue_3) (.z _returnvalue)))
  (return))

(fn TransitionUpdate
  (bind _mesh (Variables|Character|GetMesh))
  (bind _returnvalue (Components|SkeletalMesh|GetAnimInstance _mesh))
  (bind _returnvalue_2 (Animation|Curves|GetCurveValue _returnvalue "Transition"))
  (bind _returnvalue_3 (Animation|Curves|GetCurveValue _returnvalue "ToStartPosition"))
  (if (< _returnvalue_3 1.0)
    ;[1 1 1] Lerp to entry volume position at start of animation montage
    (Transformation|SetActorLocation (Math|Vector|Lerp(Vector) (Variables|Transition|GetOriginalPos) (Variables|Transition|GetStartPos) _returnvalue_3) false false)
    (Transformation|SetActorRotation (Transformation|GetWorldRotation (Variables|/Game/HorrorHo/Blueprints/Actors/Installation/BP_Spawner.BP_Spawner_C|GetEnterVolume (Variables|Spawn|GetOriginalSpawner))))
    (else
      ;[1 1 1] Lerp inside the player map
      (Transformation|SetActorLocation (+ (Math|Vector|Lerp(Vector) (Variables|Transition|GetStartPos) (Variables|Transition|GetEndPos) _returnvalue_2) (Math|Vector|MakeVector 0.0 0.0 (* (Animation|Curves|GetCurveValue _returnvalue "ZMod") (Variables|Transition|GetClimbHeight)))) true true)
      ;[1 1 1] Finish the transition
      (if (>= _returnvalue_2 0.99)
        (Utilities|FlowControl|Sequence
          (:then_0
            (Variables|AIState|SetIsTransitioningToPlayerArea false)
            (Variables|Default|SetIsTransitioned true)
            (Pawn|Components|CharacterMovement|SetMovementMode (Variables|Character|GetCharacterMovement) "MOVE_Walking" 0)
            (CallFunction|ToggleCollisionsforTransition "ECR_Block"))
          (:then_1
            (Utilities|Time|ClearandInvalidateTimerbyHandle (Variables|Transition|GetTransitionTimerHandle))
            (Animation|StopAnimMontage 0)
            (Class|BPIWavesMode|GMAddActiveZombie(Message) (Game|GetGameMode) self)))))))

(fn ToggleCollisionsforTransition
  (params (Collision%20Response :type ECollisionResponse%20Enum :default "ECR_Ignore"))
  (Collision|SetCollisionResponsetoChannel (Variables|Collision|GetCapsuleComponent) "ECC_WorldStatic" Collision%20Response)
  (Collision|SetCollisionResponsetoChannel (Variables|Character|GetMesh) "ECC_WorldStatic" Collision%20Response))

(fn GetDTSettings
  (bind _bpc_health (Variables|Default|GetBPC_Health))
  (bind _returnvalue (Utilities|GetDataTableRow "/Game/HorrorHo/Data/DataTable/ZombieParams/DT_WalkerParams.DT_WalkerParams" "Stats")
    (:then
      (bind _output_get (Variables|/Game/HorrorHo/Blueprints/Components/BPC_Health.BPC_Health_C|SetHealthMax _bpc_health (.Health (Utilities|Struct|BreakStruct_WalkerParams _returnvalue))))
      (Variables|/Game/HorrorHo/Blueprints/Components/BPC_Health.BPC_Health_C|SetHealth _bpc_health _output_get))))

(fn ZCharGetAttackCommand
  (return (Variables|AIState|GetAttackCommand)))

(fn ZCharGetCanEnterPlayerArea
  (return (Variables|AIState|GetCanEnterPlayerArea)))

(fn ZCharGetIsAttacking
  (return (Variables|AIState|GetIsAttacking)))

(fn ZCharGetIsDead
  (return false))

(fn ZCharGetIsMoving
  (return (Variables|Animation|GetIsMoving)))

(fn ZCharGetIsTransitioning
  (return false))

(fn ZCharGetSpawner
  (return (Variables|Spawn|GetOriginalSpawner)))

(fn ZCharGetZombieCharacter
  (return self))