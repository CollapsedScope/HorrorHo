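; Bomber zombie that explodes on death, damaging the player, its spawner's barricade and nearby zombies within a sphere, then destroys itself.
; BeginPlay loads health, damage and radius from DT_BomberParams, but sizes the sphere before that load.
; Tick drives a heartbeat sound whose interval, volume and pitch follow the animation's ExplodeCurve as a warning.
; Zombies take directional point damage typed as BP_ExplosionDamage.
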(event EventBeginPlay
  (Components|Sphere|SetSphereRadius (Variables|Default|GetExplosion%20Range) (Variables|Default|GetExposion%20Radius) true)
  (CallFunction|GetDTSettings))

(event Collision|EventActorBeginOverlap
  (params (OtherActor :type Actor%20Object%20Reference))
  (|CallParentFunction OtherActor) ; This node is disabled and will not be called.\nDrag off pins to build functionality.
)

(event EventTick
  (params (DeltaSeconds :type Float%20%28single-precision%29))
  (|CallParentFunction DeltaSeconds)
  (CallFunction|Heartbeat DeltaSeconds))

(event EventZCharExplode
  (bind _returnvalue (Game|Player|GetPlayerPawn 0))
  (bind _originalspawner (Variables|Default|GetOriginalSpawner))
  (Utilities|FlowControl|Sequence
    (:then_0
      ;[1 1 1] Damage player
      (if (Collision|IsOverlappingActor (Variables|Default|GetExplosion%20Range) _returnvalue :!class /Script/Engine.PrimitiveComponent)
        (Game|Damage|ApplyDamage _returnvalue (Variables|Default|GetDamageToPlayer) (Pawn|GetController) self)))
    (:then_1
      ;[1 1 1] Damage barricade
      (if (Collision|IsOverlappingActor (Variables|Default|GetExplosion%20Range) _originalspawner :!class /Script/Engine.PrimitiveComponent)
        (Class|BPISpawner|BPISpawnerAdjustHealth(Message) _originalspawner (* (Variables|Default|GetDamageToBarricade) -1))))
    (:then_2
      ;[1 1 1] Damage zombies
      (for _array_element (Collision|GetOverlappingActors (Variables|Default|GetExplosion%20Range) "/Game/HorrorHo/Blueprints/Characters/Zombies/BP_ZombieBase.BP_ZombieBase_C" :!class /Script/Engine.PrimitiveComponent)
        (Game|Damage|ApplyPointDamage _array_element (Variables|Default|GetDamageToZombies) (Math|Vector|Normalize (- (Transformation|GetActorLocation _array_element) (Transformation|GetActorLocation))) (Collision|MakeHitResult false false 0.0 0.0 "0, 0, 0" "0, 0, 0" "0,0,1" "0,0,1" 0 0) (Pawn|GetController) self "/Game/HorrorHo/Blueprints/Utilities/DamageType/BP_ExplosionDamage.BP_ExplosionDamage_C")))
    (:then_3
      ;[1 1 1] Play sound, make emitter, die
      (Audio|PlaySoundatLocation "/Game/HorrorHo/Audio/HeadShot/HeadShot.HeadShot" (Transformation|GetActorLocation) "0, 0, 0" 3e+01 0.3 0.0 "/Game/HorrorHo/Audio/SA_BomberExplosion.SA_BomberExplosion" 0 0)
      (Effects|SpawnEmitteratLocation "/Game/Art/Eda/Fx/Pt_BldExplosition.Pt_BldExplosition" (- (Transformation|GetActorLocation) (Math|Vector|MakeVector 0.0 0.0 96.0)) "0, 0, 0" "1.500000,1.500000,1.500000")
      (Actor|DestroyActor))))

(event EventAnyDamage
  (params (Damage :type Float%20%28single-precision%29) (DamageType :type Damage%20Type%20Object%20Reference) (InstigatedBy :type Controller%20Object%20Reference) (DamageCauser :type Actor%20Object%20Reference))
  (|CallParentFunction Damage DamageType InstigatedBy DamageCauser)
  (if (<= (Variables|/Game/HorrorHo/Blueprints/Utilities/BPC_Health.BPC_Health_C|GetHealth (Variables|Default|GetBPC_Health)) 0.0)
    (CallFunction|ZCharExplode)))

(fn ConstructionScript
  (|CallParentFunction))

(fn ZCharGetZombieType
  (return "NewEnumerator3"))

(fn Heartbeat
  (params (DeltaSeconds :type Float%20%28single-precision%29))
  (bind _mesh (Variables|Character|GetMesh))
  (bind _returnvalue (Components|SkeletalMesh|GetAnimInstance _mesh))
  (bind _returnvalue_2 (Animation|Curves|GetCurveValue _returnvalue "ExplodeCurve"))
  (bind _output_get (Variables|Default|SetHeartbeatTimer (- (Variables|Default|GetHeartbeatTimer) DeltaSeconds)))
  (if (<= _output_get 0.0)
    (Utilities|FlowControl|Sequence
      (:then_0
        (Audio|PlaySoundatLocation "/Game/HorrorHo/Audio/Waves/heartbeat.heartbeat" (Transformation|GetActorLocation) "0, 0, 0" (+ (Math|Float|Lerp 0.0 2e+01 (Variables|Default|GetHeartbeatAlpha)) 5.0) (+ (Math|Float|Lerp 0.0 1e+02 (Variables|Default|GetHeartbeatAlpha)) 1.0) 0.0 "/Game/HorrorHo/Audio/SA_BomberExplosion.SA_BomberExplosion" 0 0))
      (:then_1
        (if (Math|Conversions|ToBoolean(Integer) (Utilities|Array|Length (Class|AnimInstance|GetActiveCurveNames _returnvalue "AttributeCurve")))
          (Variables|Default|SetHeartbeatTimer (Math|Float|Lerp 0.5 (Variables|Default|GetHeartbeatTimerMin) _returnvalue_2))
          (Variables|Default|SetHeartbeatAlpha _returnvalue_2)
          (else
            (Variables|Default|SetHeartbeatTimer (Variables|Default|GetHeartbeatTimerMax))))))))

(fn GetDTSettings
  (bind _bpc_health (Variables|Default|GetBPC_Health))
  (bind _returnvalue (Utilities|GetDataTableRow "/Game/HorrorHo/Data/DataTable/ZombieParams/DT_BomberParams.DT_BomberParams" "Stats")
    (:then
      (Utilities|FlowControl|Sequence
        (:then_0
          (bind _output_get (Variables|/Game/HorrorHo/Blueprints/Utilities/BPC_Health.BPC_Health_C|SetHealthMax _bpc_health (.Health (Utilities|Struct|BreakStruct_BomberParams _returnvalue))))
          (Variables|/Game/HorrorHo/Blueprints/Utilities/BPC_Health.BPC_Health_C|SetHealth _bpc_health _output_get))
        (:then_1
          (Variables|Default|SetDamageToPlayer (.DamageToPlayer (Utilities|Struct|BreakStruct_BomberParams _returnvalue))))
        (:then_2
          (Variables|Default|SetDamageToBarricade (.DamageToBarricade (Utilities|Struct|BreakStruct_BomberParams _returnvalue))))
        (:then_3
          (Variables|Default|SetDamageToZombies (.DamageToZombies (Utilities|Struct|BreakStruct_BomberParams _returnvalue))))
        (:then_4
          (Variables|Default|SetExposion%20Radius (.ExplosionRadius (Utilities|Struct|BreakStruct_BomberParams _returnvalue))))))))