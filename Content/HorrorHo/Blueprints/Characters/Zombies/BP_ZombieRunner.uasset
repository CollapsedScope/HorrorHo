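; BP_ZombieRunner is a runner zombie character whose health and movement speed are driven by a data table.
; On BeginPlay it reads the "Stats" row of DT_RunnerParams through GetDTSettings.
; The row sets BPCHealth's maximum health, fills current health to that maximum, and sets CharacterMovement's max walk speed.
; It defines no other behavior of its own, and a missing row leaves those values untouched.
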(event EventBeginPlay
  (CallFunction|GetDTSettings))

(event Collision|EventActorBeginOverlap
  (params (OtherActor :type Actor%20Object%20Reference))
  (|CallParentFunction OtherActor) ; This node is disabled and will not be called.\nDrag off pins to build functionality.
)

(event EventTick
  (params (DeltaSeconds :type Float%20%28single-precision%29))
  (|CallParentFunction DeltaSeconds) ; This node is disabled and will not be called.\nDrag off pins to build functionality.
)

(fn ConstructionScript
  (|CallParentFunction))

(fn GetDTSettings
  (bind _bpc_health (Variables|Default|GetBPC_Health))
  (bind _returnvalue (Utilities|GetDataTableRow "/Game/HorrorHo/Data/DataTable/ZombieParams/DT_RunnerParams.DT_RunnerParams" "Stats")
    (:then
      (bind _output_get (Variables|/Game/HorrorHo/Blueprints/Components/BPC_Health.BPC_Health_C|SetHealthMax _bpc_health (.Health (Utilities|Struct|BreakStruct_RunnerParams _returnvalue))))
      (Variables|/Game/HorrorHo/Blueprints/Components/BPC_Health.BPC_Health_C|SetHealth _bpc_health _output_get)
      (Variables|/Script/Engine.CharacterMovementComponent|SetMaxWalkSpeed (Variables|Character|GetCharacterMovement) (.MoveSpeed (Utilities|Struct|BreakStruct_RunnerParams _returnvalue))))))