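; BP_ZombieTutorial is a tutorial zombie character that walks toward a window and dies when it takes any damage.
; A looping timer, set in the construction script at about 60 Hz, appears to drive the Move event in place of Tick.
; Move caches the first actor tagged "Window", then applies scaled-down, forced movement input toward it.
; AnyDamage only sets IsDead on the BP_Anm_TutorialWalker animation instance, without stopping movement.
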(event Custom|Move
  (Utilities|IsValid (Variables|Default|GetWindowSign)
    (:Is%20Valid
      (Pawn|Input|AddMovementInput (* (Math|Vector|Normalize (- (Transformation|GetActorLocation (Variables|Default|GetWindowSign)) (Transformation|GetActorLocation))) 0.1) 1.0 true))
    (:Is%20Not%20Valid
      (bind _outactors (Actor|GetAllActorswithTag "Window"))
      (Utilities|IsValid (Utilities|Array|Get(acopy) _outactors)
        (:Is%20Valid
          (Variables|Default|SetWindowSign (Utilities|Array|Get(acopy) _outactors)))))))

(event EventBeginPlay)

(event Collision|EventActorBeginOverlap
  (params (OtherActor :type Actor%20Object%20Reference)))

(event EventTick
  (params (DeltaSeconds :type Float%20%28single-precision%29)))

(event Game|Damage|EventAnyDamage
  (params (Damage :type Float%20%28single-precision%29) (DamageType :type Damage%20Type%20Object%20Reference) (InstigatedBy :type Controller%20Object%20Reference) (DamageCauser :type Actor%20Object%20Reference))
  (bind _asbp_anm_tutorial_walker (Utilities|Casting|CastToBP_Anm_TutorialWalker (Components|SkeletalMesh|GetAnimInstance (Variables|Character|GetMesh))))
  (Variables|/Game/HorrorHo/Animations/Walker/BP_Anm_TutorialWalker.BP_Anm_TutorialWalker_C|SetIsDead _asbp_anm_tutorial_walker true))

(fn ConstructionScript
  (Utilities|Time|SetTimerbyEvent (EventDispatchers|CreateEvent :!event Custom|Move) 0.016666 true))