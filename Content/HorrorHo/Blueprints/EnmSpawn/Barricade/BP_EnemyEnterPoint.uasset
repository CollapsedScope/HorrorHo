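; BP_EnemyEnterPoint is a barricaded enemy entry point that loses planks as it takes damage.
; BeginPlay spawns piece actors stacked vertically across BarricadeVolume with random pitch, then shuffles them so they disappear in random order.
; AdjustHealth plays particles and sound, clamps health, hides pieces by health fraction and returns whether the barricade is destroyed.
; It handles damage only: non-negative changes also return true and pieces are never re-shown.
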(event EventBeginPlay
  (Variables|Barricade|SetBarricadeHealth (Variables|Barricade|GetMaxBarricadeHealth))
  (Variables|Barricade|SetBarricadePieceHealthThreshold (/ 1.0 (Math|Conversions|ToFloat(Integer) (+ (Variables|Barricade|GetBarricadePieceCount) 1))))
  (Variables|Default|SetLivePieceCount (Variables|Barricade|GetBarricadePieceCount))
  (CallFunction|CreateBarricadePieces))

(event Collision|EventActorBeginOverlap
  (params (OtherActor :type Actor%20Object%20Reference)))

(event EventTick
  (params (DeltaSeconds :type Float%20%28single-precision%29)))

(fn ConstructionScript)

(fn AdjustHealth
  (params (ChangeAmount :type Integer))
  (bind _returnvalue (< ChangeAmount 0))
  (if (and _returnvalue (> (Variables|Barricade|GetBarricadeHealth) 0))
    (if _returnvalue
      (CallFunction|SpawnParticlesandSound))
    ;[1 1 1] Change health value within clamp
    (Variables|Barricade|SetBarricadeHealth (Math|Integer|Clamp(Integer) (+ (Variables|Barricade|GetBarricadeHealth) ChangeAmount) 0 (Variables|Barricade|GetMaxBarricadeHealth)))
    ;[1 1 1] Check if the number of remaining pieces has changed
    (bind _output_get (LocalVariables|SetNewLivePieceCount (Math|Float|Ceil (/ (/ (Math|Conversions|ToFloat(Integer) (Variables|Barricade|GetBarricadeHealth)) (Math|Conversions|ToFloat(Integer) (Variables|Barricade|GetMaxBarricadeHealth))) (Variables|Barricade|GetBarricadePieceHealthThreshold)))))
    (if (!= _output_get (Variables|Default|GetLivePieceCount))
      (Variables|Default|SetLivePieceCount (LocalVariables|GetNewLivePieceCount))
      (CallFunction|SetBarricadePieceVisibility)
      (return (<= (Variables|Barricade|GetBarricadeHealth) 0))
      (else
        ;[1 1 1] If no change, return
        (return (<= (Variables|Barricade|GetBarricadeHealth) 0))))
    (else
      ;[1 1 1] If Barrier is destroyed already, return true
      (return true))))

(fn CreateBarricadePieces
  (bind _barricadevolume (Variables|Default|GetBarricadeVolume))
  (bind _barricadevolume_2 (Variables|Default|GetBarricadeVolume))
  (bind _returnvalue (Components|Box|GetScaledBoxExtent _barricadevolume))
  (bind _returnvalue_2 (Transformation|GetWorldTransform _barricadevolume_2))
  ;[1 1 1] Calculate the (local) vertical space for each barricade piece
  (LocalVariables|SetVertical%20Offset (.z _returnvalue))
  (LocalVariables|SetVerticalInterval (/ (* (.z _returnvalue) 2.0) (Math|Conversions|ToFloat(Integer) (Variables|Barricade|GetBarricadePieceCount))))
  (for _index (range 0 (Variables|Barricade|GetBarricadePieceCount))
    (bind _returnvalue_3 (Game|SpawnActorfromClass "/Game/HorrorHo/Blueprints/EnmSpawn/Barricade/BP_BarricadePieceNew.BP_BarricadePieceNew_C" (Math|Transform|MakeTransform (.location _returnvalue_2) (.rotation _returnvalue_2)) "Undefined" 0 0))
    (bind _output_get (LocalVariables|SetTemp%20Piece _returnvalue_3))
    ;[1 1 1] Add slightly randomized rotation
    (Transformation|AddActorLocalRotation _output_get (Math|Rotator|MakeRotator 0.0 (* (Math|Random|RandomFloatinRange -1.0 1.0) (Variables|Default|GetRotationRandomness)) 0.0) false false)
    (Transformation|AddActorWorldOffset _output_get (Math|Vector|MakeVector 0.0 0.0 (- (* _index (LocalVariables|GetVerticalInterval)) (LocalVariables|GetVertical%20Offset))))
    (Utilities|Array|Add (Variables|Barricade|GetBarricadeMeshArray) (LocalVariables|GetTemp%20Piece)))
  (Utilities|Array|Shuffle (Variables|Barricade|GetBarricadeMeshArray))
  (return))

(fn SetBarricadePieceVisibility
  (for (_array_element _array_index) (Variables|Barricade|GetBarricadeMeshArray)
    ;[1 1 1] Set the broken barricade pieces to hidden
    (if (>= _array_index (Variables|Default|GetLivePieceCount))
      (Rendering|SetVisibility (Variables|/Script/Engine.Actor|GetRootComponent _array_element) false true)))
  (return))

(fn SpawnParticlesandSound
  (bind _barricadevolume (Variables|Default|GetBarricadeVolume))
  (bind _returnvalue (Transformation|GetWorldLocation _barricadevolume))
  (bind _boxextent (Variables|/Script/Engine.BoxComponent|GetBoxExtent _barricadevolume))
  (bind _returnvalue_2 (Math|Random|RandomPointinBoundingBox _returnvalue _boxextent))
  (Niagara|SpawnSystematLocation "/Game/HorrorHo/Blueprints/EnmSpawn/Barricade/NS_Barricade.NS_Barricade" _returnvalue_2)
  (Audio|PlaySoundatLocation "/Game/HorrorHo/Audio/Concrete_footsteps_4.Concrete_footsteps_4" _returnvalue_2 "0, 0, 0" 1.0 1.0 0.0 0 0 0)
  (return))