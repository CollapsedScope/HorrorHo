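; Zombie enemy character that takes damage, dies, and downgrades to a lightweight stand-in when the player moves away.
; Damage runs through BPCHealth and the health bar, playing a random hit sound or, on death, flagging the anim instance and destroying the actor after a delay.
; When the player is over two rooms away, it swaps itself for a collisionless FakeAI keeping its room ID.
; Death releases its ZombieManager spawn and attack permission; swapping releases only the latter.
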(event Custom|OnPlayerMovedAway
  ;[1 1 1] Called when player character moved more than 2 rooms away from the zombie
  (CallFunction|SwaptoFakeAI))

(event Game|Damage|EventAnyDamage
  (params (Damage :type Float%20%28single-precision%29) (DamageType :type Damage%20Type%20Object%20Reference) (InstigatedBy :type Controller%20Object%20Reference) (DamageCauser :type Actor%20Object%20Reference))
  ;[1 1 1] Take damage, initiate death behavior if no hp left
  (bind _zero (Default|CalculateHealth (Variables|Default|GetBPC_Health) Damage (UserInterface|GetUserWidgetObject (Variables|Default|GetHealthBar))))
  (if _zero
    (Audio|SpawnSoundatLocation "/Game/HorrorHo/Audio/extra/death_splatter.death_splatter" (Transformation|GetActorLocation) "0, 0, 0" 1.0 1.0 0.0 0 0)
    (if (not (Variables|AIState|GetIsDead))
      (Variables|AIState|SetIsDead true)
      (CallFunction|InitDeathState)
      (Utilities|FlowControl|Delay 5.0)
      (Actor|DestroyActor))
    (else
      (CallFunction|PlayHitSound))))

(event Collision|EventActorBeginOverlap
  (params (OtherActor :type Actor%20Object%20Reference)))

(event EventTick
  (params (DeltaSeconds :type Float%20%28single-precision%29)))

(event EventDestroyed)

(fn ConstructionScript
  (|CallParentFunction))

(fn SwaptoFakeAI
  (bind _returnvalue (Transformation|GetActorTransform))
  (bind _returnvalue_2 (Game|SpawnActorfromClass "/Game/HorrorHo/Blueprints/EnmSpawn/RoomSys/FakeAI.FakeAI_C" (Math|Transform|MakeTransform (Math|Vector|MakeVector (.x (.location _returnvalue)) (.y (.location _returnvalue)) (- (.z (.location _returnvalue)) 96.0)) (.rotation _returnvalue) (.scale _returnvalue)) "Undefined" 0 0))
  (Variables|/Game/HorrorHo/Blueprints/EnmSpawn/RoomSys/FakeAI.FakeAI_C|SetCurrentRoomID _returnvalue_2 (Variables|Default|GetCurrentRoomID))
  (if (Variables|AIState|GetPlayerAttackPermission)
    ;[1 1 1] Release attack permission if needed
    (bind _zombiesmode (Class|ZombiesGameModeInterface|GetZombiesMode(Message) (Game|GetGameMode)))
    (Default|ReleaseAttackPermission (Variables|/Game/HorrorHo/Blueprints/GameMode/ZombiesGameMode.ZombiesGameMode_C|GetZombieManager _zombiesmode) self))
  ;[1 1 1] Deactivate the controller so that it does not call behavior tree functions with a faulty actor reference
  (Actor|DestroyActor)
  (Class|Pawn|DetachfromControllerPendingDestroy))

(fn InitDeathState
  (bind _aszom_1anm (Utilities|Casting|CastTozom1Anm (Components|SkeletalMesh|GetAnimInstance (Variables|Character|GetMesh))))
  (Variables|/Game/HorrorHo/Blueprints/EnmSpawn/AIZombie/ZomA_Anim/zom1Anm.zom1Anm_C|SetIsDead _aszom_1anm true)
  (bind _zombiecontroller (Class|BPZombieControllerInterface|GetZombieController(Message) (Pawn|GetController)))
  (Default|InitDestroy _zombiecontroller)
  (Class|Pawn|DetachfromControllerPendingDestroy)
  ;[1 1 1] Release player attack permissions
  (bind _zombiesmode (Class|ZombiesGameModeInterface|GetZombiesMode(Message) (Game|GetGameMode)))
  (Default|ReleaseSpawn (Variables|/Game/HorrorHo/Blueprints/GameMode/ZombiesGameMode.ZombiesGameMode_C|GetZombieManager _zombiesmode) self)
  (Default|ReleaseAttackPermission (Variables|/Game/HorrorHo/Blueprints/GameMode/ZombiesGameMode.ZombiesGameMode_C|GetZombieManager _zombiesmode) self))

(fn PlayHitSound
  (bind _returnvalue (Transformation|GetActorLocation))
  (switch int (Math|Random|RandomInteger 4)
    (:0
      (Audio|PlaySoundatLocation "/Game/HorrorHo/Audio/Body_Flesh_1.Body_Flesh_1" _returnvalue "0, 0, 0" 0.5 1.0 0.0 0 0 0))
    (:1
      (Audio|PlaySoundatLocation "/Game/HorrorHo/Audio/Body_Flesh_2.Body_Flesh_2" _returnvalue "0, 0, 0" 0.5 1.0 0.0 0 0 0))
    (:2
      (Audio|PlaySoundatLocation "/Game/HorrorHo/Audio/Body_Flesh_3.Body_Flesh_3" _returnvalue "0, 0, 0" 0.6 0.8 0.0 0 0 0))
    (:3
      (Audio|PlaySoundatLocation "/Game/HorrorHo/Audio/Body_Flesh_4.Body_Flesh_4" _returnvalue "0, 0, 0" 0.8 0.5 0.0 0 0 0))
    (:4
      (Audio|PlaySoundatLocation "/Game/HorrorHo/Audio/Body_Flesh_5.Body_Flesh_5" _returnvalue "0, 0, 0" 0.6 1.0 0.0 0 0 0))))

(fn GetZombieCharacter
  (return self))