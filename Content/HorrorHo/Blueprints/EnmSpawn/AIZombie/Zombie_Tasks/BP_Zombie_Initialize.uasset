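; Behavior tree task that initializes a zombie's AI by picking its nearest level entrance.
; It loops over the game mode's level entry points, measuring navigation path length from the zombie to each enter volume and keeping the shortest successful path.
; The chosen entrance, index and location go to the blackboard, alongside reset initialization, movement and attack-permission flags, then the task finishes successfully.
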(event EventReceiveExecute
  (params (OwnerActor :type Actor%20Object%20Reference))
  (bind _zombiecontroller (Class|BPZombieControllerInterface|GetZombieController(Message) OwnerActor))
  (bind _targetentrance (CallFunction|FindClosestEntrance _zombiecontroller))
  (AI|BehaviorTree|SetBlackboardValueasVector (Variables|Default|GetClosestEntranceLocation) _targetentrance)
  (Class|BTFunctionLibrary|SetBlackboardValueasBool (Variables|Default|GetIsInitialized) true)
  (Class|BTFunctionLibrary|SetBlackboardValueasBool (Variables|Default|GetEntranceAttackPermission) false)
  (Class|BTFunctionLibrary|SetBlackboardValueasBool (Variables|Default|GetIsMoving) false)
  (AI|BehaviorTree|FinishExecute true))

(fn FindClosestEntrance
  (params (Controller :type BP%20Zombie%20Controller%20Object%20Reference))
  ;[1 1 1] Collect the distances to each entrance
  (bind _zombie (Default|GetControlledZombie Controller))
  (bind _zombiesmode (Class|ZombiesGameModeInterface|GetZombiesMode(Message) (Game|GetGameMode)))
  (LocalVariables|SetActorLocation (Transformation|GetActorLocation _zombie))
  (for (_array_element _array_index) (Variables|/Game/HorrorHo/Blueprints/GameMode/ZombiesGameMode.ZombiesGameMode_C|GetLevelEntryPoints _zombiesmode)
    (if (Utilities|Enum|Equal(Enum) (.ReturnValue (Class|NavigationSystemV1|GetPathLength (LocalVariables|GetActorLocation) (Transformation|GetWorldLocation (Variables|/Game/HorrorHo/Blueprints/EnmSpawn/Barricade/BP_EnemyEnterPoint.BP_EnemyEnterPoint_C|GetEnterVolume _array_element)) 0 0)) "Success")
      (if (< (.PathLength (Class|NavigationSystemV1|GetPathLength (LocalVariables|GetActorLocation) (Transformation|GetWorldLocation (Variables|/Game/HorrorHo/Blueprints/EnmSpawn/Barricade/BP_EnemyEnterPoint.BP_EnemyEnterPoint_C|GetEnterVolume _array_element)) 0 0)) (LocalVariables|GetShortestDistance))
        (LocalVariables|SetShortestDistance (.PathLength (Class|NavigationSystemV1|GetPathLength (LocalVariables|GetActorLocation) (Transformation|GetWorldLocation (Variables|/Game/HorrorHo/Blueprints/EnmSpawn/Barricade/BP_EnemyEnterPoint.BP_EnemyEnterPoint_C|GetEnterVolume _array_element)) 0 0)))
        (LocalVariables|SetClosestFoundEntrance (Transformation|GetWorldLocation (Variables|/Game/HorrorHo/Blueprints/EnmSpawn/Barricade/BP_EnemyEnterPoint.BP_EnemyEnterPoint_C|GetEnterVolume _array_element)))
        (Class|BTFunctionLibrary|SetBlackboardValueasObject (Variables|Default|GetEnterPoint) _array_element)
        (Class|BTFunctionLibrary|SetBlackboardValueasInt (Variables|Default|GetTargetEntranceID) _array_index))))
  (return (LocalVariables|GetClosestFoundEntrance)))