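; Behavior tree task in which a zombie attacks the barricade at its enemy entry point.
; After an attack-speed delay, noted as temporary, it sets the CanEnter blackboard key if the zombie can already enter the player area.
; Otherwise it checks the entry point's barricade health, flagging the zombie to start attacking while health remains or to enter once it is zero.
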(event EventReceiveExecute
  (params (OwnerActor :type Actor%20Object%20Reference))
  ;[1 1 1] Temporary Attack Speed Delay
  (Utilities|FlowControl|Delay (Variables|Default|GetAttackSpeed))
  (bind _zombie (Class|BPZombieControllerInterface|GetControlledZombie(Message) OwnerActor))
  (if (Variables|/Game/HorrorHo/Blueprints/EnmSpawn/AIZombie/BP_ZombieCharacter.BP_ZombieCharacter_C|GetCanEnterPlayerArea _zombie)
    ;[1 1 1] If the barricade is destroyed, wait to transition into player area
    (Class|BTFunctionLibrary|SetBlackboardValueasBool (Variables|Default|GetCanEnter) true)
    (AI|BehaviorTree|FinishExecute true)
    (else
      (bind _asbp_enemy_enter_point (Utilities|Casting|CastToBP_EnemyEnterPoint (AI|BehaviorTree|GetBlackboardValueasActor (Variables|Default|GetEnterPoint))))
      (if (Math|Conversions|ToBoolean(Integer) (Variables|/Game/HorrorHo/Blueprints/EnmSpawn/Barricade/BP_EnemyEnterPoint.BP_EnemyEnterPoint_C|GetBarricadeHealth _asbp_enemy_enter_point))
        ;[1 1 1] Attack if the barricade is still alive
        (Variables|/Game/HorrorHo/Blueprints/EnmSpawn/AIZombie/BP_ZombieCharacter.BP_ZombieCharacter_C|SetStartAttack _zombie true)
        (else
          ;[1 1 1] Skip attacking if the barricade is already  dead
          (Variables|/Game/HorrorHo/Blueprints/EnmSpawn/AIZombie/BP_ZombieCharacter.BP_ZombieCharacter_C|SetCanEnterPlayerArea _zombie true)))
      (AI|BehaviorTree|FinishExecute true))))