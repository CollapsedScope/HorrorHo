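; Behavior Tree task in which a zombie asks the game mode for permission to attack its target barricaded entrance.
; When granted, it sets the AttackPermission blackboard key and moves the zombie toward the entrance location, toggling its IsMoving flag.
; Results are inverted: a successful move finishes the task as failed, while a failed move, or a denied request after a short delay, finishes as succeeded.
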(event EventReceiveExecute
  (params (OwnerActor :type Actor%20Object%20Reference))
  (bind _zombiesmode (Class|ZombiesGameModeInterface|GetZombiesMode(Message) (Game|GetGameMode)))
  (bind _permissionresult (Default|AskPermissionAttackEntrance _zombiesmode (Class|BTFunctionLibrary|GetBlackboardValueasInt (Variables|Default|GetTargetEntranceID))))
  (if _permissionresult
    (Class|BTFunctionLibrary|SetBlackboardValueasBool (Variables|Default|GetAttackPermission) true)
    ;[1 1 1] Move closer to door before returning success
    (bind _zombiecontroller (Class|BPZombieControllerInterface|GetZombieController(Message) OwnerActor))
    (bind _zombie (Default|GetControlledZombie _zombiecontroller))
    (AI|AIMoveTo _zombie (Class|BTFunctionLibrary|GetBlackboardValueasVector (Variables|Default|GetEntranceLocation)) 0 2e+02 true
      (:then
        (Variables|/Game/HorrorHo/Blueprints/EnmSpawn/AIZombie/BP_ZombieCharacter.BP_ZombieCharacter_C|SetIsMoving _zombie true))
      (:OnSuccess
        (Variables|/Game/HorrorHo/Blueprints/EnmSpawn/AIZombie/BP_ZombieCharacter.BP_ZombieCharacter_C|SetIsMoving _zombie false)
        (AI|BehaviorTree|FinishExecute false))
      (:OnFail
        (Variables|/Game/HorrorHo/Blueprints/EnmSpawn/AIZombie/BP_ZombieCharacter.BP_ZombieCharacter_C|SetIsMoving _zombie false)
        (AI|BehaviorTree|FinishExecute true)))
    (else
      (Utilities|FlowControl|Delay 0.5)
      (AI|BehaviorTree|FinishExecute true))))