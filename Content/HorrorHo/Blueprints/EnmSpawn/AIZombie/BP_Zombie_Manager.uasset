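; BP_Zombie_Manager coordinates the zombie population and limits how many zombies can attack the player at once.
; Zombies request attack slots, and a closer one can displace a farther attacker when slots are full, receiving either an attacker or chaser target distance.
; Spawn requests create BP_ZombieCharacter actors up to a maximum, tracked in an array until released.
; BeginPlay counts pre-placed zombies but does not add them to that array.
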(event EventBeginPlay
  (Variables|Default|SetPlayerReference (Game|Player|GetPlayerPawn 0))
  (bind _outactors (Actor|GetAllActorsOfClass "/Game/HorrorHo/Blueprints/EnmSpawn/AIZombie/BP_ZombieCharacter.BP_ZombieCharacter_C"))
  (Variables|Default|SetZombiesCurrent (Utilities|Array|Length _outactors)))

(event Collision|EventActorBeginOverlap
  (params (OtherActor :type Actor%20Object%20Reference)))

(event EventTick
  (params (DeltaSeconds :type Float%20%28single-precision%29)))

(fn ConstructionScript)

(fn QueryAttackPermission
  (params (ZombieInstance :type BP%20Zombie%20Character%20Object%20Reference))
  (bind _playerreference (Variables|Default|GetPlayerReference))
  (bind _currentattackers (Variables|Default|GetCurrentAttackers))
  (for _array_element (Variables|Default|GetCurrentAttackers)
    (if (== _array_element ZombieInstance)
      (return true (Variables|Default|GetAttackerTargetDistance))))
  (if (< (Utilities|Array|Length (Variables|Default|GetCurrentAttackers)) (Variables|Default|GetAttackerMax))
    (Utilities|Array|Add (Variables|Default|GetCurrentAttackers) ZombieInstance)
    (return true (Variables|Default|GetAttackerTargetDistance))
    (else
      (LocalVariables|SetNewDistance (Transformation|GetDistanceTo _playerreference ZombieInstance))
      (for _array_element_2 (Variables|Default|GetCurrentAttackers)
        (if (< (LocalVariables|GetNewDistance) (Transformation|GetDistanceTo _playerreference _array_element_2))
          (Variables|/Game/HorrorHo/Blueprints/EnmSpawn/AIZombie/BP_ZombieCharacter.BP_ZombieCharacter_C|SetPlayerAttackPermission _array_element_2 false)
          (Utilities|Array|RemoveItem _currentattackers _array_element_2)
          (Utilities|Array|Add _currentattackers ZombieInstance)
          (return true (Variables|Default|GetAttackerTargetDistance))))
      (return false (Variables|Default|GetChaserTargetDistance)))))

(fn ReleaseAttackPermission
  (params (Zombie%20Reference :type BP%20Zombie%20Character%20Object%20Reference))
  (for _array_element (Variables|Default|GetCurrentAttackers)
    (if (== _array_element Zombie%20Reference)
      (Utilities|Array|RemoveItem (Variables|Default|GetCurrentAttackers) Zombie%20Reference))))

(fn SpawnifAble
  (params (SpawnTransform :type Transform))
  (bind _zombiesmax (Variables|Default|GetZombiesMax))
  (bind _zombiearray (Variables|Default|GetZombieArray))
  (bind _zombiearray_2 (Variables|Default|GetZombieArray))
  (bind _returnvalue (Utilities|Array|Length _zombiearray))
  (bind _returnvalue_2 (> _zombiesmax _returnvalue))
  (if _returnvalue_2
    (bind _returnvalue_3 (Game|SpawnActorfromClass "/Game/HorrorHo/Blueprints/EnmSpawn/AIZombie/BP_ZombieCharacter.BP_ZombieCharacter_C" SpawnTransform "Undefined" 0 0))
    (Utilities|Array|Add _zombiearray_2 _returnvalue_3)
    (Variables|Default|SetZombiesCurrent (Utilities|Array|Length _zombiearray_2)))
  (return _returnvalue_2))

(fn ReleaseSpawn
  (params (Zombie :type BP%20Zombie%20Character%20Object%20Reference))
  (bind _zombiearray (Variables|Default|GetZombieArray))
  (bind _returnvalue (Utilities|Array|RemoveItem _zombiearray Zombie))
  (if _returnvalue
    (Variables|Default|SetZombiesCurrent (Utilities|Array|Length _zombiearray))
    (return)
    (else
      (Development|PrintString "An unknown zombie attempted to release..."))))