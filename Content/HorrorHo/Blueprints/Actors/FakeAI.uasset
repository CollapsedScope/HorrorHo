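; Lightweight stand-in for an off-screen zombie that travels room to room toward the player's room, then becomes a real BP_ZombieCharacter.
; The game mode supplies a room path, room volumes supply doorways, and Tick lerps between them at constant speed without AI navigation.
; Player room changes trigger a repath or spawn.
; SpawnZombie initializes the zombie's blackboard, or decrements the manager's count on failure, then destroys this actor.
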(event Custom|OnPlayerChangedRooms
  (params (NewPlayerRoomID :type Integer))
  ;[1 1 1] Event called when player moves to a new room
  (bind _output_get (Variables|Navigation|SetTargetRoom NewPlayerRoomID))
  (if (!= _output_get (Variables|Default|GetCurrentRoomID))
    (Variables|Movement|SetCurrentLerpValue 0.0)
    (Variables|Movement|SetPreviousLocation (Transformation|GetActorLocation))
    (bind _success (CallFunction|TryGetTargetPath (Variables|Default|GetCurrentRoomID)))
    (Variables|Navigation|SetIsMoving _success)
    (bind _zombiesmode (Class|ZombiesGameModeInterface|GetZombiesMode(Message) (Game|GetGameMode)))
    (CallFunction|BeginNavigation (Utilities|Array|Get(acopy) (Variables|/Game/HorrorHo/Blueprints/GameMode/ZombiesGameMode.ZombiesGameMode_C|GetRoomVolumes _zombiesmode) (Variables|Default|GetCurrentRoomID)) self)
    (else
      (Utilities|FlowControl|Delay 0.1)
      (CallFunction|SpawnZombie))))

(event Custom|OnFirstNotify
  (params (PlayerRoomID :type Integer))
  (Variables|Navigation|SetTargetRoom PlayerRoomID)
  (for _array_element (Collision|GetOverlappingActors "/Script/Engine.Actor" :!class /Script/Engine.Actor)
    (bind _asroom_volume (Utilities|Casting|CastToRoomVolume _array_element))
    (bind _output_get (Variables|Default|SetCurrentRoomID (Math|Conversions|ToInteger(Byte) (Variables|/Game/HorrorHo/Blueprints/Actors/Installation/RoomVolume.RoomVolume_C|GetRoomID _asroom_volume))))
    (if (!= _output_get (Variables|Navigation|GetTargetRoom))
      (Utilities|FlowControl|Delay 0.1)
      (CallFunction|SpawnZombie)
      (else
        (bind _success (CallFunction|TryGetTargetPath (Math|Conversions|ToInteger(Byte) (Variables|/Game/HorrorHo/Blueprints/Actors/Installation/RoomVolume.RoomVolume_C|GetRoomID _asroom_volume))))
        (Variables|Navigation|SetIsMoving _success)
        (CallFunction|BeginNavigation _asroom_volume self)))))

(event EventBeginPlay
  (bind _zombiesmode (Class|ZombiesGameModeInterface|GetZombiesMode(Message) (Game|GetGameMode)))
  (bind _output_get (Variables|Default|SetGameModeReference _zombiesmode))
  (Variables|Navigation|SetTargetRoom (Variables|/Game/HorrorHo/Blueprints/GameMode/ZombiesGameMode.ZombiesGameMode_C|GetPlayerRoomID _output_get)))

(event Collision|EventActorBeginOverlap
  (params (OtherActor :type Actor%20Object%20Reference)))

(event EventTick
  (params (DeltaSeconds :type Float%20%28single-precision%29))
  (if (Variables|Navigation|GetIsMoving)
    (CallFunction|MoveAlongPath DeltaSeconds)
    (elif (Variables|Default|GetInitialMoveTrigger)
      (Variables|Default|SetInitialMoveTrigger false)
      (if (>= (Variables|Default|GetCurrentRoomID) 0)
        (bind _zombiesmode (Class|ZombiesGameModeInterface|GetZombiesMode(Message) (Game|GetGameMode)))
        (bind _success (CallFunction|TryGetTargetPath (Variables|Default|GetCurrentRoomID)))
        (Variables|Navigation|SetIsMoving _success)
        (CallFunction|BeginNavigation (Utilities|Array|Get(acopy) (Variables|/Game/HorrorHo/Blueprints/GameMode/ZombiesGameMode.ZombiesGameMode_C|GetRoomVolumes _zombiesmode) (Variables|Default|GetCurrentRoomID)) self)
        (else
          (for _array_element (Collision|GetOverlappingActors "/Script/Engine.Actor" :!class /Script/Engine.Actor)
            (bind _asroom_volume (Utilities|Casting|CastToRoomVolume _array_element))
            (Variables|Default|SetCurrentRoomID (Math|Conversions|ToInteger(Byte) (Variables|/Game/HorrorHo/Blueprints/Actors/Installation/RoomVolume.RoomVolume_C|GetRoomID _asroom_volume)))
            (bind _success_2 (CallFunction|TryGetTargetPath (Math|Conversions|ToInteger(Byte) (Variables|/Game/HorrorHo/Blueprints/Actors/Installation/RoomVolume.RoomVolume_C|GetRoomID _asroom_volume))))
            (Variables|Navigation|SetIsMoving _success_2)
            (CallFunction|BeginNavigation _asroom_volume self)))))))

(fn ConstructionScript)

(fn MoveAlongPath
  (params (DeltaTime :type Float%20%28single-precision%29))
  (bind _targetpath (Variables|Navigation|GetTargetPath))
  (Variables|Movement|SetCurrentLerpValue (Math|Float|Clamp(Float) (+ (Variables|Movement|GetCurrentLerpValue) (* DeltaTime (Variables|Movement|GetCurrentLerpSpeed)))))
  ;[1 1 1] Temporary: this is just to visually represent the movement,  in the finished system we don't actually need to move the fake AI at all
  (Transformation|SetActorLocation (Math|Vector|Lerp(Vector) (Variables|Movement|GetPreviousLocation) (Variables|Movement|GetNextLocation) (Variables|Movement|GetCurrentLerpValue)) false false)
  ;[1 1 1] When the lerp is complete, the fake AI has reached the next room
  (if (>= (Variables|Movement|GetCurrentLerpValue) 1.0)
    (Variables|Movement|SetCurrentLerpValue 0.0)
    ;[1 1 1] Remove the first member of the target path.  If it was the last one, switch to a real zombie
    (if (== (Utilities|Array|Length _targetpath) 1)
      (CallFunction|SpawnZombie)
      (else
        ;[1 1 1] Get a reference to the room volume we just "entered" and then remove it from the path index
        (bind _zombiesmode (Class|ZombiesGameModeInterface|GetZombiesMode(Message) (Game|GetGameMode)))
        (bind _output_get (LocalVariables|SetTempRoomVolume (Utilities|Array|Get(acopy) (Variables|/Game/HorrorHo/Blueprints/GameMode/ZombiesGameMode.ZombiesGameMode_C|GetRoomVolumes _zombiesmode) (Utilities|Array|Get(acopy) _targetpath))))
        (Variables|Default|SetCurrentRoomID (Math|Conversions|ToInteger(Byte) (Variables|/Game/HorrorHo/Blueprints/Actors/Installation/RoomVolume.RoomVolume_C|GetRoomID _output_get)))
        (Utilities|Array|RemoveIndex _targetpath)
        ;[1 1 1] Save the door we just got to, and then begin navigation to the next doorway
        (Variables|Navigation|SetPreviousDoorReference (Variables|Navigation|GetNextDoorReference))
        (CallFunction|BeginNavigation (LocalVariables|GetTempRoomVolume) (Variables|Navigation|GetPreviousDoorReference))))))

(fn TryGetTargetPath
  (params (CurrentRoomID :type Integer))
  (bind _gamemodereference (Variables|Default|GetGameModeReference))
  (Utilities|IsValid _gamemodereference
    (:Is%20Valid
      (bind _bestfoundpath (Default|GetPathtoTargetRoom _gamemodereference CurrentRoomID (Variables|Navigation|GetTargetRoom)))
      (Variables|Navigation|SetTargetPath _bestfoundpath)
      (return true))
    (:Is%20Not%20Valid
      (return false))))

(fn QueryCurrentRoom
  (for _array_element (Collision|GetOverlappingActors "/Script/Engine.Actor" :!class /Script/Engine.Actor)
    (bind _asroom_volume (Utilities|Casting|CastToRoomVolume _array_element)
      (:then
        (return true (Math|Conversions|ToInteger(Byte) (Variables|/Game/HorrorHo/Blueprints/Actors/Installation/RoomVolume.RoomVolume_C|GetRoomID _asroom_volume))))
      (:CastFailed
        (return false 0)))))

(fn BeginNavigation
  (params (CurrentRoomVolume :type Room%20Volume%20Object%20Reference) (StartingLocationActor :type Actor%20Object%20Reference))
  (bind _targetpath (Variables|Navigation|GetTargetPath))
  (bind _returnvalue (Transformation|GetActorLocation StartingLocationActor))
  ;[1 1 1] If we are attempting to navigate without a path, abort and spawn a zombie
  (if (<= (Utilities|Array|Length _targetpath) 0)
    (Variables|Navigation|SetIsMoving false)
    (else
      (bind _doorvolume (Default|TryGetTargetDoorway CurrentRoomVolume (Utilities|Array|Get(acopy) _targetpath) self))
      (Utilities|IsValid _doorvolume
        (:Is%20Valid
          (bind _output_get (Variables|Navigation|SetNextDoorReference _doorvolume))
          (Variables|Movement|SetNextLocation (Transformation|GetActorLocation _output_get))
          (Variables|Movement|SetPreviousLocation _returnvalue)
          (Variables|Movement|SetCurrentLerpSpeed (/ (Variables|Movement|GetMovementPerSecond) (Math|Vector|Distance(Vector) _returnvalue (Transformation|GetActorLocation _output_get))))
          ;[1 1 1] Set general rotation (good enough for fake AI)
          (Transformation|SetActorRotation (Math|Conversions|RotationFromXVector (- (Variables|Movement|GetNextLocation) (Variables|Movement|GetPreviousLocation)))))))))

(fn SpawnZombie
  (bind _returnvalue (Math|Vector|MakeVector 0.0 0.0 0.0))
  (bind _returnvalue_2 (Game|GetPlayerCharacter 0))
  (bind _returnvalue_3 (Transformation|GetActorLocation))
  (bind _returnvalue_4 (Transformation|GetActorLocation _returnvalue_2))
  (Utilities|IsValid _returnvalue_2
    (:Is%20Valid
      (Class|KismetMathLibrary|VectorSet _returnvalue (.x _returnvalue_4) (.y _returnvalue_4) 0.0))
    (:Is%20Not%20Valid
      _))
  (bind _returnvalue_5 (Game|SpawnActorfromClass "/Game/HorrorHo/Blueprints/Characters/BP_ZombieCharacter.BP_ZombieCharacter_C" (Math|Transform|MakeTransform (+ _returnvalue_3 "0, 0,100.000000") (Math|Conversions|RotationFromXVector (Math|Vector|Normalize (- _returnvalue _returnvalue_3))) "1,1,1") "AdjustIfPossibleButDontSpawnIfColliding" 0 0))
  (Utilities|IsValid _returnvalue_5
    (:Is%20Valid
      (Variables|/Game/HorrorHo/Blueprints/Characters/BP_ZombieCharacter.BP_ZombieCharacter_C|SetCurrentRoomID _returnvalue_5 (Variables|Default|GetCurrentRoomID))
      (bind _zombiecontroller (Class|BPIZombieController|ZConGetZombieController(Message) (Pawn|GetController _returnvalue_5)))
      ;[1 1 1] Initiate zombie's bt state
      (AI|Components|Blackboard|SetValueasBool (AI|GetBlackboard _zombiecontroller) (Utilities|Name|MakeLiteralName "IsInitialized") true)
      (AI|Components|Blackboard|SetValueasBool (AI|GetBlackboard _zombiecontroller) (Utilities|Name|MakeLiteralName "IsInsidePlayerArea") true)
      (Actor|DestroyActor))
    (:Is%20Not%20Valid
      (Math|Integer|DecrementInt (Variables|/Game/HorrorHo/Blueprints/Utilities/BP_Zombie_Manager.BP_Zombie_Manager_C|GetZombiesCurrent (Variables|/Game/HorrorHo/Blueprints/GameMode/ZombiesGameMode.ZombiesGameMode_C|GetZombieManager (Variables|Default|GetGameModeReference)))
        (:%20%20
          (Actor|DestroyActor))))))

(fn CheckForceSpawn
  (params (RoomID1 :type Integer) (RoomID2 :type Integer))
  (bind _currentroomid (Variables|Default|GetCurrentRoomID))
  (if (== RoomID1 _currentroomid)
    (CallFunction|SpawnZombie :!label _label)
    (elif (== RoomID2 _currentroomid)
      (goto _label))))