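; BP_EnemySpawnFieldOLD is a spawner actor for zombies mode that periodically requests zombie spawns at random points inside its SpawnVolume box.
; BeginPlay destroys it if disabled; otherwise it sets the initial delay and gets the game mode via GetZombiesModeMessage.
; Tick counts down, asks the ZombieManager to SpawnIfAble, then resets the timer.
; The interval shrinks as the spawner's lifetime grows, scaled by SpawnMultiplier and capped by MaxMultiplier.
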(event EventBeginPlay
  (if (Variables|Default|GetDisableSpawner)
    (Actor|DestroyActor)
    (else
      (Variables|Spawn|SetSpawnTimer (+ (Variables|Spawn|GetBaseTimer) (Variables|Spawn|GetInitialTimer)))
      (bind _zombiesmode (Class|ZombiesGameModeInterface|GetZombiesMode(Message) (Game|GetGameMode)))
      (Variables|Default|SetGameModeReference _zombiesmode))))

(event Collision|EventActorBeginOverlap
  (params (OtherActor :type Actor%20Object%20Reference)))

(event EventTick
  (params (DeltaSeconds :type Float%20%28single-precision%29))
  (bind _output_get (Variables|Spawn|SetSpawnTimer (- (Variables|Spawn|GetSpawnTimer) DeltaSeconds)))
  (if (< _output_get 0.0)
    (CallFunction|TrySpawnZombie)
    (CallFunction|SetTimer)))

(fn ConstructionScript)

(fn TrySpawnZombie
  (bind _spawnvolume (Variables|Default|GetSpawnVolume))
  (Default|SpawnifAble (Variables|/Game/HorrorHo/Blueprints/GameMode/ZombiesGameMode.ZombiesGameMode_C|GetZombieManager (Variables|Default|GetGameModeReference)) (Math|Conversions|ToTransform(Vector) (Math|Random|RandomPointinBoundingBox (Transformation|GetWorldLocation _spawnvolume) (Components|Box|GetScaledBoxExtent _spawnvolume))))
  (return))

(fn SetTimer
  ;[1 1 1] The spawn timer is divided by 1 + the number of minutes since the game started * the spawn multiplier.  Change the multiplier to change the spawn speed. The spawn speed will not exceed Max Multiplier times  faster.
  (Variables|Spawn|SetSpawnTimer (/ (Variables|Spawn|GetBaseTimer) (Math|Float|Min(Float) (+ (* (/ (Actor|GetGameTimeSinceCreation) 6e+01) (Variables|Spawn|GetSpawnMultiplier)) 1.0) (Variables|Spawn|GetMaxMultiplier))))
  (return))