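; BP_ActionWidgetVolume is an installation actor that shows a world action prompt widget with a child progress gauge.
; On BeginPlay it initializes the main widget with its action type, hides the child widget and nudges it upward.
; Interface events for action start, tick and end toggle the gauge, feed it the progress rate, reset it, and play the main widget's transition animation, reusing the barricading widget interface.
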(event EventBeginPlay
  (bind _childwidget (Variables|Default|GetChildWidget))
  (Class|BPIActionWidget|BPIInitialize(Message) (UserInterface|GetUserWidgetObject (Variables|Default|GetWidget)) (Variables|Default|GetActionWidgetType))
  (Rendering|SetVisibility _childwidget false false)
  (Class|Widget|SetRenderTransform (UserInterface|GetUserWidgetObject _childwidget) (Utilities|Struct|MakeWidgetTransform "(X=0.000000,Y=-8.000000)" "(X=1.000000,Y=1.000000)" "(X=0.000000,Y=0.000000)" 0.0)))

(event Collision|EventActorBeginOverlap
  (params (OtherActor :type Actor%20Object%20Reference)))

(event EventTick
  (params (DeltaSeconds :type Float%20%28single-precision%29)))

(event EventBPIActionWidgetVolumeonEndAction
  (Class|BPIBarricadingWidget|BPIBarricadingWidgetResetBarricadingGauge(Message) (UserInterface|GetUserWidgetObject (Variables|Default|GetChildWidget)))
  (Rendering|SetVisibility (Variables|Default|GetChildWidget) false false)
  (Class|BPIActionWidget|BPIPlayTransitAnimation(Message) (UserInterface|GetUserWidgetObject (Variables|Default|GetWidget)) true))

(event EventBPIActionWidgetVolumeonStartAction
  (Class|BPIBarricadingWidget|BPIBarricadingWidgetProgressRate(Message) (UserInterface|GetUserWidgetObject (Variables|Default|GetChildWidget)) 0.0 0.0)
  (Rendering|SetVisibility (Variables|Default|GetChildWidget) true false)
  (Class|BPIActionWidget|BPIPlayTransitAnimation(Message) (UserInterface|GetUserWidgetObject (Variables|Default|GetWidget)) false))

(event EventBPIActionWidgetVolumeTickAction
  (params (ProgressRate :type Float%20%28single-precision%29))
  (Class|BPIBarricadingWidget|BPIBarricadingWidgetProgressRate(Message) (UserInterface|GetUserWidgetObject (Variables|Default|GetChildWidget)) ProgressRate 0.0))

(fn ConstructionScript)