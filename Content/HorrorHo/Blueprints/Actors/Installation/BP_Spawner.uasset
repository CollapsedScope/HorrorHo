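; Enemy spawn point fronted by a breakable, repairable barricade, optionally prebuilt, that also tracks which enemy types its settings allow per wave.
; BeginPlay stacks jittered piece actors across BarricadeVolume and shuffles them, so they appear and disappear in random order.
; Damage and healing convert health into a visible piece count, with hit effects on damage and a returned flag at zero health.
; UpdateWaveSpawnSettings enables enemy types by wave thresholds, without spawning them here.
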(event EventBeginPlay
  (Variables|Barricade|SetPieceMaxHealth (/ (Variables|コンフィグBarricade|GetMaxBarricadeHealth) (Variables|コンフィグBarricade|GetBarricadePieceCount)))
  (Barricade|InitBarricadeHealth)
  (Barricade|CreateBarricadePieces)
  (Display|SetBarricadePieceVisibility))

(event Collision|EventActorBeginOverlap
  (params (OtherActor :type Actor%20Object%20Reference)))

(event EventTick
  (params (DeltaSeconds :type Float%20%28single-precision%29)))

(fn ConstructionScript)

(fn AdjustHealth
  (params (ChangeAmount :type Integer))
  (Utilities|FlowControl|Sequence
    (:then_0
      (Variables|Barricade|SetBarricadeHealth (Math|Integer|Clamp(Integer) (+ (Variables|Barricade|GetBarricadeHealth) ChangeAmount) 0 (Variables|コンフィグBarricade|GetMaxBarricadeHealth)))
      (bind _difference (Utility|GetPieceCountChange))
      (LocalVariables|SetCountChange _difference)
      (Variables|Barricade|SetLivePieceCount (+ (Variables|Barricade|GetLivePieceCount) (LocalVariables|GetCountChange))))
    (:then_1
      (Display|SpawnParticlesandSound (LocalVariables|GetCountChange) ChangeAmount)
      (if (> (Math|Integer|Absolute(Integer) (LocalVariables|GetCountChange)) 0)
        (Display|SetBarricadePieceVisibility)
        (if (< ChangeAmount 0)
          _
          (else
            _)))
      (return (<= (Variables|Barricade|GetBarricadeHealth) 0)))))

(fn CreateBarricadePieces
  (bind _barricadevolume (Variables|Default|GetBarricadeVolume))
  (bind _barricadevolume_2 (Variables|Default|GetBarricadeVolume))
  (bind _returnvalue (Components|Box|GetScaledBoxExtent _barricadevolume))
  (bind _returnvalue_2 (Transformation|GetWorldTransform _barricadevolume_2))
  ;[1 1 1] Calculate the (local) vertical space for each barricade piece
  (LocalVariables|SetVertical%20Offset (.z _returnvalue))
  (LocalVariables|SetVerticalInterval (/ (* (.z _returnvalue) 2.0) (Math|Conversions|ToFloat(Integer) (Variables|コンフィグBarricade|GetBarricadePieceCount))))
  (for _index (range 0 (Variables|コンフィグBarricade|GetBarricadePieceCount))
    (bind _returnvalue_3 (Game|SpawnActorfromClass "/Game/HorrorHo/Blueprints/Actors/Props/BP_BarricadePieceNew.BP_BarricadePieceNew_C" (Math|Transform|MakeTransform (.location _returnvalue_2) (.rotation _returnvalue_2)) "Undefined" 0 0))
    ;[1 1 1] Slightly random offset
    (bind _output_get (LocalVariables|SetTemp%20Piece _returnvalue_3))
    (Transformation|AddActorLocalOffset _output_get (Math|Vector|MakeVector (Math|Random|RandomFloatinRange -1e+01 1e+01) (Math|Random|RandomFloatinRange -3.0 3.0) 0.0) false false)
    ;[1 1 1] Add slightly randomized rotation
    (Transformation|AddActorLocalRotation _output_get (Math|Rotator|MakeRotator 0.0 (* (Math|Random|RandomFloatinRange -1.0 1.0) (Variables|コンフィグBarricade|GetRotationRandomness)) 0.0) false false)
    (Transformation|AddActorWorldOffset _output_get (Math|Vector|MakeVector 0.0 0.0 (- (* _index (LocalVariables|GetVerticalInterval)) (LocalVariables|GetVertical%20Offset))))
    (Utilities|Array|Add (Variables|Barricade|GetBarricadeMeshArray) (LocalVariables|GetTemp%20Piece)))
  (Utilities|Array|Shuffle (Variables|Barricade|GetBarricadeMeshArray))
  (return))

(fn SetBarricadePieceVisibility
  (for (_array_element _array_index) (Variables|Barricade|GetBarricadeMeshArray)
    (if (>= _array_index (Variables|Barricade|GetLivePieceCount))
      (Class|BPIBarricadePiece|BarricadePieceToggleVisibility(Message) _array_element false)
      (else
        (Class|BPIBarricadePiece|BarricadePieceToggleVisibility(Message) _array_element true)))))

(fn SpawnParticlesandSound
  (params (PieceCountChange :type Integer) (HealthChange :type Integer))
  (bind _barricadevolume (Variables|Default|GetBarricadeVolume))
  (if (and (< HealthChange 0) (> (Variables|Barricade|GetLivePieceCount) 0))
    ;[1 1 1] TODO: spawn particles directly at broken piece
    (LocalVariables|SetSpawnPos (Math|Random|RandomPointinBoundingBox (Transformation|GetWorldLocation _barricadevolume) (Variables|/Script/Engine.BoxComponent|GetBoxExtent _barricadevolume)))
    (Effects|SpawnEmitteratLocation "/Game/Art/Eda/Fx/Pt_ClashS.Pt_ClashS" (LocalVariables|GetSpawnPos))
    (Audio|PlaySoundatLocation "/Game/HorrorHo/Audio/extra/wood_hit_1.wood_hit_1" (LocalVariables|GetSpawnPos) "0, 0, 0" 1.0 1.0 0.0 0 0 0)
    (return)))

(fn IsFullHealth
  (return (== (Variables|Barricade|GetBarricadeHealth) (Variables|コンフィグBarricade|GetMaxBarricadeHealth))))

(fn InitBarricadeHealth
  ;[1 1 1] If the barricade is prebuilt, make all of the barricade pieces.  Otherwise set them to 0.
  (if (Variables|コンフィグBarricade|GetIsPrebuilt)
    (Variables|Barricade|SetBarricadeHealth (Variables|コンフィグBarricade|GetMaxBarricadeHealth))
    (Variables|Barricade|SetLivePieceCount (Variables|コンフィグBarricade|GetBarricadePieceCount))
    (else
      (Variables|Barricade|SetBarricadeHealth 0)
      (Variables|Barricade|SetLivePieceCount 0)))
  (return))

(fn GetNextBreakablePieceHealth
  (bind _barricadehealth (Variables|Barricade|GetBarricadeHealth))
  (bind _piecemaxhealth (Variables|Barricade|GetPieceMaxHealth))
  (bind _returnvalue (Math|Integer|%(Integer) _barricadehealth _piecemaxhealth))
  (return _returnvalue (/ (Math|Conversions|ToFloat(Integer) _returnvalue) (Math|Conversions|ToFloat(Integer) _piecemaxhealth))))

(fn GetPieceCountChange
  (return (- (/ (Variables|Barricade|GetBarricadeHealth) (Variables|Barricade|GetPieceMaxHealth)) (Variables|Barricade|GetLivePieceCount))))

(fn SetMaterialChanges
  (bind _piecehealthpercent (Utility|GetNextBreakablePieceHealth))
  (Class|BPIBarricadePiece|BarricadePieceSwapMaterial(Message) (Utilities|Array|Get(acopy) (Variables|Barricade|GetBarricadeMeshArray) (- (Variables|Barricade|GetLivePieceCount) 1)) (Math|Float|Floor (* 3 _piecehealthpercent))))

(fn UpdateWaveSpawnSettings
  (params (Wave%20Number :type Integer))
  (bind _spawnsettings (Variables|コンフィグSpawn|GetSpawnSettings))
  (bind (_canspawnwalker _spawnwalkerafterwavenumber _canspawnrunner _spawnrunnerafterwavenumber _canspawncrawler _spawncrawlerafterwavenumber _canspawnbomber _spawnbomberafterwavenumber _canspawnscreamer _spawnscreamerafterwavenumber _canspawnwatcher _spawnwatcherafterwavenumber _canspawnworm _spawnwormafterwavenumber) (Utilities|Struct|BreakStruct_SpawnerSettings _spawnsettings))
  (Utilities|FlowControl|Sequence
    (:then_0
      (if (Utility|IsinRange _spawnwalkerafterwavenumber 0 Wave%20Number)
        (Utilities|Struct|SetmembersinStruct_SpawnerSettings (Variables|コンフィグSpawn|GetSpawnSettings) true)))
    (:then_1
      (if (Utility|IsinRange _spawnrunnerafterwavenumber 0 Wave%20Number)
        (Utilities|Struct|SetmembersinStruct_SpawnerSettings (Variables|コンフィグSpawn|GetSpawnSettings) true)))
    (:then_2
      (if (Utility|IsinRange _spawncrawlerafterwavenumber 0 Wave%20Number)
        (Utilities|Struct|SetmembersinStruct_SpawnerSettings (Variables|コンフィグSpawn|GetSpawnSettings) true)))
    (:then_3
      (if (Utility|IsinRange _spawnbomberafterwavenumber 0 Wave%20Number)
        (Utilities|Struct|SetmembersinStruct_SpawnerSettings (Variables|コンフィグSpawn|GetSpawnSettings) true)))
    (:then_4
      (if (Utility|IsinRange _spawnscreamerafterwavenumber 0 Wave%20Number)
        (Utilities|Struct|SetmembersinStruct_SpawnerSettings (Variables|コンフィグSpawn|GetSpawnSettings) true)))
    (:then_5
      (if (Utility|IsinRange _spawnwatcherafterwavenumber 0 Wave%20Number)
        (Utilities|Struct|SetmembersinStruct_SpawnerSettings (Variables|コンフィグSpawn|GetSpawnSettings) true)))
    (:then_6
      (if (Utility|IsinRange _spawnwormafterwavenumber 0 Wave%20Number)
        (Utilities|Struct|SetmembersinStruct_SpawnerSettings (Variables|コンフィグSpawn|GetSpawnSettings) true)))))

(fn IsinRange
  (params (Num :type Integer) (Min :type Integer) (Max :type Integer))
  (return (and (>= Num Min) (<= Num Max))))

(fn HealBarricade
  (Variables|Barricade|SetBarricadeHealth (Math|Integer|Clamp(Integer) (+ (Variables|Barricade|GetBarricadeHealth) (Variables|Barricade|GetPieceMaxHealth)) 0 (Variables|コンフィグBarricade|GetMaxBarricadeHealth)))
  (bind _difference (Utility|GetPieceCountChange))
  (LocalVariables|SetCountChange _difference)
  (Variables|Barricade|SetLivePieceCount (+ (Variables|Barricade|GetLivePieceCount) (LocalVariables|GetCountChange)))
  (Display|SetBarricadePieceVisibility))