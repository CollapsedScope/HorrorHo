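; BP_Weapon is a weapon actor that gets equipped on the player character and provides its own shooting effects.
; On BeginPlay it sends an attach-weapon interface message to player 0's character, passing itself and its equip socket name.
; An interface event spawns the muzzle emitter on the mesh socket and plays the firing sound at the actor's location, while another interface function exposes the weapon mesh.
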(event EventBeginPlay
  (Class|BPIPlayer|BPIAttachWeapon(Message) (Game|GetPlayerCharacter 0) self (Variables|Default|GetEquipedSocketName)))

(event EventBPISpawnShootingEffect
  (Effects|SpawnEmitterAttached (Variables|Default|GetVFX_Shooting) (Variables|Default|GetWeaponMesh) (Variables|Default|GetMuzzleSocketName))
  (Audio|PlaySoundatLocation (Variables|Default|GetSFX_Shooting) (Transformation|GetActorLocation) "0, 0, 0" 1.0 1.0 0.0 0 0 0))

(fn ConstructionScript)

(fn BPIGetSkeletalMeshComponent
  (return (Variables|Default|GetWeaponMesh)))