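; A barricade piece prop actor that picks one of three wooden barricade variants at random.
; ChooseRandomBarricadePieceType sets the static mesh and stores that variant's normal, light-damage and heavy-damage meshes.
; It also creates a matching wood dynamic material instance and stores it as the repair material.
; The event graph holds only disabled stubs, and the construction script just calls the parent, so this file does not call the function itself.
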(event EventBeginPlay
  (|CallParentFunction) ; This node is disabled and will not be called.\nDrag off pins to build functionality.
)

(event Collision|EventActorBeginOverlap
  (params (OtherActor :type Actor%20Object%20Reference))
  (|CallParentFunction OtherActor) ; This node is disabled and will not be called.\nDrag off pins to build functionality.
)

(event EventTick
  (params (DeltaSeconds :type Float%20%28single-precision%29))
  (|CallParentFunction DeltaSeconds) ; This node is disabled and will not be called.\nDrag off pins to build functionality.
)

(fn ConstructionScript
  (|CallParentFunction))

(fn ChooseRandomBarricadePieceType
  (switch int (Math|Random|RandomIntegerinRange 0 2)
    (:0
      (Components|StaticMesh|SetStaticMesh (Variables|Default|GetBarricadeMesh) "/Game/Art/Eda/MDL/Barricade/S/BarricadeA.BarricadeA")
      (Variables|Default|SetMeshNormal "/Game/Art/Eda/MDL/Barricade/S/BarricadeA.BarricadeA")
      (Variables|Default|SetMeshLightDamage "/Game/Art/Eda/MDL/Barricade/S/BarricadeA30.BarricadeA30")
      (Variables|Default|SetMeshHeavyDamage "/Game/Art/Eda/MDL/Barricade/S/BarricadeA60.BarricadeA60")
      (bind _returnvalue (Rendering|Material|CreateDynamicMaterialInstance "/Game/Art/Eda/MTL/MI/Wood/MI_WoodA0.MI_WoodA0" "None" "None" :!class /Script/Engine.KismetMaterialLibrary))
      (Variables|Default|SetRepairMat _returnvalue))
    (:1
      (Components|StaticMesh|SetStaticMesh (Variables|Default|GetBarricadeMesh) "/Game/Art/Eda/MDL/Barricade/S/BarricadeB.BarricadeB")
      (Variables|Default|SetMeshNormal "/Game/Art/Eda/MDL/Barricade/S/BarricadeB.BarricadeB")
      (Variables|Default|SetMeshLightDamage "/Game/Art/Eda/MDL/Barricade/S/BarricadeB30.BarricadeB30")
      (Variables|Default|SetMeshHeavyDamage "/Game/Art/Eda/MDL/Barricade/S/BarricadeB60.BarricadeB60")
      (bind _returnvalue_2 (Rendering|Material|CreateDynamicMaterialInstance "/Game/Art/Eda/MTL/MI/Wood/MI_WoodB0.MI_WoodB0" "None" "None" :!class /Script/Engine.KismetMaterialLibrary))
      (Variables|Default|SetRepairMat _returnvalue_2))
    (:2
      (Components|StaticMesh|SetStaticMesh (Variables|Default|GetBarricadeMesh) "/Game/Art/Eda/MDL/Barricade/S/BarricadeC.BarricadeC")
      (Variables|Default|SetMeshNormal "/Game/Art/Eda/MDL/Barricade/S/BarricadeC.BarricadeC")
      (Variables|Default|SetMeshLightDamage "/Game/Art/Eda/MDL/Barricade/S/BarricadeC30.BarricadeC30")
      (Variables|Default|SetMeshHeavyDamage "/Game/Art/Eda/MDL/Barricade/S/BarricadeC60.BarricadeC60")
      (bind _returnvalue_3 (Rendering|Material|CreateDynamicMaterialInstance "/Game/Art/Eda/MTL/MI/Wood/MI_WoodC0.MI_WoodC0" "None" "None" :!class /Script/Engine.KismetMaterialLibrary))
      (Variables|Default|SetRepairMat _returnvalue_3))))