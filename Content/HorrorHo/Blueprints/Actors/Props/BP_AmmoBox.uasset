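; BP_AmmoBox is an ammo pickup that expires after a lifetime read from the DT_GeneralGameParams data table.
; On overlap with a BPI_Player actor, it passes its ammo count, records an item-pickup stat through the game instance, plays a sound and destroys itself.
; A looping timer, rather than Tick, drives TickLiveTimer, which yaws the widget toward the player and destroys the box when time runs out.
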(event OnComponentBeginOverlap(Collider)
  (params (OverlappedComponent :type Primitive%20Component%20Object%20Reference) (OtherActor :type Actor%20Object%20Reference) (OtherComp :type Primitive%20Component%20Object%20Reference) (OtherBodyIndex :type Integer) (bFromSweep :type Boolean) (SweepResult :type Hit%20Result%20Structure%20%28by%20ref%29))
  (if (Utilities|DoesObjectImplementInterface OtherActor "/Game/HorrorHo/Blueprints/Interfaces/BPI_Player.BPI_Player_C")
    (Class|BPIPlayer|BPIPlayerCollectAmmoBox(Message) OtherActor (Variables|Config|GetAmmoCount))
    (Class|BPIGameInstance|BPIGIIncrementStats(Message) (Game|GetGameInstance) false "NewEnumerator0" false false true false false false)
    (Audio|PlaySound2D "/Engine/VREditor/Sounds/UI/Gizmo_Handle_Clicked.Gizmo_Handle_Clicked" 1.0 1.0 0.0 0 0)
    (Actor|DestroyActor)))

(event EventBeginPlay
  (bind _returnvalue (Utilities|GetDataTableRow "/Game/HorrorHo/Data/DataTable/DT_GeneralGameParams.DT_GeneralGameParams" "Settings")
    (:then
      (Variables|Default|SetLiveTimer (.ItemDestroyTimer (Utilities|Struct|BreakStruct_GeneralGameParams _returnvalue)))
      (bind _returnvalue_2 (Utilities|Time|SetTimerbyEvent (EventDispatchers|CreateEvent :!event TickLiveTimer) (Variables|Default|GetTickFreq) true))
      (Variables|Default|SetHandle _returnvalue_2))))

(fn ConstructionScript)

(fn TickLiveTimer
  (bind _returnvalue (Game|GetPlayerCharacter 0))
  (bind _returnvalue_2 (Transformation|GetActorLocation))
  (bind _returnvalue_3 (Transformation|GetActorLocation _returnvalue))
  (bind _returnvalue_4 (- _returnvalue_3 _returnvalue_2))
  (bind _returnvalue_5 (Math|Vector|Normalize _returnvalue_4))
  (Transformation|SetWorldRotation (Variables|Default|GetWidget) (Math|Conversions|RotationFromXVector (Math|Vector|MakeVector (.x _returnvalue_5) (.y _returnvalue_5) 0.0)) false false)
  (bind _output_get (Variables|Default|SetLiveTimer (- (Variables|Default|GetLiveTimer) (Variables|Default|GetTickFreq))))
  (if (<= _output_get 0.0)
    (Utilities|Time|ClearandInvalidateTimerbyHandle (Variables|Default|GetHandle))
    (Actor|DestroyActor)))