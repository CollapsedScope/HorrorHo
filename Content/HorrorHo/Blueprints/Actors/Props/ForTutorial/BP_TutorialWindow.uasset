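; Tutorial window prop that can swap its mesh and show a pulsing highlight outline.
; ChangeWindowMesh switches the main component to the BO_windowc mesh.
; ShowOutline reveals a separate outline mesh with a dynamic material and starts a looping 60 Hz timer, evidently driving CalculateOutlineScale, which loops a float curve into the material's Scale parameter.
; ClearOutline stops the timer, zeroes Scale and hides the outline mesh.
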(event Custom|ChangeWindowMesh
  (Components|StaticMesh|SetStaticMesh (Variables|Debug|GetStaticMeshComponent) "/Game/Art/Atlas/MDL/BlockOut/BO_windowc.BO_windowc"))

(event Custom|ClearOutline
  (Utilities|Time|ClearandInvalidateTimerbyHandle (Variables|Default|GetOutlineScaleTimer))
  (Rendering|Material|SetScalarParameterValue (Variables|Default|GetOutlineMat) "Scale" 0.0 :!class /Script/Engine.MaterialInstanceDynamic)
  (Development|SetHiddeninGame (Variables|Default|GetStaticMesh) true false))

(event Custom|ShowOutline
  (bind _returnvalue (Rendering|Material|CreateDynamicMaterialInstance "/Game/HorrorHo/Materials/MI_Outline.MI_Outline" "None" "None" :!class /Script/Engine.KismetMaterialLibrary))
  (bind _output_get (Variables|Default|SetOutlineMat _returnvalue))
  (Rendering|Material|SetMaterial (Variables|Default|GetStaticMesh) 0 _output_get)
  (bind _returnvalue_2 (Utilities|Time|SetTimerbyEvent (EventDispatchers|CreateEvent :!event CalculateOutlineScale) (CallFunction|GetOneFrameTime 6e+01) true))
  (Variables|Default|SetOutlineScaleTimer _returnvalue_2)
  (Development|SetHiddeninGame (Variables|Default|GetStaticMesh) false false))

(event EventBeginPlay)

(event Collision|EventActorBeginOverlap
  (params (OtherActor :type Actor%20Object%20Reference)))

(event EventTick
  (params (DeltaSeconds :type Float%20%28single-precision%29)))

(fn ConstructionScript)

(fn CalculateOutlineScale
  (bind _outlinescalecurve (Variables|Default|GetOutlineScaleCurve))
  (bind _output_get (Variables|Default|SetCurrentTime (+ (Variables|Default|GetCurrentTime) (CallFunction|GetOneFrameTime 6e+01))))
  (Rendering|Material|SetScalarParameterValue (Variables|Default|GetOutlineMat) "Scale" (Math|Curves|GetFloatValue _outlinescalecurve (Math|Float|%(Float) _output_get (.MaxTime (Math|Curves|GetTimeRange _outlinescalecurve)))) :!class /Script/Engine.MaterialInstanceDynamic))