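; Tutorial radio prop that can start or stop its audio and shows an animated outline.
; BeginPlay silences the audio, puts a dynamic outline material on StaticMesh1 and starts a looping timer at a 60 fps interval.
; CalculateOutlineScale drives the material's Scale from a looping float curve.
; ClearOutline stops the timer, zeroes the scale and hides the outline mesh.
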(event Custom|Play
  (params (Play? :type Boolean))
  (bind _audio (Variables|Default|GetAudio))
  (if Play?
    (Audio|Components|Audio|Play _audio 0.0)
    (else
      (Audio|Components|Audio|Stop _audio))))

(event Custom|ClearOutline
  (Utilities|Time|ClearandInvalidateTimerbyHandle (Variables|Default|GetOutlineScaleTimer))
  (Rendering|Material|SetScalarParameterValue (Variables|Default|GetOutlineMat) "Scale" 0.0 :!class /Script/Engine.MaterialInstanceDynamic)
  (Development|SetHiddeninGame (Variables|Default|GetStaticMesh1) true false))

(event EventBeginPlay
  (Audio|Components|Audio|Stop (Variables|Default|GetAudio))
  (bind _returnvalue (Rendering|Material|CreateDynamicMaterialInstance "/Game/HorrorHo/Materials/MI_Outline.MI_Outline" "None" "None" :!class /Script/Engine.KismetMaterialLibrary))
  (bind _output_get (Variables|Default|SetOutlineMat _returnvalue))
  (Rendering|Material|SetMaterial (Variables|Default|GetStaticMesh1) 0 _output_get)
  (bind _returnvalue_2 (Utilities|Time|SetTimerbyEvent (EventDispatchers|CreateEvent :!event CalculateOutlineScale) (CallFunction|GetOneFrameTime 6e+01) true))
  (Variables|Default|SetOutlineScaleTimer _returnvalue_2))

(fn ConstructionScript)

(fn CalculateOutlineScale
  (bind _outlinescalecurve (Variables|Default|GetOutlineScaleCurve))
  (bind _output_get (Variables|Default|SetCurrentTime (+ (Variables|Default|GetCurrentTime) (CallFunction|GetOneFrameTime 6e+01))))
  (Rendering|Material|SetScalarParameterValue (Variables|Default|GetOutlineMat) "Scale" (Math|Curves|GetFloatValue _outlinescalecurve (Math|Float|%(Float) _output_get (.MaxTime (Math|Curves|GetTimeRange _outlinescalecurve)))) :!class /Script/Engine.MaterialInstanceDynamic))