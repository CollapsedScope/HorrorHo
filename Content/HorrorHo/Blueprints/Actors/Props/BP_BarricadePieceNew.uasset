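; A single barricade piece prop that picks one of three wooden mesh variants at random and can show damage or be hidden.
; The random pick runs in the construction script and again on BeginPlay, also setting the damage-state materials for variants B and C, but not A.
; Custom events swap between healthy, light and heavy damage materials and toggle visibility, restoring the healthy material when a hidden piece reappears.
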(event EventBeginPlay
  (CallFunction|ChooseRandomBarricadePieceType))

(event Collision|EventActorBeginOverlap
  (params (OtherActor :type Actor%20Object%20Reference)))

(event EventTick
  (params (DeltaSeconds :type Float%20%28single-precision%29)))

(event EventBarricadePieceSwapMaterial
  (params (MaterialSwitch :type Integer))
  (switch int MaterialSwitch
    (:0
      (Rendering|Material|SetMaterial (Variables|Default|GetBarricadeMesh) 0 (Variables|Default|GetMatHealthy)))
    (:1
      (Rendering|Material|SetMaterial (Variables|Default|GetBarricadeMesh) 0 (Variables|Default|GetMatLightDamage)))
    (:2
      (Rendering|Material|SetMaterial (Variables|Default|GetBarricadeMesh) 0 (Variables|Default|GetMatHeavyDamage)))))

(event EventBarricadePieceToggleVisibility
  (params (IsVisible :type Boolean))
  (bind _barricademesh (Variables|Default|GetBarricadeMesh))
  (if IsVisible
    (if (not (Rendering|IsVisible _barricademesh))
      (Rendering|SetVisibility _barricademesh true false)
      (Rendering|Material|SetMaterial (Variables|Default|GetBarricadeMesh) 0 (Variables|Default|GetMatHealthy)))
    (else
      (Rendering|SetVisibility (Variables|Default|GetBarricadeMesh) false false))))

(fn ConstructionScript
  (CallFunction|ChooseRandomBarricadePieceType))

(fn ChooseRandomBarricadePieceType
  (bind _barricademesh (Variables|Default|GetBarricadeMesh))
  (bind _barricademesh_2 (Variables|Default|GetBarricadeMesh))
  (bind _barricademesh_3 (Variables|Default|GetBarricadeMesh))
  (switch int (Math|Random|RandomIntegerinRange 0 2)
    (:0
      (Components|StaticMesh|SetStaticMesh _barricademesh_2 "/Game/Art/Eda/MDL/Barricade/BarricadeA.BarricadeA")
      (Rendering|Material|SetMaterial _barricademesh_2 0 "/Game/Art/Eda/MTL/MI/Wood/MI_WoodA.MI_WoodA"))
    (:1
      (Components|StaticMesh|SetStaticMesh _barricademesh_3 "/Game/Art/Eda/MDL/Barricade/BarricadeB.BarricadeB")
      (Rendering|Material|SetMaterial _barricademesh_3 0 "/Game/Art/Eda/MTL/MI/Wood/MI_WoodB.MI_WoodB")
      (Variables|Default|SetMatHealthy "/Game/Art/Eda/MTL/MI/Wood/MI_WoodB.MI_WoodB")
      (Variables|Default|SetMatLightDamage "/Game/Art/Eda/MTL/MI/Wood/MI_WoodB30.MI_WoodB30")
      (Variables|Default|SetMatHeavyDamage "/Game/Art/Eda/MTL/MI/Wood/MI_WoodB60.MI_WoodB60"))
    (:2
      (Components|StaticMesh|SetStaticMesh _barricademesh "/Game/Art/Eda/MDL/Barricade/BarricadeC.BarricadeC")
      (Rendering|Material|SetMaterial _barricademesh 0 "/Game/Art/Eda/MTL/MI/Wood/MI_WoodC.MI_WoodC")
      (Variables|Default|SetMatHealthy "/Game/Art/Eda/MTL/MI/Wood/MI_WoodC.MI_WoodC")
      (Variables|Default|SetMatLightDamage "/Game/Art/Eda/MTL/MI/Wood/MI_WoodC30.MI_WoodC30")
      (Variables|Default|SetMatHeavyDamage "/Game/Art/Eda/MTL/MI/Wood/MI_WoodC60.MI_WoodC60"))))