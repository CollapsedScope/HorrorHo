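; Barricade piece prop that shows damage and repair states for a barricade.
; On construction and again at BeginPlay it randomly picks one of three wood variants, caching its normal, light and heavy damage meshes plus a dynamic repair material.
; Interface events swap the mesh by health thresholds, toggle visibility, and apply or remove the repair material, stamping a StartTime parameter to time its effect.
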(event EventBeginPlay
  (CallFunction|ChooseRandomBarricadePieceType))

(event Collision|EventActorBeginOverlap
  (params (OtherActor :type Actor%20Object%20Reference)))

(event EventTick
  (params (DeltaSeconds :type Float%20%28single-precision%29)))

(event EventBPISetRepairMaterial
  (bind _repairmat (Variables|Default|GetRepairMat))
  (Rendering|Material|SetMaterial (Variables|Default|GetBarricadeMesh) 0 _repairmat)
  (Rendering|Material|SetScalarParameterValue _repairmat "StartTime" (Utilities|Time|GetGameTimeinSeconds) :!class /Script/Engine.MaterialInstanceDynamic))

(event EventBPIRemoveRepairMaterial
  (Rendering|Material|SetMaterial (Variables|Default|GetBarricadeMesh) 0 (Rendering|Material|GetMaterial (Variables|Default|GetMeshNormal) 0)))

(event EventBPISwapMaterial
  (params (HealthPercent :type Float%20%28single-precision%29))
  (if (> HealthPercent (Variables|Default|GetThresholdLight))
    (Components|StaticMesh|SetStaticMesh (Variables|Default|GetBarricadeMesh) (Variables|Default|GetMeshNormal))
    (elif (> HealthPercent (Variables|Default|GetThresholdHeavy))
      (Components|StaticMesh|SetStaticMesh (Variables|Default|GetBarricadeMesh) (Variables|Default|GetMeshLightDamage))
      (else
        (Components|StaticMesh|SetStaticMesh (Variables|Default|GetBarricadeMesh) (Variables|Default|GetMeshHeavyDamage))))))

(event EventBPIToggleVisibility
  (params (IsVisible :type Boolean))
  (bind _barricademesh (Variables|Default|GetBarricadeMesh))
  (if IsVisible
    (if (not (Rendering|IsVisible _barricademesh))
      (Rendering|SetVisibility _barricademesh true false))
    (else
      (Rendering|SetVisibility (Variables|Default|GetBarricadeMesh) false false))))

(fn ConstructionScript
  (CallFunction|ChooseRandomBarricadePieceType))

(fn ChooseRandomBarricadePieceType
  (switch int (Math|Random|RandomIntegerinRange 0 2)
    (:0
      (Components|StaticMesh|SetStaticMesh (Variables|Default|GetBarricadeMesh) "/Game/Art/Eda/MDL/Barricade/M/BarricadeA.BarricadeA")
      (Variables|Default|SetMeshNormal "/Game/Art/Eda/MDL/Barricade/M/BarricadeA.BarricadeA")
      (Variables|Default|SetMeshLightDamage "/Game/Art/Eda/MDL/Barricade/M/BarricadeA30.BarricadeA30")
      (Variables|Default|SetMeshHeavyDamage "/Game/Art/Eda/MDL/Barricade/M/BarricadeA60.BarricadeA60")
      (bind _returnvalue (Rendering|Material|CreateDynamicMaterialInstance "/Game/Art/Eda/MTL/MI/Wood/MI_WoodA0.MI_WoodA0" "None" "None" :!class /Script/Engine.KismetMaterialLibrary))
      (Variables|Default|SetRepairMat _returnvalue))
    (:1
      (Components|StaticMesh|SetStaticMesh (Variables|Default|GetBarricadeMesh) "/Game/Art/Eda/MDL/Barricade/M/BarricadeB.BarricadeB")
      (Variables|Default|SetMeshNormal "/Game/Art/Eda/MDL/Barricade/M/BarricadeB.BarricadeB")
      (Variables|Default|SetMeshLightDamage "/Game/Art/Eda/MDL/Barricade/M/BarricadeB30.BarricadeB30")
      (Variables|Default|SetMeshHeavyDamage "/Game/Art/Eda/MDL/Barricade/M/BarricadeB60.BarricadeB60")
      (bind _returnvalue_2 (Rendering|Material|CreateDynamicMaterialInstance "/Game/Art/Eda/MTL/MI/Wood/MI_WoodB0.MI_WoodB0" "None" "None" :!class /Script/Engine.KismetMaterialLibrary))
      (Variables|Default|SetRepairMat _returnvalue_2))
    (:2
      (Components|StaticMesh|SetStaticMesh (Variables|Default|GetBarricadeMesh) "/Game/Art/Eda/MDL/Barricade/M/BarricadeC.BarricadeC")
      (Variables|Default|SetMeshNormal "/Game/Art/Eda/MDL/Barricade/M/BarricadeC.BarricadeC")
      (Variables|Default|SetMeshLightDamage "/Game/Art/Eda/MDL/Barricade/M/BarricadeC30.BarricadeC30")
      (Variables|Default|SetMeshHeavyDamage "/Game/Art/Eda/MDL/Barricade/M/BarricadeC60.BarricadeC60")
      (bind _returnvalue_3 (Rendering|Material|CreateDynamicMaterialInstance "/Game/Art/Eda/MTL/MI/Wood/MI_WoodC0.MI_WoodC0" "None" "None" :!class /Script/Engine.KismetMaterialLibrary))
      (Variables|Default|SetRepairMat _returnvalue_3))))