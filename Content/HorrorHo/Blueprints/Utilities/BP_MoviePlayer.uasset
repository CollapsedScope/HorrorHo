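; Movie player actor that shows full-screen videos through a MediaPlayer and UI_Movie widget, driven by BPI_MoviePlayer calls.
; Interface events set the file, show black, play with fades or immediately, stop and close the screen.
; Looping per-frame timers poll until playback begins before revealing the video.
; It tracks playback state, disables player movement until the movie ends or stops, and briefly shows UI text on key press.
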(event EventBeginPlay
  (bind _returnvalue (UserInterface|CreateWidget "/Game/HorrorHo/Blueprints/Widgets/UI_Movie.UI_Movie_C"))
  (Variables|Default|SetMovieWidget _returnvalue)
  (Media|MediaPlayer|BindEventtoOnEndReached (Variables|Default|GetMediaPlayer) (EventDispatchers|CreateEvent :!event OnEndReached)))

(event EventTick
  (params (DeltaSeconds :type Float%20%28single-precision%29)))

(event EventBPIMoviePlayerPlayAfterFadeOut
  ;[1 1 1] 既に黒画面の状態からフェードアウトして、映像を再生する。ただし、映像が再生可能になるまでは黒画面状態をつづける。
  (CallFunction|PlayMovie)
  (bind _returnvalue (Utilities|Time|SetTimerbyEvent (EventDispatchers|CreateEvent :!event FadeinAfterMovieLoaded) (CallFunction|GetOneFrameTime 6e+01) true))
  (Variables|Default|SetLoad-MovieTimer _returnvalue))

(event EventBPIMoviePlayerPlayAfterDarkChange
  (bind _moviewidget (Variables|Default|GetMovieWidget))
  ;[1 1 1] ゲーム画面を描画している状態から、フェードを入れて、映像を再生する。ただし、映像が再生可能になるまでは黒画面状態をつづける。
  (Default|StartFadeOut _moviewidget)
  (EventDispatchers|BindEventtoDispatchEventAfterFadein _moviewidget (delegate EventBPIMoviePlayerPlayAfterFadeOut)))

(event EventBPIMoviePlayerPlayImmediately
  ;[1 1 1] 映像の再生準備ができたら即時映像再生
  (bind _returnvalue (Utilities|Time|SetTimerbyEvent (EventDispatchers|CreateEvent :!event AddtoViewportAfterMovieLoaded) (CallFunction|GetOneFrameTime 6e+01) true))
  (Variables|Default|SetLoad-MovieTimer _returnvalue))

(event EventBPIMoviePlayerBlackScreen
  (bind _moviewidget (Variables|Default|GetMovieWidget))
  ;[1 1 1] 黒画面表示
  (Default|DarkenScreen _moviewidget)
  (if (not (UserInterface|Viewport|IsinViewport _moviewidget))
    (UserInterface|Viewport|AddtoViewport _moviewidget 0)))

(event EventBPIMoviePlayerSetMovieFile
  (params (MovieFile :type File%20Media%20Source%20Object%20Reference))
  ;[1 1 1] 次に再生する映像を設定
  (Variables|Default|SetCurrentMovieFileRef MovieFile))

(event EventBPIMoviePlayerCloseScreen
  (bind _moviewidget (Variables|Default|GetMovieWidget))
  (if (UserInterface|Viewport|IsinViewport _moviewidget)
    (Widget|RemovefromParent _moviewidget)))

(event EventBPIMoviePlayerStopImmediately
  (Utilities|Time|ClearandInvalidateTimerbyHandle (Variables|Default|GetTickTimer))
  (Media|MediaPlayer|Close (Variables|Default|GetMediaPlayer) :!class /Script/MediaAssets.MediaPlayer)
  (Variables|Default|SetMoviePlayerState "NewEnumerator3")
  (CallFunction|OnEndReached))

(fn PlayMovie
  (bind _moviewidget (Variables|Default|GetMovieWidget))
  (Media|MediaPlayer|OpenSource (Variables|Default|GetMediaPlayer) (Variables|Default|GetCurrentMovieFileRef))
  (Variables|Default|SetMoviePlayerState "NewEnumerator0")
  (if (not (UserInterface|Viewport|IsinViewport _moviewidget))
    (UserInterface|Viewport|AddtoViewport _moviewidget 0)))

(fn CheckHasLoadedMovie
  (return (Audio|Components|Audio|IsPlaying (Variables|Default|GetMediaPlayer))))

(fn FadeinAfterMovieLoaded
  (if (CallFunction|CheckHasLoadedMovie)
    (Default|StartFadein (Variables|Default|GetMovieWidget))
    (Utilities|Time|ClearandInvalidateTimerbyHandle (Variables|Default|GetLoad-MovieTimer))
    (Variables|Default|SetMoviePlayerState "NewEnumerator2")
    (CallFunction|OnStartPlaying)))

(fn AddtoViewportAfterMovieLoaded
  (bind _moviewidget (Variables|Default|GetMovieWidget))
  (if (CallFunction|CheckHasLoadedMovie)
    (Utilities|Time|ClearandInvalidateTimerbyHandle (Variables|Default|GetLoad-MovieTimer))
    (Variables|Default|SetMoviePlayerState "NewEnumerator2")
    (CallFunction|OnStartPlaying)
    (if (not (UserInterface|Viewport|IsinViewport _moviewidget))
      (UserInterface|Viewport|AddtoViewport _moviewidget 0))))

(fn PauseMovie
  (bind _mediaplayer (Variables|Default|GetMediaPlayer))
  (if (and (Audio|Components|Audio|IsPlaying _mediaplayer) (Class|MediaPlayer|CanPause _mediaplayer))
    (Sequencer|Player|Pause _mediaplayer)))

(fn ResumeMovie
  (bind _mediaplayer (Variables|Default|GetMediaPlayer))
  (if (Class|MediaPlayer|IsPaused _mediaplayer)
    (Media|MediaPlayer|Play _mediaplayer :!class /Script/MediaAssets.MediaPlayer)))

(fn OnEndReached
  (Variables|Default|SetMoviePlayerState "NewEnumerator3")
  (Utilities|Time|ClearandInvalidateTimerbyHandle (Variables|Default|GetTickTimer))
  (Media|MediaPlayer|Close (Variables|Default|GetMediaPlayer) :!class /Script/MediaAssets.MediaPlayer)
  (Class|BPIPlayer|BPIPlayerEnabletoMove(Message) (Game|GetPlayerCharacter 0) true))

(fn OnStartPlaying
  (Class|BPIPlayer|BPIPlayerEnabletoMove(Message) (Game|GetPlayerCharacter 0) false))

(fn OnAnyKey
  (if (Utilities|Enum|Equal(Enum) (Variables|Default|GetMoviePlayerState) "NewEnumerator2")
    (Default|ShowUIText (Variables|Default|GetMovieWidget) true)
    (bind _returnvalue (Utilities|Time|SetTimerbyEvent (EventDispatchers|CreateEvent :!event OnKeyKeepReleased) 5.0))
    (Variables|Default|SetAnyKeyTimer _returnvalue)))

(fn OnKeyKeepReleased
  (Utilities|Time|ClearandInvalidateTimerbyHandle (Variables|Default|GetAnyKeyTimer))
  (Default|ShowUIText (Variables|Default|GetMovieWidget) false))

(fn BPIMoviePlayerGetState
  (return (Variables|Default|GetMoviePlayerState)))