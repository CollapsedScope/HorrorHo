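; Zombie spawn manager that sorts the level's BP_Spawner actors into per-type arrays at BeginPlay, then pulses one Walker from every eligible spawner.
; SpawnZombies picks the array by type, though every type currently uses BP_ZombieBase, and spawns at random spawners or, in pulse mode, all of them.
; Each zombie records its spawner and gets a BP_ZombieController with an initialized blackboard.
; Wave table lookup is unconnected, so no wave progression runs.
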(event EventBeginPlay
  (Initialization|SaveSpawnerArrays)
  (Spawn|SpawnZombies "NewEnumerator0" 1 true))

(event EventTick
  (params (DeltaSeconds :type Float%20%28single-precision%29)))

(fn SaveSpawnerArrays
  (bind _outactors (Actor|GetAllActorsOfClass "/Game/HorrorHo/Blueprints/Actors/Installation/BP_Spawner.BP_Spawner_C"))
  (for _array_element _outactors
    (Initialization|AddSpawnertoArrays _array_element))
  (return))

(fn AddSpawnertoArrays
  (params (New%20Spawner :type BP%20Spawner%20Object%20Reference))
  (bind _spawnsettings (Variables|/Game/HorrorHo/Blueprints/Actors/Installation/BP_Spawner.BP_Spawner_C|GetSpawnSettings New%20Spawner))
  (bind (_canspawnwalker _canspawnrunner _canspawncrawler _canspawnbomber _canspawnscreamer _canspawnwatcher _canspawnworm) (Utilities|Struct|BreakStruct_SpawnerSettings _spawnsettings))
  (LocalVariables|SetSpawner New%20Spawner)
  (Utilities|FlowControl|Sequence
    (:then_0
      (if _canspawnwalker
        (Utilities|Array|Add (Variables|Spawners|GetWalkerSpawners) (LocalVariables|GetSpawner))))
    (:then_1
      (if _canspawnrunner
        (Utilities|Array|Add (Variables|Spawners|GetRunnerSpawners) (LocalVariables|GetSpawner))))
    (:then_2
      (if _canspawncrawler
        (Utilities|Array|Add (Variables|Spawners|GetCrawlerSpawners) (LocalVariables|GetSpawner))))
    (:then_3
      (if _canspawnbomber
        (Utilities|Array|Add (Variables|Spawners|GetBomberSpawners) (LocalVariables|GetSpawner))))
    (:then_4
      (if _canspawnscreamer
        (Utilities|Array|Add (Variables|Spawners|GetScreamerSpawners) (LocalVariables|GetSpawner))))
    (:then_5
      (if _canspawnwatcher
        (Utilities|Array|Add (Variables|Spawners|GetWatcherSpawners) (LocalVariables|GetSpawner))))
    (:then_6
      (if _canspawnworm
        (Utilities|Array|Add (Variables|Spawners|GetWormSpawners) (LocalVariables|GetSpawner))))))

(fn SpawnZombies
  (params (Zombie%20Type :type EZombieType%20Enum :default "NewEnumerator0") (Number%20of%20Zombies :type Integer) (IsPulse :type Boolean))
  (switch Utilities|FlowControl|Switch|SwitchonEZombieType Zombie%20Type
    (:NewEnumerator0
      (LocalVariables|SetZombieClass "/Game/HorrorHo/Blueprints/Characters/BP_ZombieBase.BP_ZombieBase_C")
      (LocalVariables|SetSpawnerArray (Variables|Spawners|GetWalkerSpawners)))
    (:NewEnumerator1
      (LocalVariables|SetZombieClass "/Game/HorrorHo/Blueprints/Characters/BP_ZombieBase.BP_ZombieBase_C")
      (LocalVariables|SetSpawnerArray (Variables|Spawners|GetRunnerSpawners)))
    (:NewEnumerator2
      (LocalVariables|SetZombieClass "/Game/HorrorHo/Blueprints/Characters/BP_ZombieBase.BP_ZombieBase_C")
      (LocalVariables|SetSpawnerArray (Variables|Spawners|GetCrawlerSpawners)))
    (:NewEnumerator3
      (LocalVariables|SetZombieClass "/Game/HorrorHo/Blueprints/Characters/BP_ZombieBase.BP_ZombieBase_C")
      (LocalVariables|SetSpawnerArray (Variables|Spawners|GetBomberSpawners)))
    (:NewEnumerator4
      (LocalVariables|SetZombieClass "/Game/HorrorHo/Blueprints/Characters/BP_ZombieBase.BP_ZombieBase_C")
      (LocalVariables|SetSpawnerArray (Variables|Spawners|GetScreamerSpawners)))
    (:NewEnumerator5
      (LocalVariables|SetZombieClass "/Game/HorrorHo/Blueprints/Characters/BP_ZombieBase.BP_ZombieBase_C")
      (LocalVariables|SetSpawnerArray (Variables|Spawners|GetWatcherSpawners)))
    (:NewEnumerator6
      (LocalVariables|SetZombieClass "/Game/HorrorHo/Blueprints/Characters/BP_ZombieBase.BP_ZombieBase_C")
      (LocalVariables|SetSpawnerArray (Variables|Spawners|GetWormSpawners))))
  (for _index (range 1 (Math|Integer|Max(Integer) Number%20of%20Zombies 1))
    (if IsPulse
      (CallFunction|SpawnZombiePulsefromClass (LocalVariables|GetZombieClass) (LocalVariables|GetSpawnerArray))
      (else
        (CallFunction|SpawnZombiefromClass (LocalVariables|GetZombieClass) (LocalVariables|GetSpawnerArray))))))

(fn SpawnZombiefromClass
  (params (ZombieClass :type Actor%20Class%20Reference) (SpawnerArray :type Array%20of%20BP%20Spawner%20Object%20References))
  (bind _outitem (Utilities|Array|Random SpawnerArray))
  (bind _spawnlocation (Variables|/Game/HorrorHo/Blueprints/Actors/Installation/BP_Spawner.BP_Spawner_C|GetSpawnLocation _outitem))
  (bind _returnvalue (Transformation|GetWorldTransform _spawnlocation))
  (CallFunction|SpawnZombieandController ZombieClass (Math|Transform|MakeTransform (.location _returnvalue) (.rotation _returnvalue)) _outitem))

(fn SpawnZombiePulsefromClass
  (params (ZombieClass :type Actor%20Class%20Reference) (SpawnerArray :type Array%20of%20BP%20Spawner%20Object%20References))
  (for _array_element SpawnerArray
    (CallFunction|SpawnZombieandController ZombieClass (Math|Transform|MakeTransform (.location (Transformation|GetWorldTransform (Variables|/Game/HorrorHo/Blueprints/Actors/Installation/BP_Spawner.BP_Spawner_C|GetSpawnLocation _array_element))) (.rotation (Transformation|GetWorldTransform (Variables|/Game/HorrorHo/Blueprints/Actors/Installation/BP_Spawner.BP_Spawner_C|GetSpawnLocation _array_element)))) _array_element)))

(fn SpawnZombieandController
  (params (Class :type Actor%20Class%20Reference) (SpawnTransform :type Transform) (Spawner :type BP%20Spawner%20Object%20Reference))
  (bind _returnvalue (Game|SpawnActorfromClass Class SpawnTransform "AdjustIfPossibleButAlwaysSpawn" 0 0))
  (bind _zombiecharacter (Class|BPZombieCharacterInterface|ZCharGetZombieCharacter(Message) _returnvalue))
  (Variables|/Game/HorrorHo/Blueprints/Characters/BP_ZombieBase.BP_ZombieBase_C|SetOriginalSpawner _zombiecharacter Spawner)
  (bind _returnvalue_2 (Game|SpawnActorfromClass "/Game/HorrorHo/Blueprints/Controller/BP_ZombieController.BP_ZombieController_C" (Transformation|GetActorTransform _zombiecharacter) "Undefined" 0 0))
  (Pawn|Possess _returnvalue_2 _zombiecharacter)
  (Default|InitBlackBoard _returnvalue_2))