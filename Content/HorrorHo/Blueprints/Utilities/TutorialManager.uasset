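; Tutorial manager that runs data-asset-driven tutorials, currently handling only the Movement phase of the Tutorial Level type.
; On BeginPlay it waits the asset's initial delay, then calls an interface next-phase event that delays again and prints the current set's title and explanation.
; An interface axis check records input direction, but the forward pair is overwritten with opposite values, so its advance condition never passes; State is never changed here.
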(event Custom|StartTutorial
  (bind _tutorialdataasset (Variables|Default|GetTutorialDataAsset)
    (:then
      (Utilities|FlowControl|Delay (Variables|/Game/HorrorHo/Data/DataAssets/ParentBP/TutorialSetData_BPP.TutorialSetData_BPP_C|GetInitialStartDelayTime (Utilities|ResolveSoftReference _tutorialdataasset)))
      (CallFunction|BPITutorialNextPhase))
    (:else)))

(event EventBeginPlay
  (CallFunction|StartTutorial))

(event EventTick
  (params (DeltaSeconds :type Float%20%28single-precision%29)))

(event EventBPITutorialNextPhase
  (bind _state (Variables|Default|GetState))
  (bind _tutorialdataasset (Variables|Default|GetTutorialDataAsset))
  (bind _returnvalue (Math|Conversions|ToInteger(Byte) _state))
  (bind _output (Utilities|ResolveSoftReference _tutorialdataasset))
  (bind _tutorialsets (Variables|/Game/HorrorHo/Data/DataAssets/ParentBP/TutorialSetData_BPP.TutorialSetData_BPP_C|GetTutorialSets _output))
  (bind _output_2 (Utilities|Array|Get(acopy) _tutorialsets _returnvalue))
  (bind (_header _buttonicon _title _explanation) (Utilities|Struct|BreakStruct_TutorialSet _output_2))
  (Utilities|FlowControl|Delay (Variables|/Game/HorrorHo/Data/DataAssets/ParentBP/TutorialSetData_BPP.TutorialSetData_BPP_C|GetDelayTime _output))
  (switch Utilities|FlowControl|Switch|SwitchonETutorialType (Variables|/Game/HorrorHo/Data/DataAssets/ParentBP/TutorialSetData_BPP.TutorialSetData_BPP_C|GetTutorialType _output)
    (:NewEnumerator0
      (switch Utilities|FlowControl|Switch|SwitchonETutorialLevelPhase (Utilities|Enum|ByteToEnumETutorialLevelPhase _state)
        (:NewEnumerator0
          (Development|PrintString (Utilities|String|ToString(Text) _title))
          (Development|PrintString (Utilities|String|ToString(Text) _explanation)))))))

(event EventBPITutorialCheckAxisValue
  (params (AxisValue :type Float%20%28single-precision%29) (IsForward :type Boolean))
  (bind _movementcheck (Variables|Default|GetMovementCheck))
  (bind _movementcheck_2 (Variables|Default|GetMovementCheck))
  (bind _output (Utilities|Array|Get(acopy) _movementcheck 2))
  (bind _output_2 (Utilities|Array|Get(acopy) _movementcheck_2 3))
  (if IsForward
    (|SetBy-RefVar _output (>= AxisValue 0.0))
    (|SetBy-RefVar _output_2 (< AxisValue 0.0))
    (if (and _output _output_2)
      (CallFunction|BPITutorialNextPhase))
    (else
      (|SetBy-RefVar (Utilities|Array|Get(acopy) (Variables|Default|GetMovementCheck)) (>= AxisValue 0.0))
      (|SetBy-RefVar (Utilities|Array|Get(acopy) (Variables|Default|GetMovementCheck) 1) (< AxisValue 0.0)))))