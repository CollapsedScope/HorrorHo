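; Game mode for a zombie wave mode that spawns the wave manager, owns the screen fade widget and coordinates living zombies.
; A looping timer manages active zombies, with distance sorting by last nav distance to order attacks from the closest few.
; The nearest four feed a radar through a material parameter collection updated each tick with player position and camera direction.
; It also tracks remaining zombies for wave-clear checks, debug readouts and a kill switch.
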(event EventBeginPlay
  (CallFunction|SetDTParams)
  (bind _returnvalue (UserInterface|CreateWidget "/Game/HorrorHo/Blueprints/Widgets/UI_BlackScreen.UI_BlackScreen_C"))
  (bind _output_get (Variables|Default|SetFadeWidget _returnvalue))
  (UserInterface|Viewport|AddtoViewport _output_get 1)
  (CallFunction|GMFadein))

(event EventTick
  (params (DeltaSeconds :type Float%20%28single-precision%29))
  (CallFunction|UpdateZombieRadar))

(event EventGMSetWaveManager
  (params (WaveData :type Data%20Table%20Object%20Reference))
  (bind _returnvalue (Game|AddComponentbyClass "/Game/HorrorHo/Blueprints/Utilities/BP_WaveManager.BP_WaveManager_C"))
  (bind _output_get (Variables|Default|SetWaveManager _returnvalue))
  (Utilities|IsValid WaveData
    (:Is%20Valid
      (Variables|/Game/HorrorHo/Blueprints/Utilities/BP_WaveManager.BP_WaveManager_C|SetWaveTable _output_get WaveData))
    (:Is%20Not%20Valid
      _))
  (Default|BeginWaveManager _output_get))

(event EventGMAddActiveZombie
  (params (NewZombie :type BP%20Zombie%20Base%20Object%20Reference))
  (Utilities|Array|Add (Variables|Default|GetActiveZombieArray) NewZombie)
  ;[1 1 1] If there is a new active zombie and the handle to update them isnt activated yet, activate it
  (if (not (Utilities|Time|IsValidTimerHandle (Variables|Default|GetActiveZombieTimerHandle)))
    (bind _returnvalue (Utilities|Time|SetTimerbyEvent (EventDispatchers|CreateEvent :!event QueryActiveZombies) (Variables|Default|GetActiveZombieUpdateFreq) true))
    (Variables|Default|SetActiveZombieTimerHandle _returnvalue)))

(fn ConstructionScript)

(fn QueryRemainingZombies
  (bind _remainingzombiearray (Variables|Default|GetRemainingZombieArray))
  (if (Utilities|Array|IsValidIndex (Variables|Default|GetRemainingZombieArray))
    (for (_array_element _array_index) _remainingzombiearray
      (Utilities|IsValid _array_element
        (:Is%20Not%20Valid
          (Utilities|Array|RemoveIndex _remainingzombiearray _array_index))))
    (if (not (Utilities|Array|IsValidIndex _remainingzombiearray))
      (Utilities|Time|ClearandInvalidateTimerbyHandle (Variables|Default|GetPostWaveTimerHandle)))))

(fn QueryActiveZombies
  (bind _mostrecentdistances (LocalVariables|GetMostRecentDistances))
  (bind _indexofminvalue (Math|Float|MinOfFloatArray _mostrecentdistances))
  (if (Utilities|Array|IsValidIndex (Variables|Default|GetActiveZombieArray))
    (for (_array_element _array_index) (Variables|Default|GetActiveZombieArray)
      (Utilities|IsValid _array_element
        (:Is%20Valid
          (if (not (Game|IsActorBeingDestroyed _array_element))
            ;[1 1 1] Build array of distances to player
            (Utilities|Array|Add (LocalVariables|GetMostRecentDistances) (Variables|/Game/HorrorHo/Blueprints/Characters/Zombies/BP_ZombieBase.BP_ZombieBase_C|GetMostRecentNavDist _array_element))
            ;[1 1 1] Set all attack commands to false temporarily
            (Variables|/Game/HorrorHo/Blueprints/Characters/Zombies/BP_ZombieBase.BP_ZombieBase_C|SetAttackCommand _array_element false)
            (else
              ;[1 1 1] Remove invalid zombies
              (Utilities|Array|RemoveIndex (Variables|Default|GetActiveZombieArray) _array_index :!label _label))))
        (:Is%20Not%20Valid
          (goto _label))))
    (if (Utilities|Array|IsValidIndex (Variables|Default|GetActiveZombieArray))
      (Utilities|FlowControl|Sequence
        (:then_0
          ;[1 1 1] Sort zombies by distance
          (for _array_element_2 _mostrecentdistances
            (Utilities|Array|Add (LocalVariables|GetTempArray) (Utilities|Array|Get(acopy) (Variables|Default|GetActiveZombieArray) _indexofminvalue))
            (|SetBy-RefVar (Utilities|Array|Get(acopy) _mostrecentdistances _indexofminvalue) 1e+09)))
        (:then_1
          ;[1 1 1] Save the sorted array
          (Variables|Default|SetActiveZombieArray (LocalVariables|GetTempArray))
          ;[1 1 1] Reset radar zombies
          (Utilities|Array|Clear (Variables|Default|GetRadarZombies))
          (Utilities|FlowControl|Sequence
            (:then_0
              ;[1 1 1] Get the closest 4 zombies to update the radar
              (for _index (range 0 3)
                (if (Utilities|Array|IsValidIndex (Variables|Default|GetActiveZombieArray) _index)
                  (Utilities|Array|Add (Variables|Default|GetRadarZombies) (Utilities|Array|Get(acopy) (Variables|Default|GetActiveZombieArray) _index)))))
            (:then_1
              ;[1 1 1] Set attack commands for minimum number of zombies
              (for _index_2 (range 0 (- (Math|Integer|Min(Integer) (Variables|Default|GetMinimumAttackerCount) (Utilities|Array|Length (LocalVariables|GetMostRecentDistances))) 1))
                (if (not (Game|IsActorBeingDestroyed (Utilities|Array|Get(acopy) (Variables|Default|GetActiveZombieArray) _index_2)))
                  (Variables|/Game/HorrorHo/Blueprints/Characters/Zombies/BP_ZombieBase.BP_ZombieBase_C|SetAttackCommand (Utilities|Array|Get(acopy) (Variables|Default|GetActiveZombieArray) _index_2) true)))))))
      (else
        ;[1 1 1] If there are no more zombies, stop trying to update attack states
        (Utilities|Time|ClearandInvalidateTimerbyHandle (Variables|Default|GetActiveZombieTimerHandle))))))

(fn SetDTParams
  (bind _returnvalue (Utilities|GetDataTableRow "/Game/HorrorHo/Data/DataTable/DT_GeneralGameParams.DT_GeneralGameParams" "Settings")
    (:then
      (Variables|Default|SetMinimumAttackerCount (.MinimumAttackZombies (Utilities|Struct|BreakStruct_GeneralGameParams _returnvalue)))
      (Variables|Default|SetActiveZombieUpdateFreq (.AttackZombieUpdateFrequency (Utilities|Struct|BreakStruct_GeneralGameParams _returnvalue))))))

(fn UpdateZombieRadar
  (bind _radarzombies (Variables|Default|GetRadarZombies))
  ;[0.6446 1 0.552] Update the zombie radar
  (Utilities|FlowControl|Sequence
    (:then_0
      ;;[1 1 1] Save the camera direction (not usually available in UI materials)
      (Rendering|Material|SetVectorParameterValue "/Game/HorrorHo/UIMat/RadarParams.RadarParams" "CamDir" (Math|Conversions|ToLinearColor(Vector) (Transformation|GetActorForwardVector (Game|GetPlayerCameraManager 0))) :!class /Script/Engine.KismetMaterialLibrary))
    (:then_1
      ;;[1 1 1] Set player position in parameters
      (Rendering|Material|SetVectorParameterValue "/Game/HorrorHo/UIMat/RadarParams.RadarParams" "PlayerPos" (Math|Conversions|ToLinearColor(Vector) (Transformation|GetActorLocation (Game|Player|GetPlayerPawn 0))) :!class /Script/Engine.KismetMaterialLibrary))
    (:then_2
      ;;[1 1 1] Set zombie parameters
      (for _index (range 0 3)
        (if (Utilities|Array|IsValidIndex _radarzombies _index)
          (Utilities|IsValid (Utilities|Array|Get(acopy) _radarzombies _index)
            (:Is%20Valid
              (Rendering|Material|SetVectorParameterValue "/Game/HorrorHo/UIMat/RadarParams.RadarParams" (Utilities|String|StringToName (Utilities|String|Append "Pos" (Utilities|String|ToString(Integer) (+ _index 1)))) (Math|Conversions|ToLinearColor(Vector) (Transformation|GetActorLocation (Utilities|Array|Get(acopy) _radarzombies _index))) :!class /Script/Engine.KismetMaterialLibrary))
            (:Is%20Not%20Valid
              ;;;[1 1 1] Set arbitrary high value for invalid members so the radar isnt affected
              (Rendering|Material|SetVectorParameterValue "/Game/HorrorHo/UIMat/RadarParams.RadarParams" (Utilities|String|StringToName (Utilities|String|Append "Pos" (Utilities|String|ToString(Integer) (+ _index 1)))) (Utilities|Struct|MakeLinearColor 1e+08 1e+08 1e+08 1.0) :!class /Script/Engine.KismetMaterialLibrary :!label _label)))
          (else
            (goto _label)))))))

(fn GMAreAllZombiesDead
  ;[1 1 1] Currently existing zombies
  (if (Utilities|Array|IsValidIndex (Variables|Default|GetRemainingZombieArray))
    (return false)
    (else
      ;[1 1 1] Queued zombies
      (for _array_element (Variables|/Game/HorrorHo/Blueprints/Utilities/BP_WaveManager.BP_WaveManager_C|GetMasterSpawnerArray (Variables|Default|GetWaveManager))
        (if (Utilities|Array|IsValidIndex (Variables|/Game/HorrorHo/Blueprints/Actors/Installation/BP_Spawner.BP_Spawner_C|GetSpawnQueue _array_element))
          (return false)))
      ;[1 1 1] If both are empty, return true
      (return true))))

(fn GMBeginCountRemainingZombies
  (bind _outactors (Actor|GetAllActorswithTag "Zombie"))
  (bind _output_get (Variables|Default|SetRemainingZombieArray _outactors))
  (bind _returnvalue (Utilities|Time|SetTimerbyEvent (EventDispatchers|CreateEvent :!event QueryRemainingZombies) 0.2 true))
  (Variables|Default|SetPostWaveTimerHandle _returnvalue)
  (return (Utilities|Array|IsValidIndex _output_get)))

(fn GMFadein
  (bind _endtime (Class|BPIWidget|BPIWidgetFadein(Message) (Variables|Default|GetFadeWidget)))
  (return _endtime))

(fn GMFadeOut
  (bind _endtime (Class|BPIWidget|BPIWidgetFadeOut(Message) (Variables|Default|GetFadeWidget)))
  (return _endtime))

(fn GMGetDebugParams
  (bind _wavemanager (Variables|Default|GetWaveManager))
  (bind _remainingzombiearray (Variables|Default|GetRemainingZombieArray))
  (bind _activezombiearray (Variables|Default|GetActiveZombieArray))
  (Utilities|FlowControl|Sequence
    (:then_0
      (if (Utilities|Array|IsValidIndex _activezombiearray)
        (LocalVariables|SetActiveCount (Utilities|Array|Length _activezombiearray))))
    (:then_1
      (if (Utilities|Array|IsValidIndex _remainingzombiearray)
        (LocalVariables|SetRemainingCount (Utilities|Array|Length _remainingzombiearray))))
    (:then_2
      (Utilities|IsValid _wavemanager
        (:Is%20Valid
          (return (Variables|/Game/HorrorHo/Blueprints/Utilities/BP_WaveManager.BP_WaveManager_C|GetWaveNum _wavemanager) (Variables|/Game/HorrorHo/Blueprints/Utilities/BP_WaveManager.BP_WaveManager_C|GetActiveZombieTypes _wavemanager) (Variables|/Game/HorrorHo/Blueprints/Utilities/BP_WaveManager.BP_WaveManager_C|GetWaveFinishTimer _wavemanager) (Variables|/Game/HorrorHo/Blueprints/Utilities/BP_WaveManager.BP_WaveManager_C|GetLevelFinishTimer _wavemanager) (LocalVariables|GetActiveCount) (LocalVariables|GetRemainingCount)))))))

(fn GMKillSwitch
  (for _array_element (Variables|Default|GetRemainingZombieArray)
    (Class|BPIZombieBase|ZCharKillSwitch(Message) _array_element))
  (return true))

(fn GMQueryAddRemainingZombie
  (params (NewZombie :type BP%20Zombie%20Base%20Object%20Reference))
  ;[1 1 1] The handle is only valid if the game mode is currently counting zombies
  (if (Utilities|Time|IsValidTimerHandle (Variables|Default|GetPostWaveTimerHandle))
    (Utilities|Array|Add (Variables|Default|GetRemainingZombieArray) NewZombie)
    (return true)
    (else
      (return false))))