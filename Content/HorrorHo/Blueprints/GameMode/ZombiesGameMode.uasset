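; ZombiesGameMode is the game mode for the zombie mode, spawning a BP_Zombie_Manager at BeginPlay and limiting how many zombies attack each entrance at once.
; The construction script gathers all BP_EnemyEnterPoint actors and creates an attack-target struct for each, capped at three attackers.
; AskPermissionAttackEntrance and ReleasePermissionAttackEntrance act as a per-entrance slot counter by index, so attackers do not interrupt each other.
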(event EventBeginPlay
  ;[1 1 1] The zombie manager inherits from actor so it needs a spawn location, I want to switch the class it inherits from but im not sure which one is best right now.
  (bind _returnvalue (Game|SpawnActorfromClass "/Game/HorrorHo/Blueprints/AI出現/AIZombie/BP_Zombie_Manager.BP_Zombie_Manager_C" (Math|Transform|MakeTransform "0, 0, 0") "Undefined" 0 0))
  (Variables|Default|SetZombieManager _returnvalue))

(event EventTick
  (params (DeltaSeconds :type Float%20%28single-precision%29)))

(fn ConstructionScript
  (|CallParentFunction)
  (bind _outactors (Actor|GetAllActorsOfClass "/Game/HorrorHo/Blueprints/AI出現/BP_EnemyEnterPoint.BP_EnemyEnterPoint_C"))
  (bind _output_get (Variables|Default|SetLevelEntryPoints _outactors))
  ;[1 1 1] The Attack target struct is used to track how many zombies are allowed to attack a barricade at once and prevent them from interrupting eachother.  We can use these structs for any object, not just doors and windows.
  (for _array_element _output_get
    (Utilities|Array|Add (Variables|Default|GetBarricadeAttackTargets) (Utilities|Struct|MakeStruct_AttackTarget 0 3))))

(fn AskPermissionAttackEntrance
  (params (EntranceID :type Integer))
  (bind _barricadeattacktargets (Variables|Default|GetBarricadeAttackTargets))
  (bind _output (Utilities|Array|Get(acopy) _barricadeattacktargets EntranceID))
  (bind (_currentattackers _attackerlimit) (Utilities|Struct|BreakStruct_AttackTarget _output))
  (if (< _currentattackers _attackerlimit)
    ;[1 1 1] Allow this zombie to attack
    (Math|Integer|IncrementInt _currentattackers
      (:%20%20
        (return true)))
    (else
      ;[1 1 1] There are already too many zombies attacking this target.
      (return false))))

(fn ReleasePermissionAttackEntrance
  (params (EntranceID :type Integer))
  (Math|Integer|DecrementInt (.CurrentAttackers (Utilities|Struct|BreakStruct_AttackTarget (Utilities|Array|Get(acopy) (Variables|Default|GetBarricadeAttackTargets) EntranceID)))
    (:%20%20
      (return))))