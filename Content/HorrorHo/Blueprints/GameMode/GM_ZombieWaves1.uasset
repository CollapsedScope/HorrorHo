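; GM_ZombieWaves1 is the game mode for zombie wave levels, handling wave startup and the final clear-out.
; It adds a BP_WaveManager component, optionally assigns a wave table, then starts it.
; For the final step, it snapshots "Zombie"-tagged actors and starts a looping timer, with a prune function that clears it once none remain valid.
; It also exposes an all-dead check, a kill switch and wave debug values.
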(event EventBeginPlay)

(event EventTick
  (params (DeltaSeconds :type Float%20%28single-precision%29)))

(event EventGMSetWaveManager
  (params (WaveData :type Data%20Table%20Object%20Reference))
  (bind _returnvalue (Game|AddComponentbyClass "/Game/HorrorHo/Blueprints/Utilities/BP_WaveManager.BP_WaveManager_C"))
  (bind _output_get (Variables|Default|SetWaveManager _returnvalue))
  (Utilities|IsValid WaveData
    (:Is%20Valid
      (Variables|/Game/HorrorHo/Blueprints/Utilities/BP_WaveManager.BP_WaveManager_C|SetWaveTable _output_get WaveData))
    (:Is%20Not%20Valid
      _))
  (Default|BeginWaveManager _output_get))

(fn ConstructionScript)

(fn QueryRemainingZombies
  (bind _finalstepzombies (Variables|Default|GetFinalStepZombies))
  (if (Utilities|Array|IsValidIndex (Variables|Default|GetFinalStepZombies))
    (for (_ _array_index) _finalstepzombies
      (Utilities|IsValid (Utilities|Array|Get(acopy) _finalstepzombies _array_index)
        (:Is%20Not%20Valid
          (Utilities|Array|RemoveIndex _finalstepzombies _array_index))))
    (if (not (Utilities|Array|IsValidIndex _finalstepzombies))
      (Utilities|Time|ClearandInvalidateTimerbyHandle (Variables|Default|GetTransitionTimerHandle)))))

(fn GMAreAllZombiesDead
  (return (not (Utilities|Array|IsValidIndex (Variables|Default|GetFinalStepZombies)))))

(fn GMBeginCountRemainingZombies
  (bind _outactors (Actor|GetAllActorswithTag "Zombie"))
  (bind _output_get (Variables|Default|SetFinalStepZombies _outactors))
  (if (Utilities|Array|IsValidIndex _output_get)
    _
    (else
      (Development|PrintString "Init Final Step was called, but no actors with tag \"Zombie\" were found in the stage.")))
  (bind _returnvalue (Utilities|Time|SetTimerbyEvent (EventDispatchers|CreateEvent :!event QueryRemainingZombies) 0.2 true))
  (Variables|Default|SetTransitionTimerHandle _returnvalue)
  (return (Utilities|Array|IsValidIndex _output_get)))

(fn GMGetDebugParams
  (bind _wavemanager (Variables|Default|GetWaveManager))
  (Utilities|IsValid _wavemanager
    (:Is%20Valid
      (return (Variables|/Game/HorrorHo/Blueprints/Utilities/BP_WaveManager.BP_WaveManager_C|GetWaveNum _wavemanager) (Variables|/Game/HorrorHo/Blueprints/Utilities/BP_WaveManager.BP_WaveManager_C|GetActiveZombieTypes _wavemanager) (Variables|/Game/HorrorHo/Blueprints/Utilities/BP_WaveManager.BP_WaveManager_C|GetWaveTimer _wavemanager) (Variables|/Game/HorrorHo/Blueprints/Utilities/BP_WaveManager.BP_WaveManager_C|GetFinalTimer _wavemanager) 0))
    (:Is%20Not%20Valid
      (return 0 0 0.0 0.0 0))))

(fn GMKillSwitch
  (for _array_element (Variables|Default|GetFinalStepZombies)
    (Class|BPIZombieBase|ZCharKillSwitch(Message) _array_element))
  (return true))