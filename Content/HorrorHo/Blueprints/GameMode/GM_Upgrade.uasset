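; GM_Upgrade is a game mode, apparently for an upgrade level, that manages a black screen fade and runs no zombie wave logic.
; BeginPlay creates a UI_BlackScreen widget and adds it to the viewport.
; The fade in and fade out functions forward to that widget through interface messages.
; The zombie count, kill switch, wave and debug functions are stubs returning false or zero.
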(event EventBeginPlay
  (bind _returnvalue (UserInterface|CreateWidget "/Game/HorrorHo/Blueprints/Widgets/UI_BlackScreen.UI_BlackScreen_C"))
  (bind _output_get (Variables|Default|SetFadeWidget _returnvalue))
  (UserInterface|Viewport|AddtoViewport _output_get 1))

(event EventTick
  (params (DeltaSeconds :type Float%20%28single-precision%29)))

(fn ConstructionScript)

(fn GMAreAllZombiesDead
  (return false))

(fn GMBeginCountRemainingZombies
  (return false))

(fn GMFadein
  (bind _endtime (Class|BPIWidget|BPIWidgetFadein(Message) (Variables|Default|GetFadeWidget)))
  (return _endtime))

(fn GMFadeOut
  (bind _endtime (Class|BPIWidget|BPIWidgetFadeOut(Message) (Variables|Default|GetFadeWidget)))
  (return _endtime))

(fn GMGetDebugParams
  (return 0 0 0.0 0.0 0 0))

(fn GMGetWaveZombieCount
  (return 0 0))

(fn GMKillSwitch
  (return false))

(fn GMQueryAddRemainingZombie
  (params (NewZombie :type Actor%20Object%20Reference))
  (return false))