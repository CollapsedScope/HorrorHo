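; Behavior tree task meant to make a zombie attack the player within range, though its Execute event is unwired, so none of this logic runs.
; The disconnected logic gets the controlled zombie through an interface message and succeeds if it is already attacking.
; Otherwise it compares horizontal player distance to AttackRange, failing when out of range.
; In range, it snaps to face the player, sets attack flags, stops movement and succeeds.
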(event EventReceiveExecute
  (params (OwnerActor :type Actor%20Object%20Reference)))