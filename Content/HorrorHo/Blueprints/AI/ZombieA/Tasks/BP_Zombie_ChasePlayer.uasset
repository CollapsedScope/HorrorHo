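; Behavior tree task that makes a zombie chase the player.
; Each execution asks the game mode's ZombieManager for attack permission, storing it on the pawn and writing the returned target distance to the blackboard.
; If the zombie is not already moving, AIMoveTo targets the player pawn with that distance as acceptance radius.
; The task finishes successfully as the move starts, and the IsMoving flags on pawn and blackboard clear when it ends.
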(event EventReceiveExecute
  (params (OwnerActor :type Actor%20Object%20Reference))
  (bind _zombie (Class|BPZombieControllerInterface|GetControlledZombie(Message) OwnerActor))
  (Variables|Default|SetControlledPawn _zombie)
  (CallFunction|UpdateAttackPermission (Variables|Default|GetControlledPawn))
  (if (not (Variables|/Game/HorrorHo/Blueprints/Characters/BP_ZombieCharacter.BP_ZombieCharacter_C|GetIsMoving (Variables|Default|GetControlledPawn)))
    (AI|AIMoveTo (Variables|Default|GetControlledPawn) "0, 0, 0" (Game|Player|GetPlayerPawn 0) (Class|BTFunctionLibrary|GetBlackboardValueasFloat (Variables|Default|GetPermissionTargetDistance)) false
      (:then
        (Variables|/Game/HorrorHo/Blueprints/Characters/BP_ZombieCharacter.BP_ZombieCharacter_C|SetIsMoving (Variables|Default|GetControlledPawn) true)
        (Class|BTFunctionLibrary|SetBlackboardValueasBool (Variables|Default|GetIsMoving) true)
        (AI|BehaviorTree|FinishExecute true))
      (:OnSuccess
        (Variables|/Game/HorrorHo/Blueprints/Characters/BP_ZombieCharacter.BP_ZombieCharacter_C|SetIsMoving (Variables|Default|GetControlledPawn) false :!label _label)
        (Class|BTFunctionLibrary|SetBlackboardValueasBool (Variables|Default|GetIsMoving) false)
        (AI|BehaviorTree|FinishExecute false))
      (:OnFail
        (goto _label)))))

(fn UpdateAttackPermission
  (params (ControlledPawn :type Pawn%20Object%20Reference))
  (bind _zombiesmode (Class|ZombiesGameModeInterface|GetZombiesMode(Message) (Game|GetGameMode)))
  (bind (_permission _targetdistance) (Default|QueryAttackPermission (Variables|/Game/HorrorHo/Blueprints/GameMode/ZombiesGameMode.ZombiesGameMode_C|GetZombieManager _zombiesmode) (Variables|Default|GetControlledPawn)))
  (Variables|/Game/HorrorHo/Blueprints/Characters/BP_ZombieCharacter.BP_ZombieCharacter_C|SetPlayerAttackPermission (Variables|Default|GetControlledPawn) _permission)
  (Class|BTFunctionLibrary|SetBlackboardValueasFloat (Variables|Default|GetPermissionTargetDistance) _targetdistance)
  (return _permission))