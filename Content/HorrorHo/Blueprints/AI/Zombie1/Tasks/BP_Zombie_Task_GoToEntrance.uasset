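; Behavior Tree task that sends the controlled zombie to the entrance location stored in the Blackboard.
; On execute, it gets the zombie through a controller message interface and runs AIMoveTo if it is not already moving, toggling IsMoving around the move.
; The result is inverted: arrival finishes as failure, while a failed move finishes as success after a short delay.
; An invalid or already moving zombie never finishes the task.
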(event EventReceiveExecute
  (params (OwnerActor :type Actor%20Object%20Reference))
  (bind _zombiecontroller (Class|BPZombieControllerInterface|GetZombieController(Message) OwnerActor))
  (bind _zombie (Default|GetControlledZombie _zombiecontroller))
  (Utilities|IsValid _zombie
    (:Is%20Valid
      (if (not (Variables|/Game/HorrorHo/Blueprints/Characters/BP_ZombieCharacter.BP_ZombieCharacter_C|GetIsMoving _zombie))
        (AI|AIMoveTo _zombie (Class|BTFunctionLibrary|GetBlackboardValueasVector (Variables|Default|GetEntranceLocation)) 0 1.5e+02 true
          (:then
            (Variables|/Game/HorrorHo/Blueprints/Characters/BP_ZombieCharacter.BP_ZombieCharacter_C|SetIsMoving _zombie true))
          (:OnSuccess
            (Variables|/Game/HorrorHo/Blueprints/Characters/BP_ZombieCharacter.BP_ZombieCharacter_C|SetIsMoving _zombie false)
            (AI|BehaviorTree|FinishExecute false))
          (:OnFail
            (Variables|/Game/HorrorHo/Blueprints/Characters/BP_ZombieCharacter.BP_ZombieCharacter_C|SetIsMoving _zombie false)
            (Utilities|FlowControl|Delay 0.5)
            (AI|BehaviorTree|FinishExecute true)))))))