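; Behavior tree task that makes a controlled zombie attempt an attack on the player.
; It succeeds immediately if the zombie is already attacking, and fails if the player's horizontal distance is not within AttackRange.
; In range, it snaps the zombie to face the player on the horizontal plane, sets its attack flags, stops its movement and finishes successfully without waiting for the attack to end.
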(event EventReceiveExecute
  (params (OwnerActor :type Actor%20Object%20Reference))
  (bind _zombie (Class|BPZombieControllerInterface|GetControlledZombie(Message) OwnerActor))
  (bind _output_get (Variables|Default|SetControlledPawn _zombie))
  (if (Variables|/Game/HorrorHo/Blueprints/Characters/BP_ZombieCharacter.BP_ZombieCharacter_C|GetIsAttacking _output_get)
    (AI|BehaviorTree|FinishExecute true)
    (elif (< (Math|Vector|VectorLength (Math|Vector|MakeVector (.x (- (Transformation|GetActorLocation (Game|Player|GetPlayerPawn 0)) (Transformation|GetActorLocation _output_get))) (.y (- (Transformation|GetActorLocation (Game|Player|GetPlayerPawn 0)) (Transformation|GetActorLocation _output_get))) 0.0)) (Variables|Default|GetAttackRange))
      (Transformation|SetActorRotation (Variables|Default|GetControlledPawn) (Math|Conversions|RotationFromXVector (Math|Vector|Normalize (Math|Vector|MakeVector (.x (- (Transformation|GetActorLocation (Game|Player|GetPlayerPawn 0)) (Transformation|GetActorLocation _output_get))) (.y (- (Transformation|GetActorLocation (Game|Player|GetPlayerPawn 0)) (Transformation|GetActorLocation _output_get))) 0.0))))
      (Variables|/Game/HorrorHo/Blueprints/Characters/BP_ZombieCharacter.BP_ZombieCharacter_C|SetStartAttack (Variables|Default|GetControlledPawn) true)
      (Variables|/Game/HorrorHo/Blueprints/Characters/BP_ZombieCharacter.BP_ZombieCharacter_C|SetIsAttacking (Variables|Default|GetControlledPawn) true)
      ;[1 1 1] Make sure the zombie stops moving when it attacks
      (Variables|/Game/HorrorHo/Blueprints/Characters/BP_ZombieCharacter.BP_ZombieCharacter_C|SetIsMoving (Variables|Default|GetControlledPawn) false)
      (Class|NavMovementComponent|StopActiveMovement (Variables|/Script/Engine.Character|GetCharacterMovement (Variables|Default|GetControlledPawn)))
      (AI|BehaviorTree|FinishExecute true)
      (else
        (AI|BehaviorTree|FinishExecute false)))))