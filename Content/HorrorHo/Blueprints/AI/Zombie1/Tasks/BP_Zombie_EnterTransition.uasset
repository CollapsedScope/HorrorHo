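; Behavior tree task that moves a zombie through an enemy enter point into the player area, currently as a temporary teleport.
; It frees the blackboard's enter point and teleports the pawn horizontally to its exit volume, keeping the current height.
; It then flags the zombie as inside, clears its entrance attack permission and releases that entrance in ZombiesGameMode so another zombie can begin entering.
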(event EventReceiveExecute
  (params (OwnerActor :type Actor%20Object%20Reference))
  ;[1 1 1] Temporary: teleport pawn to exit location
  (bind _asbp_enemy_enter_point (Utilities|Casting|CastToBP_EnemyEnterPoint (Class|BTFunctionLibrary|GetBlackboardValueasObject (Variables|Default|GetEnterPoint))))
  (Variables|/Game/HorrorHo/Blueprints/Actors/Installation/BP_EnemyEnterPoint.BP_EnemyEnterPoint_C|SetIsBeingUsed _asbp_enemy_enter_point false)
  (bind _zombie (Class|BPZombieControllerInterface|GetControlledZombie(Message) OwnerActor))
  (Transformation|SetActorLocation _zombie (Math|Vector|MakeVector (.x (Transformation|GetWorldLocation (Variables|/Game/HorrorHo/Blueprints/Actors/Installation/BP_EnemyEnterPoint.BP_EnemyEnterPoint_C|GetExitVolume _asbp_enemy_enter_point))) (.y (Transformation|GetWorldLocation (Variables|/Game/HorrorHo/Blueprints/Actors/Installation/BP_EnemyEnterPoint.BP_EnemyEnterPoint_C|GetExitVolume _asbp_enemy_enter_point))) (.z (Transformation|GetActorLocation _zombie))) false true)
  (Class|BTFunctionLibrary|SetBlackboardValueasBool (Variables|Default|GetIsInsidePlayerArea) true)
  ;[1 1 1] Tell the game mode that this zombie is done with the entrance and to allow another zombie to begin entering
  (Class|BTFunctionLibrary|SetBlackboardValueasBool (Variables|Default|GetEntranceAttackPermission) false)
  (bind _aszombies_game_mode (Utilities|Casting|CastToZombiesGameMode (Game|GetGameMode)))
  (Default|ReleasePermissionAttackEntrance _aszombies_game_mode (Class|BTFunctionLibrary|GetBlackboardValueasInt (Variables|Default|GetEntranceID)))
  (AI|BehaviorTree|FinishExecute true))