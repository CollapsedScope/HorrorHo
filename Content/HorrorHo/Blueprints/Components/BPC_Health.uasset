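; Actor component that tracks health for its owner, starting at the maximum on BeginPlay.
; CalculateHealth subtracts damage with clamping, sends the new health ratio to a health bar widget through an interface message, and returns whether health reached zero.
; Recover adds an amount to health without clamping to the maximum.
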(event EventBeginPlay
  (Variables|Default|SetHealth (Variables|Default|GetHealthMax)))

(event EventTick
  (params (DeltaSeconds :type Float%20%28single-precision%29)))

(fn CalculateHealth
  (params (Damage :type Float%20%28single-precision%29) (HealthBarWidget :type User%20Widget%20Object%20Reference))
  (bind _output_get (Variables|Default|SetHealth (Math|Float|Clamp(Float) (- (Variables|Default|GetHealth) Damage) 0.0 (Variables|Default|GetHealthMax))))
  (if (<= _output_get 0.0)
    (Class|BPIWidget|BPIWidgetRespondtoDamage(Message) HealthBarWidget (/ (Variables|Default|GetHealth) (Variables|Default|GetHealthMax)))
    (return true)
    (else
      (Utilities|FlowControl|Sequence
        (:then_0
          (Class|BPIWidget|BPIWidgetRespondtoDamage(Message) HealthBarWidget (/ (Variables|Default|GetHealth) (Variables|Default|GetHealthMax)))
          (return false))))))

(fn Recover
  (params (Amount :type Float%20%28single-precision%29))
  (Variables|Default|SetHealth (+ Amount (Variables|Default|GetHealth))))