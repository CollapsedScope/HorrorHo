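; Blueprint interface for zombie characters in the HorrorHo game, declaring accessors for shared zombie state without implementation.
; Setters and getters cover the dead, moving, transitioning and can-enter-player-area flags.
; Two further getters return the zombie character and its spawner, so callers can reach both through the interface.
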(fn ZCharSetIsDead
  (params (IsDead :type Boolean)))

(fn ZCharSetCanEnterPlayerArea
  (params (CanEnter :type Boolean)))

(fn ZCharSetIsMoving
  (params (IsMoving :type Boolean)))

(fn ZCharSetIsTransitioning
  (params (Is%20Transitioning :type Boolean)))

(fn ZCharGetZombieCharacter
  (return 0))

(fn ZCharGetSpawner
  (return 0))

(fn ZCharGetCanEnterPlayerArea
  (return false))

(fn ZCharGetIsTransitioning
  (return false))

(fn ZCharGetIsDead
  (return false))

(fn ZCharGetIsMoving
  (return false))