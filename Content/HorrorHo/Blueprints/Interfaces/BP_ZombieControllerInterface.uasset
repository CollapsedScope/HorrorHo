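; Blueprint Interface for zombie controllers in HorrorHo, exposing read-style queries about a controller and the zombie it controls.
; Getters cover the controller itself, its controlled zombie and its spawner, plus boolean state for entering the player area, transitioning and being dead.
; It holds only empty function signatures, leaving the logic to implementing classes.
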(fn ZConGetZombieController
  (return 0))

(fn ZConGetControlledZombie
  (return 0))

(fn ZConGetCanEnterPlayerArea
  (return false))

(fn ZConGetIsTransitioning
  (return false))

(fn ZConGetIsDead
  (return false))

(fn ZConGetSpawner
  (return 0))