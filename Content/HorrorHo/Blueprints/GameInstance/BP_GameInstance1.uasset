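; Game instance that holds player settings, difficulty, score stats and level progression across levels in a zombie shooter.
; Init loads default shooter and health settings from DataTables; difficulty selects the bandage size.
; Interface calls read and update this state, with a looping timer resetting the consecutive-kill counter after a short window.
; Level changes wait on a GameMode fade, save player settings and route through a customize level before the next stage, except Clear.
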(event EventBPIGISetPlayerSettings
  (params (ShooterSettings :type Struct%20Player%20Attack%20Settings%20Structure) (HealthSettings :type Struct%20Player%20Health%20Settings%20Structure))
  (Utilities|Struct|SetmembersinStruct_GeneralPlayerSettings (Variables|Default|GetPlayerSettings) ShooterSettings HealthSettings))

(event EventInit
  (bind _playersettings (Variables|Default|GetPlayerSettings))
  (bind (_shootersettings _healthsettings) (Utilities|Struct|BreakStruct_GeneralPlayerSettings _playersettings))
  (Utilities|FlowControl|Sequence
    (:then_0
      ;[1 1 1] プレイヤーの攻撃パラメータの初期設定
      (bind _returnvalue (Utilities|GetDataTableRow "/Game/HorrorHo/Data/DataTable/Player/DT_ShooterSettings1.DT_ShooterSettings1" "Default")
        (:then
          (Utilities|Struct|SetmembersinStruct_GeneralPlayerSettings (Variables|Default|GetPlayerSettings) _returnvalue)
          ;[1 1 1] プレイヤーの体力パラメータの初期設定
          (bind _returnvalue_2 (Utilities|GetDataTableRow "/Game/HorrorHo/Data/DataTable/Player/DT_HealthSettings.DT_HealthSettings" "Default")
            (:then
              (Utilities|Struct|SetmembersinStruct_GeneralPlayerSettings (Variables|Default|GetPlayerSettings) _returnvalue_2)
              (Variables|Default|SetDefaultPlayerSettings (Variables|Default|GetPlayerSettings)))))))
    (:then_1
      (Utilities|Struct|SetmembersinStruct_PlayerAttackSettings _shootersettings (.MagazineMaxSize (Utilities|Struct|BreakStruct_PlayerAttackSettings _shootersettings)))
      (Utilities|Struct|SetmembersinStruct_PlayerHealthSettings _healthsettings (Utilities|Struct|BreakStruct_PlayerHealthSettings _healthsettings)))))

(event EventBPIGIBeginGame
  ;[1 1 1] Launch the game from the main menu
  ;;[1 1 1] In place of a loading screen for now
  (Utilities|FlowControl|Delay 0.5)
  (Game|OpenLevel(byName) (Utilities|Array|Get(acopy) (Variables|Default|GetLevelNames))))

(event EventBPIGIResetScoreStats
  (params (KeepDefeatCounter :type Boolean))
  ;[1 1 1] スコア記録
  ;;[1 1 1] ローカル変数を使うために関数化
  (CallFunction|ClearScoreStats KeepDefeatCounter))

(event EventBPIGIUpdateAccuracyStats
  (params (GeneralAccuracy :type Float%20%28single-precision%29) (HeadshotAccuracy :type Float%20%28single-precision%29))
  ;[1 1 1] スコア記録
  (Utilities|Struct|SetmembersinStruct_ScoreStats (Variables|Default|GetScore%20Stats) GeneralAccuracy HeadshotAccuracy))

(event EventBPIGITryUpdateConsecutiveKills
  (params (Killstreak :type Integer))
  (bind _score_stats (Variables|Default|GetScore%20Stats))
  ;[1 1 1] スコア記録
  (if (> Killstreak (Utilities|Struct|BreakStruct_ScoreStats _score_stats))
    (Utilities|Struct|SetmembersinStruct_ScoreStats _score_stats Killstreak)))

(event EventBPIGIIncrementStats
  (params (ZombiesKilled :type Boolean) (ZombieType :type EZombieType%20Enum :default "NewEnumerator0") (CloseRangeKills :type Boolean) (BarricadeRepairs :type Boolean) (ItemPickups :type Boolean) (TimesDamaged :type Boolean) (TimesHealed :type Boolean) (TimesDefeated :type Boolean))
  ;[1 1 1] スコア記録
  (CallFunction|IncrementAppropriateStats ZombiesKilled ZombieType CloseRangeKills BarricadeRepairs ItemPickups TimesDamaged TimesHealed TimesDefeated))

(fn IncrementZombieKill
  (params (Selection :type EZombieType%20Enum :default "NewEnumerator0"))
  (bind _score_stats (Variables|Default|GetScore%20Stats))
  (bind _score_stats_2 (Variables|Default|GetScore%20Stats))
  (bind _bestconsecutivekills (Utilities|Struct|BreakStruct_ScoreStats _score_stats_2))
  (bind (_killedwalkers _killedrunners _killedcrawlers _killedscreamers _killedbombers) (Utilities|Struct|BreakStruct_ScoreStats _score_stats))
  (Utilities|FlowControl|Sequence
    (:then_0
      (Variables|Default|SetConsecutiveTimer 2.0)
      (bind _result (Math|Integer|IncrementInt (Variables|Default|GetTempConsecutiveCounter))
        (:%20%20
          (Utilities|Struct|SetmembersinStruct_ScoreStats _score_stats_2 (Math|Integer|SelectInt _result _bestconsecutivekills (> _result _bestconsecutivekills)))
          (if (not (Utilities|Time|IsValidTimerHandle (Variables|Default|GetHandle)))
            (bind _returnvalue (Utilities|Time|SetTimerbyEvent (EventDispatchers|CreateEvent :!event DecreaseConsecutiveTimer) 0.016667 true))
            (Variables|Default|SetHandle _returnvalue)))))
    (:then_1
      (switch Utilities|FlowControl|Switch|SwitchonEZombieType Selection
        (:NewEnumerator0
          (Utilities|Struct|SetmembersinStruct_ScoreStats _score_stats (+ _killedwalkers 1)))
        (:NewEnumerator1
          (Utilities|Struct|SetmembersinStruct_ScoreStats _score_stats (+ _killedrunners 1)))
        (:NewEnumerator2
          (Utilities|Struct|SetmembersinStruct_ScoreStats _score_stats (+ _killedcrawlers 1)))
        (:NewEnumerator3
          (Utilities|Struct|SetmembersinStruct_ScoreStats _score_stats (+ _killedbombers 1)))
        (:NewEnumerator4
          (Utilities|Struct|SetmembersinStruct_ScoreStats _score_stats (+ _killedscreamers 1)))))))

(fn IncrementAppropriateStats
  (params (ZombiesKilled :type Boolean) (ZombieType :type EZombieType%20Enum :default "NewEnumerator0") (CloseRangeKills :type Boolean) (BarricadesRepaired :type Boolean) (ItemPickups :type Boolean) (TimesDamaged :type Boolean) (TimesHealed :type Boolean) (TimesDefeated :type Boolean))
  (bind _score_stats (Variables|Default|GetScore%20Stats))
  (bind _score_stats_2 (Variables|Default|GetScore%20Stats))
  (bind _score_stats_3 (Variables|Default|GetScore%20Stats))
  (bind _score_stats_4 (Variables|Default|GetScore%20Stats))
  (bind _score_stats_5 (Variables|Default|GetScore%20Stats))
  (bind _score_stats_6 (Variables|Default|GetScore%20Stats))
  (Utilities|FlowControl|Sequence
    (:then_0
      (if ZombiesKilled
        (CallFunction|IncrementZombieKill ZombieType)))
    (:then_1
      (if CloseRangeKills
        (Utilities|Struct|SetmembersinStruct_ScoreStats _score_stats (+ (Utilities|Struct|BreakStruct_ScoreStats _score_stats) 1))))
    (:then_2
      (if BarricadesRepaired
        (Utilities|Struct|SetmembersinStruct_ScoreStats _score_stats_2 (+ (Utilities|Struct|BreakStruct_ScoreStats _score_stats_2) 1))))
    (:then_3
      (if ItemPickups
        (Utilities|Struct|SetmembersinStruct_ScoreStats _score_stats_3 (+ (Utilities|Struct|BreakStruct_ScoreStats _score_stats_3) 1))))
    (:then_4
      (if TimesDamaged
        (Utilities|Struct|SetmembersinStruct_ScoreStats _score_stats_4 (+ (Utilities|Struct|BreakStruct_ScoreStats _score_stats_4) 1))))
    (:then_5
      (if TimesHealed
        (Utilities|Struct|SetmembersinStruct_ScoreStats _score_stats_5 (+ (Utilities|Struct|BreakStruct_ScoreStats _score_stats_5) 1))))
    (:then_6
      (if TimesDefeated
        (Utilities|Struct|SetmembersinStruct_ScoreStats _score_stats_6 (+ (Utilities|Struct|BreakStruct_ScoreStats _score_stats_6) 1))))))

(fn ClearScoreStats
  (params (Keep%20Defeat%20Counter :type Boolean))
  (if Keep%20Defeat%20Counter
    (bind _output_get (LocalVariables|SetTemp (Utilities|Struct|BreakStruct_ScoreStats (Variables|Default|GetScore%20Stats))))
    (bind _output_get_2 (Variables|Default|SetScore%20Stats ""))
    (Utilities|Struct|SetmembersinStruct_ScoreStats _output_get_2 _output_get)
    (else
      (Variables|Default|SetScore%20Stats ""))))

(fn DecreaseConsecutiveTimer
  (bind _output_get (Variables|Default|SetConsecutiveTimer (Math|Float|Max(Float) (- (Variables|Default|GetConsecutiveTimer) 0.016667) 0.0)))
  (if (== _output_get 0.0)
    (Utilities|Time|ClearandInvalidateTimerbyHandle (Variables|Default|GetHandle))
    (Variables|Default|SetTempConsecutiveCounter 0)))

(fn DetermineBandageSize
  (bind _returnvalue (Utilities|GetDataTableRow "/Game/HorrorHo/Data/DataTable/Player/DT_BandageSizeOnDifficulty.DT_BandageSizeOnDifficulty" "Default")
    (:then
      (Utilities|Struct|SetmembersinStruct_PlayerHealthSettings (Utilities|Struct|BreakStruct_GeneralPlayerSettings (Variables|Default|GetPlayerSettings)) (Utilities|Select :Index (Variables|Default|GetDifficulty) :Option%200 (.bandagesizeoneasy _returnvalue) :Option%201 (.bandagesizeonnormal _returnvalue) :Option%202 (.bandagesizeonhard _returnvalue))))))

(fn OpenNextLevel
  (bind _levelnames (Variables|Default|GetLevelNames))
  (bind _returnvalue (Game|GetCurrentLevelName true))
  (if (and (Utilities|Enum|NotEqual(Enum) _returnvalue (Utilities|String|ToString(Name) (Variables|Default|GetCustomizeLevelName%28const%29))) (Utilities|Enum|NotEqual(Enum) _returnvalue (Utilities|String|ToString(Name) (Variables|Default|GetTutorialLevelName%28const%29))))
    (for (_array_element _array_index) (Variables|Default|GetLevelNames)
      (if (Utilities|Name|Equal(Name) _array_element (Utilities|String|StringToName _returnvalue))
        (if (Utilities|Array|IsValidIndex _levelnames (+ _array_index 1))
          (Class|BPIPlayer|BPIPlayerSavePlayerSettings(Message) (Game|GetPlayerCharacter 0))
          (CallFunction|DetermineBandageSize)
          (bind _output_get (Variables|Default|SetNextLevelName (Utilities|Array|Get(acopy) _levelnames (+ _array_index 1))))
          (if (Utilities|Name|Equal(Name) _output_get "Clear")
            (Game|OpenLevel(byName) _output_get)
            (else
              (Game|OpenLevel(byName) (Variables|Default|GetCustomizeLevelName%28const%29)))))))
    (Development|PrintString "Unable to find next level in the game instance")
    (else
      (Game|OpenLevel(byName) (Variables|Default|GetNextLevelName)))))

(fn BPIGIGetDefaultPlayerSettings
  (return (Variables|Default|GetDefaultPlayerSettings)))

(fn BPIGIGetDifficulty
  (return (Variables|Default|GetDifficulty)))

(fn BPIGIGetNextLevelName
  (return (Variables|Default|GetNextLevelName)))

(fn BPIGIGetPlayerSettings
  (bind _playersettings (Variables|Default|GetPlayerSettings))
  (return (.shootersettings _playersettings) (.healthsettings _playersettings)))

(fn BPIGIGetScoreStats
  (return (Variables|Default|GetScore%20Stats)))

(fn BPIGIOpenNextLevel
  (bind _endtime (Class|BPIWavesMode|GMFadeOut(Message) (Game|GetGameMode)))
  (Utilities|Time|SetTimerbyEvent (EventDispatchers|CreateEvent :!event OpenNextLevel) _endtime)
  (return true))

(fn BPIGISetDifficulty
  (params (Difficulty :type Integer))
  (Variables|Default|SetDifficulty Difficulty)
  (CallFunction|DetermineBandageSize)
  (return))