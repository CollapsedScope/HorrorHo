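; Player controller that plays per-stage music and serves as the interface hub for tutorial, result screens, movie player and input mode.
; Interface calls add the tutorial manager and tooltip widgets, show result widgets, and pause or resume the movie.
; Holding MovieSkip runs a looping timer that feeds a radial widget, then skips the tutorial phase's movie or stops the player to black.
; Any key is forwarded to the movie player and visible result widget.
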(event EventBeginPlay
  (Variables|Default|SetCharacterRef (Game|GetPlayerCharacter 0))
  (Audio|Components|Audio|SetVolumeMultiplier (Variables|Default|GetMediaSound) 3.0 :!class /Script/AudioMixer.SynthComponent)
  (bind _returnvalue (Game|GetCurrentLevelName true))
  (switch name (Utilities|String|StringToName _returnvalue)
    (:Stage_Main
      (Audio|PlaySound2D "/Game/HorrorHo/Audio/BGM/Stage1.Stage1" 1.0 1.0 0.0 0 0))
    (:Stage2_Main
      (Audio|PlaySound2D "/Game/HorrorHo/Audio/BGM/Stage2.Stage2" 1.0 1.0 0.0 0 0))
    (:Stage3_Main
      (Audio|PlaySound2D "/Game/HorrorHo/Audio/BGM/Stage3.Stage3" 1.0 1.0 0.0 0 0))))

(event EventBPIPlayerControllerAddTutorialManager
  (params (DataAsset :type Tutorial%20Set%20Data%20BPP%20Object%20Reference))
  (bind _returnvalue (AddComponent|AddTutorialManager DataAsset self))
  (Variables|Default|SetTutorialManagerComponent _returnvalue)
  (bind _returnvalue_2 (UserInterface|CreateWidget "/Game/HorrorHo/Blueprints/Widgets/UI_Tooltips.UI_Tooltips_C"))
  (bind _output_get (Variables|Default|SetTutorialWidget _returnvalue_2))
  (UserInterface|Viewport|AddtoViewport _output_get 0))

(event EventBPIPlayerControllerShowTotalResultWidget
  (bind _returnvalue (UserInterface|CreateWidget "/Game/HorrorHo/Blueprints/Widgets/UI_FinalResult.UI_FinalResult_C"))
  (bind _output_get (Variables|Default|SetResultWidget _returnvalue))
  (UserInterface|Viewport|AddtoViewport _output_get 9999))

(event EventBPIPlayerControlleronPause
  ;[1 1 1] ポーズメニューを開いたら/閉じたら
  (Default|PauseMovie (Variables|Default|GetBP_MoviePlayer)))

(event EventBPIPlayerControlleronResume
  ;[1 1 1] ポーズメニューを開いたら/閉じたら
  (Default|ResumeMovie (Variables|Default|GetBP_MoviePlayer)))

(event EventBPIPlayerControllerClearTooltipCascade
  (bind _tooltipcascades (Variables|Default|GetTooltipCascades))
  (for _array_element _tooltipcascades
    (if (UserInterface|Viewport|IsinViewport _array_element)
      (Widget|RemovefromParent _array_element)))
  (Utilities|Array|Clear _tooltipcascades)
  (Default|ClearNode (Variables|Default|GetTutorialWidget)))

(event EventBPIPlayerControllerShowResultWidget
  (bind _returnvalue (UserInterface|CreateWidget "/Game/HorrorHo/Blueprints/Widgets/UI_Result.UI_Result_C"))
  (bind _output_get (Variables|Default|SetResultWidget _returnvalue))
  (UserInterface|Viewport|AddtoViewport _output_get 9999))

(event EventBPIPlayerControllerSetInputMode
  (params (UI?%20%28%20not%20game?%20%29 :type Boolean))
  (bind _self self)
  (if UI?%20%28%20not%20game?%20%29
    (Input|SetInputModeGameandUI _self 0 "DoNotLock" true)
    (Variables|/Script/Engine.PlayerController|SetbShowMouseCursor _self true)
    (else
      (Input|SetInputModeGameOnly _self)
      (Variables|/Script/Engine.PlayerController|SetbShowMouseCursor _self false))))

(event Input|ActionEvents|InputActionMovieSkip
  (params (Key :type Key%20Structure))
  (:Pressed
    (EventDispatchers|BindEventtoLongPressEventDispatcher (EventDispatchers|CreateEvent :!event OnLongPressedSelectButton))
    (Utilities|LongPress 1.0 :!label _label))
  (:Released
    (goto _label Released)))

(event Input|KeyboardEvents|AnyKey
  (params (Key :type Key%20Structure))
  (:Pressed
    (Default|OnAnyKey (Variables|Default|GetBP_MoviePlayer))
    (bind _resultwidget (Variables|Default|GetResultWidget)
      (:then
        (if (UserInterface|Viewport|IsinViewport _resultwidget)
          (Class|BPIKeyNotify|BPIPressA(Message) _resultwidget)))
      (:else))))

(fn ConstructionScript)

(fn TickforLongPress
  (bind _output_get (Variables|Default|SetLongPressTimer (+ (Variables|Default|GetLongPressTimer) 0.016666)))
  (Class|BPIRadialTimer|BPIRadialTimerSetCurrentTime(Message) (Variables|Default|GetLongPressWidget) (Variables|Default|GetLongPressTimer))
  (if (>= _output_get (Variables|Default|GetLongPressTimerMax))
    (Default|CallLongPressEventDispatcher)))

(fn OnLongPressedSelectButton
  (Variables|Default|SetLongPressTimer 0.0)
  (Utilities|Time|ClearandInvalidateTimerbyHandle (Variables|Default|GetLongPresssTimerHandle))
  (bind _tutorialmanagercomponent (Variables|Default|GetTutorialManagerComponent)
    (:then
      (bind _tutorialphaseactor (Class|BPITutorialManager|BPITutorialGetCurrentTutorialPhase(Message) _tutorialmanagercomponent))
      (Class|BPITutorialPhase|BPITutorialPhaseSkipMovie(Message) _tutorialphaseactor)
      (bind _longpresswidget (Variables|Default|GetLongPressWidget)
        (:then
          (Widget|RemovefromParent _longpresswidget))
        (:else)))
    (:else
      (Class|BPIMoviePlayer|BPIMoviePlayerStopImmediately(Message) (Variables|Default|GetBP_MoviePlayer))
      (Class|BPIMoviePlayer|BPIMoviePlayerBlackScreen(Message) (Variables|Default|GetBP_MoviePlayer)))))

(fn BPIPlayerControllerAddTooltipNode
  (params (Text :type Text) (TextColor :type Linear%20Color%20Structure) (TextHighlightedColor :type Linear%20Color%20Structure) (ImageBrush :type Slate%20Brush%20Structure) (FontSize :type Integer))
  (bind _tutorialwidget (Variables|Default|GetTutorialWidget))
  (bind _returnvalue (UserInterface|CreateWidget "/Game/HorrorHo/Blueprints/Widgets/Cascades/UI_TooltipCascade.UI_TooltipCascade_C" 0 Text FontSize TextColor TextHighlightedColor 1.0 _tutorialwidget "/Game/Art/Eda/Font/Koruri-Bold_Font.Koruri-Bold_Font" ImageBrush))
  (Utilities|Array|Add (Variables|Default|GetTooltipCascades) _returnvalue)
  (Default|AddNode _tutorialwidget _returnvalue)
  (return _returnvalue))

(fn BPIPlayerControllerGetMoviePlayerRef
  (return (Variables|Default|GetBP_MoviePlayer)))

(fn BPIPlayerControllerGetTutorialManagerComponent
  (bind _tutorialmanagercomponent (Variables|Default|GetTutorialManagerComponent)
    (:then
      (return _tutorialmanagercomponent true))
    (:else
      (return 0 false))))