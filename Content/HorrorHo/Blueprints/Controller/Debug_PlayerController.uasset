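; Debug player controller that adds a debug HUD and developer hotkeys for the player character.
; On BeginPlay it caches the player character and creates the UI_DebugHUD widget.
; Q toggles the character info display and K toggles invincibility through CanBeDamaged, with both notifying the HUD through interface calls.
; It also implements BPI_GetDebugInfo to report the focused character and debug display flags.
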(event EventBeginPlay
  (|CallParentFunction)
  (Variables|Debug|SetCharacterRef (Game|GetPlayerCharacter 0))
  ;[0.6282 1 0.9299] デバッグ用ウィジェットを作成し、アタッチする
  (bind _returnvalue (UserInterface|CreateWidget "/Game/HorrorHo/Blueprints/Widgets/DEBUG/UI_DebugHUD.UI_DebugHUD_C"))
  (bind _output_get (Variables|Default|SetDebuggingWidget _returnvalue))
  (UserInterface|Viewport|AddtoViewport _output_get 0))

(event EventTick
  (params (DeltaSeconds :type Float%20%28single-precision%29))
  (|CallParentFunction DeltaSeconds) ; This node is disabled and will not be called.\nDrag off pins to build functionality.
)

(event Input|KeyboardEvents|Q
  (params (Key :type Key%20Structure :default "None"))
  ;[1 0.6235 0.6706] Debug
  (:Pressed
    (bind _output_get (Variables|Debug|SetShowCharacterInfo (not (Variables|Debug|GetShowCharacterInfo))))
    (Class|BPIPlayer|BPIDebugon(Message) (Game|GetPlayerCharacter 0) _output_get)
    (Class|BPIWidget|BPIToggleDebugState(Message) (Variables|Default|GetDebuggingWidget))))

(event Input|KeyboardEvents|K
  (params (Key :type Key%20Structure :default "None"))
  ;[1 0.6235 0.6706] 無敵状態に
  (:Pressed
    (bind _isa (Utilities|FlowControl|FlipFlop)
      (:A
        _)
      (:B
        _))
    (Variables|/Script/Engine.Actor|SetbCanBeDamaged (Variables|Debug|GetCharacterRef) (not _isa))
    (Class|BPIWidget|BPIToggleInvincible(Message) (Variables|Default|GetDebuggingWidget))))

(fn ConstructionScript
  (|CallParentFunction))

(fn BPIGetDebugInfo
  (return (Variables|Debug|GetCharacterRef) false (Variables|Debug|GetShowCharacterInfo) (Variables|Debug|GetShowDebugShapes) (Variables|Debug|GetShowHUD) false (Variables|Debug|GetShowTraces)))