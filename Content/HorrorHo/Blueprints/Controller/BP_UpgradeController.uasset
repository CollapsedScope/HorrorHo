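; Player controller for the between-stage upgrade screen, playing a transition movie before showing the power-up menu.
; BeginPlay picks the movie by next level name and starts a per-frame timer to poll player state, creating UI_Powerup when playback ends.
; Menu buttons and movement axes forward to the widget through interface messages, with edge detection turning stick pushes into single steps.
; On destruction, it shows the cursor and restores game-only input.
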(event EventBeginPlay
  (bind _bp_movieplayer (Variables|Default|GetBP_MoviePlayer))
  (bind _returnvalue (Class|BPIGameInstance|BPIGIGetNextLevelName(Message) (Game|GetGameInstance)))
  (switch name _returnvalue
    (:Default
      (Default|BPIMoviePlayerSetMovieFile _bp_movieplayer "/Game/Movies/Stage1toUpgrade.Stage1toUpgrade" :!label _label))
    (:Stage2_Main
      (goto _label))
    (:Stage3_Main
      (Default|BPIMoviePlayerSetMovieFile _bp_movieplayer "/Game/Movies/Stage2toUpgrade.Stage2toUpgrade")))
  (Default|BPIMoviePlayerBlackScreen _bp_movieplayer)
  (Class|BPIWavesMode|GMFadein(Message) (Game|GetGameMode))
  (Class|BPIMoviePlayer|BPIMoviePlayerPlayAfterFadeOut(Message) _bp_movieplayer)
  (bind _returnvalue_2 (Utilities|Time|SetTimerbyEvent (EventDispatchers|CreateEvent :!event CheckEndMovie) (CallFunction|GetOneFrameTime 6e+01) true))
  (Variables|Default|SetCheckEndMovieTimer _returnvalue_2)
  (Audio|Components|Audio|SetVolumeMultiplier (Variables|Default|GetMediaSound) 3.0 :!class /Script/AudioMixer.SynthComponent))

(event EventDestroyed
  (Variables|Default|SetbShowMouseCursor true)
  (Input|SetInputModeGameOnly self))

(event Input|ActionEvents|InputActionMenuChoose/Climb
  (params (Key :type Key%20Structure :default "None"))
  (:Pressed
    (Class|BPIKeyNotify|BPIPressA(Message) (Variables|Default|GetWidget))))

(event Input|ActionEvents|InputActionMenuDown
  (params (Key :type Key%20Structure :default "None"))
  (:Pressed
    (Class|BPIKeyNotify|BPIDown(Message) (Variables|Default|GetWidget))))

(event Input|ActionEvents|InputActionMenuLeft
  (params (Key :type Key%20Structure :default "None"))
  (:Pressed
    (Class|BPIKeyNotify|BPILeft(Message) (Variables|Default|GetWidget))))

(event Input|ActionEvents|InputActionMenuRight
  (params (Key :type Key%20Structure :default "None"))
  (:Pressed
    (Class|BPIKeyNotify|BPIRight(Message) (Variables|Default|GetWidget))))

(event Input|ActionEvents|InputActionMenuUp/Heal
  (params (Key :type Key%20Structure :default "None"))
  (:Pressed
    (Class|BPIKeyNotify|BPIUp(Message) (Variables|Default|GetWidget))))

(event Input|ActionEvents|InputActionMenuCancel/Barricade
  (params (Key :type Key%20Structure :default "None"))
  (:Pressed
    (Class|BPIKeyNotify|BPIPressB(Message) (Variables|Default|GetWidget))))

(event Input|AxisEvents|InputAxisMoveForward
  (params (AxisValue :type Float%20%28single-precision%29))
  (bind _widget (Variables|Default|GetWidget))
  (Utilities|Y-AxisInput AxisValue
    (:+
      (Class|BPIKeyNotify|BPIUp(Message) _widget))
    (:-
      (Class|BPIKeyNotify|BPIDown(Message) _widget))))

(event Input|AxisEvents|InputAxisMoveRight
  (params (AxisValue :type Float%20%28single-precision%29))
  (bind _widget (Variables|Default|GetWidget))
  (Utilities|X-AxisInput AxisValue
    (:+
      (Class|BPIKeyNotify|BPIRight(Message) _widget))
    (:-
      (Class|BPIKeyNotify|BPILeft(Message) _widget))))

(fn ConstructionScript)

(fn CheckEndMovie
  (bind _state (Class|BPIMoviePlayer|BPIMoviePlayerGetState(Message) (Variables|Default|GetBP_MoviePlayer)))
  (if (Utilities|Enum|Equal(Enum) _state "NewEnumerator3")
    (Class|BPIMoviePlayer|BPIMoviePlayerCloseScreen(Message) (Variables|Default|GetBP_MoviePlayer))
    (bind _returnvalue (UserInterface|CreateWidget "/Game/HorrorHo/Blueprints/Widgets/Menus/UI_Powerup.UI_Powerup_C"))
    (bind _output_get (Variables|Default|SetWidget _returnvalue))
    (UserInterface|Viewport|AddtoViewport _output_get 0)
    (Utilities|Time|ClearandInvalidateTimerbyHandle (Variables|Default|GetCheckEndMovieTimer))))