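; AI controller for zombies that sets up the zombie blackboard and runs its behavior tree on begin play.
; InitBlackBoard seeds the closest entrance, chosen by navigation path length across the game mode's level entry points, and clears entry state flags.
; InitDestroy stops the brain, releases any held entrance attack permission and frees an entry point mid-transition before destroying the controller.
; A cached getter supplies the controlled zombie character.
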(event EventBeginPlay
  (bind _blackboardcomponent (Class|AIController|UseBlackboard "/Game/HorrorHo/Blueprints/AI/ZombieA/BP_ZombieAI_BB.BP_ZombieAI_BB"))
  (AI|Components|Blackboard|SetValueasVector _blackboardcomponent (Utilities|String|StringToName "ClosestEntranceLocation") "0, 0, 0")
  (AI|RunBehaviorTree "/Game/HorrorHo/Blueprints/AI/ZombieA/BP_ZombieAI_BT.BP_ZombieAI_BT"))

(event EventTick
  (params (DeltaSeconds :type Float%20%28single-precision%29)))

(event EventDestroyed)

(fn ConstructionScript)

(fn InitBlackBoard
  (bind _targetentrance (CallFunction|FindClosestEntrance))
  (bind _blackboardcomponent (Class|AIController|UseBlackboard "/Game/HorrorHo/Blueprints/AI/ZombieA/BP_ZombieAI_BB.BP_ZombieAI_BB"))
  (AI|Components|Blackboard|SetValueasVector _blackboardcomponent (Utilities|String|StringToName "ClosestEntranceLocation") _targetentrance)
  (AI|Components|Blackboard|SetValueasBool _blackboardcomponent (Utilities|String|StringToName "CanEnter") false)
  (AI|Components|Blackboard|SetValueasBool _blackboardcomponent (Utilities|String|StringToName "IsInitialized") false))

(fn FindClosestEntrance
  ;[1 1 1] Collect the distances to each entrance
  (LocalVariables|SetActorLocation (Transformation|GetActorLocation (Pawn|GetControlledPawn)))
  (bind _aszombies_game_mode (Utilities|Casting|CastToZombiesGameMode (Game|GetGameMode)))
  (for _array_element (Variables|/Game/HorrorHo/Blueprints/GameMode/ZombiesGameMode.ZombiesGameMode_C|GetLevelEntryPoints _aszombies_game_mode)
    (if (and (< (.PathLength (Class|NavigationSystemV1|GetPathLength (LocalVariables|GetActorLocation) (Transformation|GetWorldLocation (Variables|/Game/HorrorHo/Blueprints/Actors/Installation/BP_EnemyEnterPoint.BP_EnemyEnterPoint_C|GetEnterVolume _array_element)) 0 0)) (LocalVariables|GetShortestDistance)) (Utilities|Enum|Equal(Enum) (.ReturnValue (Class|NavigationSystemV1|GetPathLength (LocalVariables|GetActorLocation) (Transformation|GetWorldLocation (Variables|/Game/HorrorHo/Blueprints/Actors/Installation/BP_EnemyEnterPoint.BP_EnemyEnterPoint_C|GetEnterVolume _array_element)) 0 0)) "Success"))
      (LocalVariables|SetShortestDistance (.PathLength (Class|NavigationSystemV1|GetPathLength (LocalVariables|GetActorLocation) (Transformation|GetWorldLocation (Variables|/Game/HorrorHo/Blueprints/Actors/Installation/BP_EnemyEnterPoint.BP_EnemyEnterPoint_C|GetEnterVolume _array_element)) 0 0)))
      (LocalVariables|SetClosestFoundEntrance (Transformation|GetWorldLocation (Variables|/Game/HorrorHo/Blueprints/Actors/Installation/BP_EnemyEnterPoint.BP_EnemyEnterPoint_C|GetEnterVolume _array_element)))))
  (return (LocalVariables|GetClosestFoundEntrance)))

(fn InitDestroy
  (bind _blackboard (Variables|Default|GetBlackboard))
  ;[1 1 1] If the zombie is killed while trying to enter through a barricade, we have to release their permission here
  (AI|Logic|StopLogic (Variables|Default|GetBrainComponent) "")
  (if (ScalableFloat|GetValueasBool (Variables|Default|GetBlackboard) (Utilities|Name|MakeLiteralName "EntranceAttackPermission"))
    (bind _zombiesmode (Class|ZombiesGameModeInterface|GetZombiesMode(Message) (Game|GetGameMode)))
    (Default|ReleasePermissionAttackEntrance _zombiesmode (Class|BlackboardComponent|GetValueasInt (Variables|Default|GetBlackboard) (Utilities|Name|MakeLiteralName "IntendedEntranceAttackTarget"))))
  (if (and (ScalableFloat|GetValueasBool _blackboard (Utilities|Name|MakeLiteralName "IsTransitioning")) (not (ScalableFloat|GetValueasBool _blackboard (Utilities|Name|MakeLiteralName "IsInsidePlayerArea"))))
    (bind _asbp_enemy_enter_point (Utilities|Casting|CastToBP_EnemyEnterPoint (AI|Components|Blackboard|GetValueasObject (Variables|Default|GetBlackboard) (Utilities|Name|MakeLiteralName "EnterPoint")))
      (:then
        (Variables|/Game/HorrorHo/Blueprints/Actors/Installation/BP_EnemyEnterPoint.BP_EnemyEnterPoint_C|SetIsBeingUsed _asbp_enemy_enter_point false))
      (:CastFailed
        _)))
  (Actor|DestroyActor))

(fn GetControlledZombie
  (Utilities|IsValid (Variables|Default|GetZombieCharacter)
    (:Is%20Valid
      _)
    (:Is%20Not%20Valid
      (bind _asbp_zombie_character (Utilities|Casting|CastToBP_ZombieCharacter (Pawn|GetControlledPawn)))
      (Variables|Default|SetZombieCharacter _asbp_zombie_character)))
  (return (Variables|Default|GetZombieCharacter)))

(fn GetZombieController
  (return self))