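; Player controller for a shooting game that creates the gunsight and shooting HUD widgets and passes possessed pawns to BP_CameraManager.
; The Pause action opens UI_Pause with the game paused and cursor shown, or messages the open menu and clears its reference.
; Gamepad D-pad and bottom face button drive pause-menu navigation and selection.
; Number keys toggle debug display flags, exposed to other Blueprints through BPI_GetDebugInfo.
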(event EventBeginPlay
  ;[1 1 1] ヘアクロスの描画設定
  (bind _returnvalue (UserInterface|CreateWidget "/Game/HorrorHo/Blueprints/Widgets/UI_GunSight.UI_GunSight_C"))
  (bind _output_get (Variables|Default|SetGunSightWidget _returnvalue))
  (UserInterface|Viewport|AddtoViewport _output_get 0)
  ;[1 1 1] HUD描画設定
  (bind _returnvalue_2 (UserInterface|CreateWidget "/Game/HorrorHo/Blueprints/Widgets/UI_Shooting.UI_Shooting_C"))
  (bind _output_get_2 (Variables|Default|SetShootingWidget _returnvalue_2))
  (UserInterface|Viewport|AddtoViewport _output_get_2 0)
  (Variables|Debug|SetDebugFocusCharacter (Game|GetPlayerCharacter 0)))

(event EventTick
  (params (DeltaSeconds :type Float%20%28single-precision%29)))

(event EventPossess
  (params (PossessedPawn :type Pawn%20Object%20Reference))
  ;[1 1 1] Pawn にこのコントローラが設置されたとき
  (bind _asbp_camera_manager (Utilities|Casting|CastToBP_CameraManager (Variables|Default|GetPlayerCameraManager)))
  (Default|OnPossess _asbp_camera_manager PossessedPawn))

(event Input|ActionEvents|InputActionPause
  (params (Key :type Key%20Structure :default "None"))
  (:Pressed
    (Utilities|IsValid (Variables|Default|GetPauseWidget)
      (:Is%20Valid
        (Class|BPIController|PauseMapped(Message) (stale _returnvalue))
        (Variables|Default|SetPauseWidget 0))
      (:Is%20Not%20Valid
        (bind _returnvalue (UserInterface|CreateWidget "/Game/HorrorHo/Blueprints/Widgets/UI_Pause.UI_Pause_C"))
        (bind _output_get (Variables|Default|SetPauseWidget _returnvalue))
        (UserInterface|Viewport|AddtoViewport _output_get 0)
        (Game|SetGamePaused true)
        (Input|SetInputModeGameandUI self (Variables|Default|GetPauseWidget) "DoNotLock" true)
        (Variables|/Script/Engine.PlayerController|SetbShowMouseCursor self true)
        (Audio|PlaySound2D "/Engine/VREditor/Sounds/UI/Click_on_Button_Cue.Click_on_Button_Cue" 1.0 1.0 0.0 0 0)))))

(event Input|GamepadEvents|GamepadDPadUp
  (params (Key :type Key%20Structure :default "None"))
  ;[1 1 1] Select Pause Menu
  (:Pressed
    (Utilities|IsValid (Variables|Default|GetPauseWidget)
      (:Is%20Valid
        (Default|ReceiveNavigationRequest (Variables|Default|GetPauseWidget) "NewEnumerator0")))))

(event Input|GamepadEvents|GamepadDPadDown
  (params (Key :type Key%20Structure :default "None"))
  ;[1 1 1] Select Pause Menu
  (:Pressed
    (Utilities|IsValid (Variables|Default|GetPauseWidget)
      (:Is%20Valid
        (Default|ReceiveNavigationRequest (Variables|Default|GetPauseWidget) "NewEnumerator1"))))
  (:Released
    (Utilities|Time|ClearandInvalidateTimerbyHandle (Variables|Default|GetD-padDownTimer))))

(event Input|GamepadEvents|GamepadFaceButtonBottom
  (params (Key :type Key%20Structure :default "None"))
  ;[1 1 1] Choose
  (:Pressed
    (Utilities|IsValid (Variables|Default|GetPauseWidget)
      (:Is%20Valid
        (Default|PressA (Variables|Default|GetPauseWidget))
        (if (== (Variables|/Game/HorrorHo/Blueprints/Widgets/UI_Pause.UI_Pause_C|GetMainNavigationIndex (Variables|Default|GetPauseWidget)) 0)
          (Variables|Default|SetPauseWidget 0))))))

(event Input|KeyboardEvents|1
  (params (Key :type Key%20Structure :default "None"))
  ;[1 1 1] Debug
  (:Pressed
    (Variables|Debug|SetDebugView (not (Variables|Debug|GetDebugView)))))

(event Input|KeyboardEvents|2
  (params (Key :type Key%20Structure :default "None"))
  ;[1 1 1] Debug
  (:Pressed
    (Variables|Debug|SetShowHUD (not (Variables|Debug|GetShowHUD)))))

(event Input|KeyboardEvents|3
  (params (Key :type Key%20Structure :default "None"))
  ;[1 1 1] Debug
  (:Pressed
    (Variables|Debug|SetShowDebugShapes (not (Variables|Debug|GetShowDebugShapes)))))

(event Input|KeyboardEvents|4
  (params (Key :type Key%20Structure :default "None"))
  ;[1 1 1] Debug
  (:Pressed
    (Variables|Debug|SetShowCharacterInfo (not (Variables|Debug|GetShowCharacterInfo)))))

(event Input|KeyboardEvents|5
  (params (Key :type Key%20Structure :default "None"))
  ;[1 1 1] Debug
  (:Pressed
    (Variables|Debug|SetShowLayerColor (not (Variables|Debug|GetShowLayerColor)))))

(event Input|KeyboardEvents|6
  (params (Key :type Key%20Structure :default "None"))
  ;[1 1 1] Debug
  (:Pressed
    (Variables|Debug|SetShowTrace (not (Variables|Debug|GetShowTrace)))))

(fn ConstructionScript)

(fn BPIGetDebugInfo
  (return (Variables|Debug|GetDebugView) (Variables|Debug|GetShowCharacterInfo) (Variables|Debug|GetShowDebugShapes) (Variables|Debug|GetShowHUD) (Variables|Debug|GetShowLayerColor) (Variables|Debug|GetShowTrace)))