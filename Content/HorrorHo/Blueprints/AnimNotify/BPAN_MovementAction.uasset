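; Anim notify state that sets the player's movement action for the duration of an animation window.
; On begin, it passes its configured MovementAction to the mesh owner through Blueprint interface messages.
; On end, it resets the action to the enum's first entry only if the current action still matches, so a different action set meanwhile is preserved.
; The notify's displayed name includes the chosen action.
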(fn ReceivedNotifyBegin
  (params (MeshComp :type Skeletal%20Mesh%20Component%20Object%20Reference) (Animation :type Anim%20Sequence%20Base%20Object%20Reference) (TotalDuration :type Float%20%28single-precision%29))
  (Class|BPIPlayer|BPIPlayerSetMovementAction(Message) (Components|GetOwner MeshComp) (Variables|Default|GetMovementAction))
  (return false))

(fn ReceivedNotifyEnd
  (params (MeshComp :type Skeletal%20Mesh%20Component%20Object%20Reference) (Animation :type Anim%20Sequence%20Base%20Object%20Reference))
  (bind _movementaction (Class|BPIPlayer|BPIPlayerGetCurrentStates(Message) (Components|GetOwner MeshComp)))
  (if (Utilities|Enum|Equal(Enum) _movementaction (Variables|Default|GetMovementAction))
    (Class|BPIPlayer|BPIPlayerSetMovementAction(Message) (Components|GetOwner MeshComp) "NewEnumerator0")
    (return false)
    (else
      (return false))))

(fn GetNotifyName
  (return (Utilities|String|Append "Movement Action: " (Utilities|String|EnumtoString (Variables|Default|GetMovementAction)))))