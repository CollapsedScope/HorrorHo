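; Anim notify state that cuts a configured montage short during its window, shown as Early_BlendOut in the editor.
; Each tick it queries the owning actor through Blueprint interface messages, with optional checks for a matching movement state or for active movement input.
; When an enabled check passes, it stops the montage on the mesh's anim instance using the configured blend-out time.
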(fn ReceivedNotifyTick
  (params (MeshComp :type Skeletal%20Mesh%20Component%20Object%20Reference) (Animation :type Anim%20Sequence%20Base%20Object%20Reference) (FrameDeltaTime :type Float%20%28single-precision%29))
  (LocalVariables|SetAnimInstance (Components|SkeletalMesh|GetAnimInstance MeshComp))
  (LocalVariables|SetOwningActor (Components|GetOwner MeshComp))
  (Utilities|FlowControl|Sequence
    (:then_0
      (if (Variables|Default|GetCheckMovementState)
        (bind _movementstate (Class|BPIPlayer|BPIGetCurrentStates(Message) (LocalVariables|GetOwningActor)))
        (if (Utilities|Enum|Equal(Enum) _movementstate (Variables|Default|GetMovementStateEquals))
          (Animation|Montage|MontageStop (LocalVariables|GetAnimInstance) (Variables|Default|GetBlendOutTime) (Variables|Default|GetThisMontage))
          (return true))))
    (:then_2
      (if (Variables|Default|GetCheckMovementInput)
        (bind _hasmovementinput (Class|BPIPlayer|BPIGetEssentialValues(Message) (LocalVariables|GetOwningActor)))
        (if _hasmovementinput
          (Animation|Montage|MontageStop (LocalVariables|GetAnimInstance) (Variables|Default|GetBlendOutTime) (Variables|Default|GetThisMontage)))))))

(fn GetNotifyName
  (return "Early_BlendOut"))