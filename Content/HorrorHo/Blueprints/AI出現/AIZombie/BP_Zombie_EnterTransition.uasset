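; BP_Zombie_EnterTransition is a behavior tree task that moves a zombie into the player area through an enemy enter point.
; It reads the BP_EnemyEnterPoint from the blackboard and teleports the zombie controller's pawn to that point's exit volume without sweeping.
; It then sets the IsInsidePlayerArea blackboard flag and finishes successfully.
; The teleport is marked as temporary, and a failed cast stops the task without calling FinishExecute.
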(event EventReceiveExecute
  (params (OwnerActor :type Actor%20Object%20Reference))
  ;[1 1 1] Temporary: teleport pawn to exit location
  (bind _asbp_zombie_controller (Utilities|Casting|CastToBP_ZombieController OwnerActor))
  (bind _asbp_enemy_enter_point (Utilities|Casting|CastToBP_EnemyEnterPoint (Class|BTFunctionLibrary|GetBlackboardValueasObject (Variables|Default|GetEnterPoint))))
  (Transformation|SetActorLocation (Pawn|GetControlledPawn _asbp_zombie_controller) (Transformation|GetWorldLocation (Variables|/Game/HorrorHo/Blueprints/AI出現/BP_EnemyEnterPoint.BP_EnemyEnterPoint_C|GetExitVolume _asbp_enemy_enter_point)) false true)
  (Class|BTFunctionLibrary|SetBlackboardValueasBool (Variables|Default|GetIsInsidePlayerArea) true)
  (AI|BehaviorTree|FinishExecute true))