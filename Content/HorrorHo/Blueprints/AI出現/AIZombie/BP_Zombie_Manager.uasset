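; Zombie manager that limits how many zombies may attack the player at once.
; It caches the player pawn on BeginPlay, and QueryAttackPermission grants free slots in CurrentAttackers up to AttackerMax.
; When slots are full, a requester closer to the player replaces the first farther attacker found, whose permission is revoked.
; It returns a permission flag with either the attacker or chaser target distance.
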(event EventBeginPlay
  (Variables|Default|SetPlayerReference (Game|Player|GetPlayerPawn 0)))

(event Collision|EventActorBeginOverlap
  (params (OtherActor :type Actor%20Object%20Reference)))

(event EventTick
  (params (DeltaSeconds :type Float%20%28single-precision%29)))

(fn ConstructionScript)

(fn QueryAttackPermission
  (params (ZombieInstance :type BP%20Zombie%20Character%20Object%20Reference))
  (bind _playerreference (Variables|Default|GetPlayerReference))
  (bind _currentattackers (Variables|Default|GetCurrentAttackers))
  (if (< (Utilities|Array|Length (Variables|Default|GetCurrentAttackers)) (Variables|Default|GetAttackerMax))
    (Utilities|Array|Add (Variables|Default|GetCurrentAttackers) ZombieInstance)
    (return true (Variables|Default|GetAttackerTargetDistance))
    (else
      (LocalVariables|SetNewDistance (Transformation|GetDistanceTo _playerreference ZombieInstance))
      (for _array_element (Variables|Default|GetCurrentAttackers)
        (if (< (LocalVariables|GetNewDistance) (Transformation|GetDistanceTo _playerreference _array_element))
          (Variables|/Game/HorrorHo/Blueprints/AI出現/AIZombie/BP_ZombieCharacter.BP_ZombieCharacter_C|SetAttackPermission _array_element false)
          (Utilities|Array|RemoveItem _currentattackers _array_element)
          (Utilities|Array|Add _currentattackers ZombieInstance)
          (return true (Variables|Default|GetAttackerTargetDistance))))
      (return false (Variables|Default|GetChaserTargetDistance)))))