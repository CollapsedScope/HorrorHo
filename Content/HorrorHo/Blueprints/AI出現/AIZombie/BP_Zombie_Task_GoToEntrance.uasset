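; Behavior tree task that sends a zombie to the EntranceLocation stored in its blackboard.
; It finishes successfully if the controlled pawn is already at that point within a small tolerance, otherwise it issues AIMoveTo.
; When the move succeeds, it sets the IsTransitioning key and finishes as failed; a failed move has no handler, so the task does not finish on that path.
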(event EventReceiveExecute
  (params (OwnerActor :type Actor%20Object%20Reference))
  (bind _entrancelocation (Variables|Default|GetEntranceLocation))
  (bind _returnvalue (Class|BTFunctionLibrary|GetBlackboardValueasVector _entrancelocation))
  (bind _asbp_zombie_controller (Utilities|Casting|CastToBP_ZombieController OwnerActor))
  (if (Math|Vector|Equal(Vector) (Transformation|GetActorLocation (Pawn|GetControlledPawn _asbp_zombie_controller)) _returnvalue 1e+01)
    (AI|BehaviorTree|FinishExecute true)
    (else
      (AI|AIMoveTo (Pawn|GetControlledPawn _asbp_zombie_controller) _returnvalue 0 5.0 false
        (:OnSuccess
          (Class|BTFunctionLibrary|SetBlackboardValueasBool (Variables|Default|GetIsTransitioning) true)
          (AI|BehaviorTree|FinishExecute false))))))