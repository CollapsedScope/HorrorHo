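; Behavior tree task that makes a zombie attack the barricade at its enemy enter point until it can move into the player area.
; After an attack-speed delay, it reads the enter point from the blackboard and flags the zombie to attack while barricade health remains, otherwise to allow entry.
; When entry is already allowed, it sets the CanEnter blackboard key instead.
; Each of these branches finishes the task successfully.
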(event EventReceiveExecute
  (params (OwnerActor :type Actor%20Object%20Reference))
  ;[1 1 1] Temporary Attack Speed Delay
  (Utilities|FlowControl|Delay (Variables|Default|GetAttackSpeed))
  (bind _asbp_zombie_controller (Utilities|Casting|CastToBP_ZombieController OwnerActor))
  (bind _asbp_zombie_character (Utilities|Casting|CastToBP_ZombieCharacter (Pawn|GetControlledPawn _asbp_zombie_controller)))
  (if (Variables|/Game/HorrorHo/Blueprints/AI出現/AIZombie/BP_ZombieCharacter.BP_ZombieCharacter_C|GetCanEnterPlayerArea _asbp_zombie_character)
    ;[1 1 1] If the barricade is destroyed, wait to transition into player area
    (Class|BTFunctionLibrary|SetBlackboardValueasBool (Variables|Default|GetCanEnter) true)
    (AI|BehaviorTree|FinishExecute true)
    (else
      (bind _asbp_enemy_enter_point (Utilities|Casting|CastToBP_EnemyEnterPoint (AI|BehaviorTree|GetBlackboardValueasActor (Variables|Default|GetEnterPoint))))
      (if (Math|Conversions|ToBoolean(Integer) (Variables|/Game/HorrorHo/Blueprints/AI出現/BP_EnemyEnterPoint.BP_EnemyEnterPoint_C|GetBarricadeHealth _asbp_enemy_enter_point))
        ;[1 1 1] Attack if the barricade is still alive
        (Variables|/Game/HorrorHo/Blueprints/AI出現/AIZombie/BP_ZombieCharacter.BP_ZombieCharacter_C|SetStartAttack _asbp_zombie_character true)
        (else
          ;[1 1 1] Skip attacking if the barricade is already  dead
          (Variables|/Game/HorrorHo/Blueprints/AI出現/AIZombie/BP_ZombieCharacter.BP_ZombieCharacter_C|SetCanEnterPlayerArea _asbp_zombie_character true)))
      (AI|BehaviorTree|FinishExecute true))))