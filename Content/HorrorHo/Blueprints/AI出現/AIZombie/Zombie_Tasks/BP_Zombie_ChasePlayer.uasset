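; Behavior tree task that sends a zombie after the player pawn.
; If the zombie lacks attack permission, it queries the game mode's ZombieManager, storing permission on the character and target distance in the blackboard.
; That distance becomes the AIMoveTo acceptance radius.
; The task finishes successfully once the move is issued, setting IsMoving; either move outcome later clears it and calls FinishExecute as failed.
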(event EventReceiveExecute
  (params (OwnerActor :type Actor%20Object%20Reference))
  (bind _ismoving (Variables|Default|GetIsMoving))
  (bind _asbp_zombie_controller (Utilities|Casting|CastToBP_ZombieController OwnerActor))
  (bind _asbp_zombie_character (Utilities|Casting|CastToBP_ZombieCharacter (Pawn|GetControlledPawn _asbp_zombie_controller)))
  (bind _output_get (Variables|Default|SetControlledPawn _asbp_zombie_character))
  (if (Variables|/Game/HorrorHo/Blueprints/AI出現/AIZombie/BP_ZombieCharacter.BP_ZombieCharacter_C|GetAttackPermission _output_get)
    _
    (else
      (CallFunction|UpdateAttackPermission)))
  (AI|AIMoveTo (Variables|Default|GetControlledPawn) "0, 0, 0" (Game|Player|GetPlayerPawn 0) (Class|BTFunctionLibrary|GetBlackboardValueasFloat (Variables|Default|GetPermissionTargetDistance)) false
    (:then
      (Class|BTFunctionLibrary|SetBlackboardValueasBool _ismoving true)
      (AI|BehaviorTree|FinishExecute true))
    (:OnSuccess
      (Class|BTFunctionLibrary|SetBlackboardValueasBool _ismoving false :!label _label)
      (AI|BehaviorTree|FinishExecute false))
    (:OnFail
      (goto _label))))

(fn UpdateAttackPermission
  (params (ControlledPawn :type Pawn%20Object%20Reference) (Player :type Pawn%20Object%20Reference))
  (bind _aszombies_game_mode (Utilities|Casting|CastToZombiesGameMode (Game|GetGameMode)))
  (bind (_permission _targetdistance) (Default|QueryAttackPermission (Variables|/Game/HorrorHo/Blueprints/GameMode/ZombiesGameMode.ZombiesGameMode_C|GetZombieManager _aszombies_game_mode) (Variables|Default|GetControlledPawn)))
  (Variables|/Game/HorrorHo/Blueprints/AI出現/AIZombie/BP_ZombieCharacter.BP_ZombieCharacter_C|SetAttackPermission (Variables|Default|GetControlledPawn) _permission)
  (Class|BTFunctionLibrary|SetBlackboardValueasFloat (Variables|Default|GetPermissionTargetDistance) _targetdistance))