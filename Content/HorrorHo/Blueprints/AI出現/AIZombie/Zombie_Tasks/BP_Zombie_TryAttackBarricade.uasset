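; Behavior tree task for zombie AI that asks the game mode for permission to attack a barricaded entrance, identified by a blackboard entrance ID.
; If granted, it sets the AttackPermission key and moves the controlled zombie to the blackboard entrance location.
; Finish results are inverted: reaching the entrance reports failure, while a failed move, or a denied request after a short delay, reports success.
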(event EventReceiveExecute
  (params (OwnerActor :type Actor%20Object%20Reference))
  (bind _zombiesmode (Class|ZombiesGameModeInterface|GetZombiesMode(Message) (Game|GetGameMode)))
  (bind _permissionresult (Default|AskPermissionAttackEntrance _zombiesmode (Class|BTFunctionLibrary|GetBlackboardValueasInt (Variables|Default|GetTargetEntranceID))))
  (if _permissionresult
    (Class|BTFunctionLibrary|SetBlackboardValueasBool (Variables|Default|GetAttackPermission) true)
    ;[1 1 1] Move closer to door before returning success
    (bind _asbp_zombie_controller (Utilities|Casting|CastToBP_ZombieController OwnerActor))
    (AI|AIMoveTo (Pawn|GetControlledPawn _asbp_zombie_controller) (Class|BTFunctionLibrary|GetBlackboardValueasVector (Variables|Default|GetEntranceLocation)) 0 1e+02 true
      (:OnSuccess
        (AI|BehaviorTree|FinishExecute false))
      (:OnFail
        (AI|BehaviorTree|FinishExecute true)))
    (else
      (Utilities|FlowControl|Delay 0.5)
      (AI|BehaviorTree|FinishExecute true))))