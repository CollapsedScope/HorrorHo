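; Behavior tree task that lets a zombie claim an enemy entry point to cross into the player area.
; It reads the enter point from the blackboard and fails if another zombie is using it, so the zombie waits.
; Otherwise it flags the zombie as transitioning for its animation, marks the entry point as in use, sets the IsTransitioning key and succeeds.
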(event EventReceiveExecute
  (params (OwnerActor :type Actor%20Object%20Reference))
  (bind _asbp_enemy_enter_point (Utilities|Casting|CastToBP_EnemyEnterPoint (Class|BTFunctionLibrary|GetBlackboardValueasObject (Variables|Default|GetEnterPoint))))
  (if (Variables|/Game/HorrorHo/Blueprints/AI出現/BP_EnemyEnterPoint.BP_EnemyEnterPoint_C|GetIsBeingUsed _asbp_enemy_enter_point)
    ;[1 1 1] The entrance is being used, so return fail in order to wait.
    (AI|BehaviorTree|FinishExecute false)
    (else
      ;[1 1 1] The entrance is open right now, so we will switch to the transition animation and stop other zombies from using the door for now.  Also tell the zombie to play its transition animation
      (bind _asbp_zombie_controller (Utilities|Casting|CastToBP_ZombieController OwnerActor))
      (bind _zombie (Default|GetZombie _asbp_zombie_controller))
      (Variables|/Game/HorrorHo/Blueprints/AI出現/AIZombie/BP_ZombieCharacter.BP_ZombieCharacter_C|SetIsTransitioningToPlayerArea _zombie true)
      (Variables|/Game/HorrorHo/Blueprints/AI出現/BP_EnemyEnterPoint.BP_EnemyEnterPoint_C|SetIsBeingUsed _asbp_enemy_enter_point true)
      (Class|BTFunctionLibrary|SetBlackboardValueasBool (Variables|Default|GetIsTransitioning) true)
      (AI|BehaviorTree|FinishExecute true))))