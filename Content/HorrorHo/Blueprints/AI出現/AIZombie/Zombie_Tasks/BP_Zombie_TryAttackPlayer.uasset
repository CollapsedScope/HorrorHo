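; Behavior tree task that makes a zombie attempt a melee-range attack on the player in a horror game.
; It succeeds immediately if the controlled zombie is already attacking, otherwise compares its distance to player 0 against AttackRange.
; In range, it snaps the zombie's rotation toward the player, sets its StartAttack and IsAttacking flags and succeeds.
; Out of range, the task fails.
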(event EventReceiveExecute
  (params (OwnerActor :type Actor%20Object%20Reference))
  (bind _asbp_zombie_controller (Utilities|Casting|CastToBP_ZombieController OwnerActor))
  (bind _asbp_zombie_character (Utilities|Casting|CastToBP_ZombieCharacter (Pawn|GetControlledPawn _asbp_zombie_controller)))
  (bind _output_get (Variables|Default|SetControlledPawn _asbp_zombie_character))
  (if (Variables|/Game/HorrorHo/Blueprints/AI出現/AIZombie/BP_ZombieCharacter.BP_ZombieCharacter_C|GetIsAttacking _output_get)
    (AI|BehaviorTree|FinishExecute true)
    (elif (< (Math|Vector|VectorLength (- (Transformation|GetActorLocation (Game|Player|GetPlayerPawn 0)) (Transformation|GetActorLocation _output_get))) (Variables|Default|GetAttackRange))
      (Transformation|SetActorRotation (Variables|Default|GetControlledPawn) (Math|Conversions|RotationFromXVector (Math|Vector|Normalize (- (Transformation|GetActorLocation (Game|Player|GetPlayerPawn 0)) (Transformation|GetActorLocation _output_get)))))
      (Variables|/Game/ThirdPersonBP/Blueprints/ThirdPersonCharacter.ThirdPersonCharacter_C|SetStartAttack (Variables|Default|GetControlledPawn) true)
      (Variables|/Game/HorrorHo/Blueprints/AI出現/AIZombie/BP_ZombieCharacter.BP_ZombieCharacter_C|SetIsAttacking (Variables|Default|GetControlledPawn) true)
      (AI|BehaviorTree|FinishExecute true)
      (else
        (AI|BehaviorTree|FinishExecute false)))))