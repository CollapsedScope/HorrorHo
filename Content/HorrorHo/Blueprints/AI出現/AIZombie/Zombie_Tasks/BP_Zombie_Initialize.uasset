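; Behavior tree task that initializes a zombie AI by choosing the level entrance it will target.
; It loops over the game mode's LevelEntryPoints and picks the barricade volume with the shortest path length from the controlled pawn.
; The search writes the entry point and its index to the blackboard.
; The task then stores the location, marks the zombie initialized, clears attack permission and moving flags, and finishes successfully.
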(event EventReceiveExecute
  (params (OwnerActor :type Actor%20Object%20Reference))
  (bind _asbp_zombie_controller (Utilities|Casting|CastToBP_ZombieController OwnerActor))
  (bind _targetentrance (CallFunction|FindClosestEntrance _asbp_zombie_controller))
  (AI|BehaviorTree|SetBlackboardValueasVector (Variables|Default|GetClosestEntranceLocation) _targetentrance)
  (Class|BTFunctionLibrary|SetBlackboardValueasBool (Variables|Default|GetIsInitialized) true)
  (Class|BTFunctionLibrary|SetBlackboardValueasBool (Variables|Default|GetEntranceAttackPermission) false)
  (Class|BTFunctionLibrary|SetBlackboardValueasBool (Variables|Default|GetIsMoving) false)
  (AI|BehaviorTree|FinishExecute true))

(fn FindClosestEntrance
  (params (Controller :type BP%20Zombie%20Controller%20Object%20Reference))
  ;[1 1 1] Collect the distances to each entrance
  (bind _aszombies_game_mode (Utilities|Casting|CastToZombiesGameMode (Game|GetGameMode)))
  (LocalVariables|SetActorLocation (Transformation|GetActorLocation (Pawn|GetControlledPawn Controller)))
  (for (_array_element _array_index) (Variables|/Game/HorrorHo/Blueprints/GameMode/ZombiesGameMode.ZombiesGameMode_C|GetLevelEntryPoints _aszombies_game_mode)
    (if (< (.PathLength (Class|NavigationSystemV1|GetPathLength (LocalVariables|GetActorLocation) (Transformation|GetWorldLocation (Variables|/Game/HorrorHo/Blueprints/AI出現/BP_EnemyEnterPoint.BP_EnemyEnterPoint_C|GetBarricadeVolume _array_element)) 0 0)) (LocalVariables|GetShortestDistance))
      (LocalVariables|SetShortestDistance (.PathLength (Class|NavigationSystemV1|GetPathLength (LocalVariables|GetActorLocation) (Transformation|GetWorldLocation (Variables|/Game/HorrorHo/Blueprints/AI出現/BP_EnemyEnterPoint.BP_EnemyEnterPoint_C|GetBarricadeVolume _array_element)) 0 0)))
      (LocalVariables|SetClosestFoundEntrance (Transformation|GetWorldLocation (Variables|/Game/HorrorHo/Blueprints/AI出現/BP_EnemyEnterPoint.BP_EnemyEnterPoint_C|GetBarricadeVolume _array_element)))
      (Class|BTFunctionLibrary|SetBlackboardValueasObject (Variables|Default|GetEnterPoint) _array_element)
      (Class|BTFunctionLibrary|SetBlackboardValueasInt (Variables|Default|GetTargetEntranceID) _array_index)))
  (return (LocalVariables|GetClosestFoundEntrance)))