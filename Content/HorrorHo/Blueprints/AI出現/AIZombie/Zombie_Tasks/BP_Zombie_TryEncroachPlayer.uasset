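; Behavior tree task that makes a waiting zombie without attack permission slowly creep toward the player once already close.
; Each run adds frame delta to a Blackboard timer, which linearly shrinks the move acceptance radius from the permission distance by up to EncroachLength.
; It succeeds immediately after issuing the move.
; It fails when permission is granted or the player is out of range, resetting the timer in the latter case.
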(event EventReceiveExecute
  (params (OwnerActor :type Actor%20Object%20Reference))
  ;[1 1 1] If the zombie does not have attack permission but is already close to the player, slowly approach the player while waiting
  (bind _asbp_zombie_controller (Utilities|Casting|CastToBP_ZombieController OwnerActor))
  (bind _asbp_zombie_character (Utilities|Casting|CastToBP_ZombieCharacter (Pawn|GetControlledPawn _asbp_zombie_controller)))
  (if (not (Variables|/Game/HorrorHo/Blueprints/AI出現/AIZombie/BP_ZombieCharacter.BP_ZombieCharacter_C|GetAttackPermission _asbp_zombie_character))
    (bind _output_get (Variables|Default|SetPlayerReference (Game|Player|GetPlayerPawn 0)))
    (if (< (Transformation|GetDistanceTo (Pawn|GetControlledPawn _asbp_zombie_controller) _output_get) (+ (Class|BTFunctionLibrary|GetBlackboardValueasFloat (Variables|Default|GetPermissionTargetDistance)) 1e+02))
      (CallFunction|UpdateElapsedTime)
      (bind _distance (CallFunction|CalculateAdjustedTargetDistance))
      (AI|AIMoveTo (Pawn|GetControlledPawn _asbp_zombie_controller) "0, 0, 0" (Variables|Default|GetPlayerReference) _distance false
        (:then
          _)
        (:OnSuccess
          _)
        (:OnFail
          _))
      (AI|BehaviorTree|FinishExecute true)
      (else
        ;[1 1 1] If we are out of range, fail this task and begin chasing again.
        (Class|BTFunctionLibrary|SetBlackboardValueasFloat (Variables|Default|GetElapsedTime) 0.0)
        (AI|BehaviorTree|FinishExecute false)))
    (else
      (AI|BehaviorTree|FinishExecute false))))

(fn CalculateAdjustedTargetDistance
  (return (- (Class|BTFunctionLibrary|GetBlackboardValueasFloat (Variables|Default|GetPermissionTargetDistance)) (* (LocalVariables|GetEncroachLength) (Math|Float|Min(Float) (/ (Class|BTFunctionLibrary|GetBlackboardValueasFloat (Variables|Default|GetElapsedTime)) (LocalVariables|GetEncroachSpeed)) 1.0)))))

(fn UpdateElapsedTime
  (bind _elapsedtime (Variables|Default|GetElapsedTime))
  (Class|BTFunctionLibrary|SetBlackboardValueasFloat _elapsedtime (+ (Class|BTFunctionLibrary|GetBlackboardValueasFloat _elapsedtime) (Utilities|Time|GetWorldDeltaSeconds))))