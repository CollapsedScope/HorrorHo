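; AI controller for zombies that sets up their blackboard and runs the zombie behavior tree.
; BeginPlay zeroes the ClosestEntranceLocation key before starting the tree.
; InitBlackBoard, not called within this graph, fills that key using FindClosestEntrance.
; FindClosestEntrance compares path lengths, rather than straight-line distances, from the controlled pawn to each of the ZombiesGameMode's level entry volumes and returns the nearest.
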(event EventBeginPlay
  (bind _blackboardcomponent (Class|AIController|UseBlackboard "/Game/HorrorHo/Blueprints/AI出現/AIZombie/BP_ZombieAI_BB.BP_ZombieAI_BB"))
  (AI|Components|Blackboard|SetValueasVector _blackboardcomponent (Utilities|String|StringToName "ClosestEntranceLocation") "0, 0, 0")
  (AI|RunBehaviorTree "/Game/HorrorHo/Blueprints/AI出現/AIZombie/BP_ZombieAI_BT.BP_ZombieAI_BT"))

(event EventTick
  (params (DeltaSeconds :type Float%20%28single-precision%29)))

(fn ConstructionScript)

(fn InitBlackBoard
  (bind _targetentrance (CallFunction|FindClosestEntrance))
  (bind _blackboardcomponent (Class|AIController|UseBlackboard "/Game/HorrorHo/Blueprints/AI出現/AIZombie/BP_ZombieAI_BB.BP_ZombieAI_BB"))
  (AI|Components|Blackboard|SetValueasVector _blackboardcomponent (Utilities|String|StringToName "ClosestEntranceLocation") _targetentrance))

(fn FindClosestEntrance
  ;[1 1 1] Collect the distances to each entrance
  (bind _aszombies_game_mode (Utilities|Casting|CastToZombiesGameMode (Game|GetGameMode)))
  (LocalVariables|SetActorLocation (Transformation|GetActorLocation (Pawn|GetControlledPawn)))
  (for _array_element (Variables|/Game/HorrorHo/Blueprints/GameMode/ZombiesGameMode.ZombiesGameMode_C|GetLevelEntryPoints _aszombies_game_mode)
    (if (< (.PathLength (Class|NavigationSystemV1|GetPathLength (LocalVariables|GetActorLocation) (Transformation|GetWorldLocation (Variables|/Game/HorrorHo/Blueprints/AI出現/BP_EnemyEnterPoint.BP_EnemyEnterPoint_C|GetEnterVolume _array_element)) 0 0)) (LocalVariables|GetShortestDistance))
      (LocalVariables|SetShortestDistance (.PathLength (Class|NavigationSystemV1|GetPathLength (LocalVariables|GetActorLocation) (Transformation|GetWorldLocation (Variables|/Game/HorrorHo/Blueprints/AI出現/BP_EnemyEnterPoint.BP_EnemyEnterPoint_C|GetEnterVolume _array_element)) 0 0)))
      (LocalVariables|SetClosestFoundEntrance (Transformation|GetWorldLocation (Variables|/Game/HorrorHo/Blueprints/AI出現/BP_EnemyEnterPoint.BP_EnemyEnterPoint_C|GetEnterVolume _array_element)))))
  (return (LocalVariables|GetClosestFoundEntrance)))